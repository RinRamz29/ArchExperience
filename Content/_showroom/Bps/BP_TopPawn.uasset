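; BP_TopPawn is a showroom pawn, apparently for a top view, that returns control to the first-person character on pause.
; Both look inputs share one control-rotation update that clamps pitch.
; Pause unhides "Ceiling"-tagged actors, hides "POI" BP_PawnChanger widgets and the cursor, then blends the view and possesses BP_FirstPersonCharacter after a matching delay.
; SetCursor, despite its name, only caches all BP_PawnChanger actors.
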(event Custom|Hide%20UI
  (params (InVisibility :type ESlateVisibility%20Enum :default "Visible"))
  (bind _outactors (Actor|GetAllActorswithTag "POI"))
  (for _array_element _outactors
    (bind _asbp_pawn_changer (Utilities|Casting|CastToBP_PawnChanger _array_element))
    (Widget|SetVisibility (UserInterface|GetWidget (Variables|/Game/_showroom/Bps/BP_PawnChanger.BP_PawnChanger_C|GetWidget _asbp_pawn_changer)) InVisibility)))

(event Custom|Unhide%20Ceiling
  (params (bNewHidden :type Boolean))
  (bind _outactors (Actor|GetAllActorswithTag "Ceiling"))
  (for _array_element _outactors
    (Rendering|SetActorHiddenInGame _array_element bNewHidden)
    (Collision|SetActorEnableCollision _array_element true)))

(event Input|EnhancedActionEvents|EnhancedInputActionIA_LookTopUp
  (params (ActionValue :type Float%20%28double-precision%29) (ElapsedSeconds :type Float%20%28double-precision%29) (TriggeredSeconds :type Float%20%28double-precision%29) (InputAction :type Input%20Action%20Object%20Reference :default "/Game/FirstPerson/Input/Actions/IA_LookTopUp.IA_LookTopUp"))
  (bind _returnvalue (Game|GetPlayerController 0))
  (bind _returnvalue_2 (Pawn|GetControlRotation _returnvalue :!class /Script/Engine.Controller))
  (Pawn|SetControlRotation _returnvalue (Math|Rotator|MakeRotator 0.0 (Math|Float|ClampAngle (+ (.pitch _returnvalue_2) (* ActionValue -2.0)) (Variables|Default|GetPitch%20limit%20min) (Variables|Default|GetPitch%20limit%20max)) (+ (* (stale Input|EnhancedActionEvents|EnhancedInputActionIA_LookTopRight ActionValue) -2.0) (.yaw _returnvalue_2)))))

(event Input|EnhancedActionEvents|EnhancedInputActionIA_LookTopRight
  (params (ActionValue :type Float%20%28double-precision%29) (ElapsedSeconds :type Float%20%28double-precision%29) (TriggeredSeconds :type Float%20%28double-precision%29) (InputAction :type Input%20Action%20Object%20Reference :default "/Game/FirstPerson/Input/Actions/IA_LookTopRight.IA_LookTopRight"))
  (bind _returnvalue (Game|GetPlayerController 0))
  (bind _returnvalue_2 (Pawn|GetControlRotation _returnvalue :!class /Script/Engine.Controller))
  (Pawn|SetControlRotation _returnvalue (Math|Rotator|MakeRotator 0.0 (Math|Float|ClampAngle (+ (.pitch _returnvalue_2) (* (stale Input|EnhancedActionEvents|EnhancedInputActionIA_LookTopUp ActionValue) -2.0)) (Variables|Default|GetPitch%20limit%20min) (Variables|Default|GetPitch%20limit%20max)) (+ (* ActionValue -2.0) (.yaw _returnvalue_2)))))

(event Input|EnhancedActionEvents|EnhancedInputActionIA_Pause
  (params (ActionValue :type Boolean) (ElapsedSeconds :type Float%20%28double-precision%29) (TriggeredSeconds :type Float%20%28double-precision%29) (InputAction :type Input%20Action%20Object%20Reference :default "/Game/FirstPerson/Input/Actions/IA_Pause.IA_Pause"))
  (bind _returnvalue (Game|GetPlayerController 0))
  (CallFunction|UnhideCeiling false)
  (CallFunction|HideUI "Hidden")
  (Variables|/Script/Engine.PlayerController|SetbShowMouseCursor (Game|GetPlayerController 0) false)
  (bind _outactors (Actor|GetAllActorsOfClass "/Game/FirstPerson/Blueprints/BP_FirstPersonCharacter.BP_FirstPersonCharacter_C"))
  (Game|Player|SetViewTargetwithBlend _returnvalue 0 0.7 "VTBlend_Linear" 0.0 false)
  (Utilities|FlowControl|Delay 0.7)
  (Pawn|Possess _returnvalue (Utilities|Array|Get(acopy) _outactors)))

(event EventTick
  (params (DeltaSeconds :type Float%20%28single-precision%29)))

(event Collision|EventActorBeginOverlap
  (params (OtherActor :type Actor%20Object%20Reference)))

(fn ConstructionScript)

(fn SetCursor
  (bind _outactors (Actor|GetAllActorsOfClass "/Game/_showroom/Bps/BP_PawnChanger.BP_PawnChanger_C"))
  (Variables|Default|SetChangers _outactors))