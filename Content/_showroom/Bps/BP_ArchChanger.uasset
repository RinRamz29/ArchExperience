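; BP_ArchChanger is a showroom Blueprint that cycles a group of static meshes through preset material sets.
; The ChangeMats event applies every material in the current Mats entry to each mesh in Meshes, using the array position as the material slot.
; It then advances CurrentIndex with modulo wraparound, so each call shows the next set; nothing in this Blueprint calls the event.
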(event EventBeginPlay)

(event Collision|EventActorBeginOverlap
  (params (OtherActor :type Actor%20Object%20Reference)))

(event EventTick
  (params (DeltaSeconds :type Float%20%28single-precision%29)))

(event EventChangeMats
  (bind _mats (Variables|Default|GetMats))
  (for _array_element (Variables|Default|GetMeshes)
    (for (_array_element_2 _array_index) (Utilities|Struct|BreakMatStruct (Utilities|Array|Get(acopy) _mats (Variables|Default|GetCurrentIndex)))
      (Rendering|Material|SetMaterial (Variables|/Script/Engine.StaticMeshActor|GetStaticMeshComponent _array_element) _array_index _array_element_2)))
  (Variables|Default|SetCurrentIndex (Math|Integer|%(Integer) (+ (Variables|Default|GetCurrentIndex) 1) (Utilities|Array|Length _mats))))

(fn ConstructionScript)