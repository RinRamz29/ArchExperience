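; BP_PawnChanger is a showroom point of interest with a widget marker and a menu for swapping material sets on its assigned meshes.
; BeginPlay initializes the marker and creates a collapsed WB_Mats menu; SetMenu feeds it the sets, and ChangeMats applies one by index.
; IA_Pause collapses the menu, hides ceilings and shows markers through BP_TopPawn, then blends the view back and possesses that pawn.
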(event Custom|Hide%20UI
  (params (InVisibility :type ESlateVisibility%20Enum :default "Visible"))
  (bind _outactors (Actor|GetAllActorswithTag "POI"))
  (for _array_element _outactors
    (bind _asbp_pawn_changer (Utilities|Casting|CastToBP_PawnChanger _array_element))
    (Widget|SetVisibility (UserInterface|GetWidget (Variables|BP_PawnChanger_C|GetWidget _asbp_pawn_changer)) InVisibility)))

(event Custom|Unhide%20Ceiling
  (params (bNewHidden :type Boolean))
  (bind _outactors (Actor|GetAllActorswithTag "Ceiling"))
  (for _array_element _outactors
    (Rendering|SetActorHiddenInGame _array_element bNewHidden)
    (Collision|SetActorEnableCollision _array_element true)))

(event Input|EnhancedActionEvents|EnhancedInputActionIA_Pause
  (params (ActionValue :type Boolean) (ElapsedSeconds :type Float%20%28double-precision%29) (TriggeredSeconds :type Float%20%28double-precision%29) (InputAction :type Input%20Action%20Object%20Reference :default "/Game/FirstPerson/Input/Actions/IA_Pause.IA_Pause"))
  (bind _returnvalue (Game|GetPlayerController 0))
  (Widget|SetVisibility (Variables|Default|GetMatsMenuReference) "Collapsed")
  (bind _outactors (Actor|GetAllActorsOfClass "/Game/_showroom/Bps/BP_TopPawn.BP_TopPawn_C"))
  (Default|UnhideCeiling (Utilities|Array|Get(acopy) _outactors) true)
  (Default|HideUI (Utilities|Array|Get(acopy) _outactors) "Visible")
  (Game|Player|SetViewTargetwithBlend _returnvalue (Utilities|Array|Get(acopy) _outactors) 0.7 "VTBlend_Linear" 0.0 false)
  (Utilities|FlowControl|Delay 0.7)
  (Pawn|Possess _returnvalue (Utilities|Array|Get(acopy) _outactors)))

(event EventBeginPlay
  (Utilities|FlowControl|Sequence
    (:then_0
      (bind _aswb_mat_changer_ui (Utilities|Casting|CastToWB_MatChangerUI (UserInterface|GetWidget (Variables|Default|GetWidget))))
      (Default|SetTypeOfBP _aswb_mat_changer_ui (Variables|Default|GetText) (Variables|Default|GetIn%20Style) self))
    (:then_1
      (CallFunction|ToggleMenu)
      (Widget|SetVisibility (Variables|Default|GetMatsMenuReference) "Collapsed"))))

(event EventTick
  (params (DeltaSeconds :type Float%20%28single-precision%29)))

(event EventChangeMats
  (params (Index :type Integer))
  (for _array_element (Variables|Default|GetMeshes)
    (for (_array_element_2 _array_index) (Utilities|Struct|BreakMatStruct (Utilities|Array|Get(acopy) (Variables|Default|GetMats) Index))
      (Rendering|Material|SetMaterial (Variables|/Script/Engine.StaticMeshActor|GetStaticMeshComponent _array_element) _array_index _array_element_2))))

(fn ConstructionScript)

(fn ToggleMenu
  (bind _returnvalue (UserInterface|CreateWidget "/Game/_showroom/Bps/WB_Mats.WB_Mats_C"))
  (bind _output_get (Variables|Default|SetMatsMenuReference _returnvalue))
  (UserInterface|Viewport|AddtoViewport _output_get 0))

(fn SetMenu
  (bind _matsmenureference (Variables|Default|GetMatsMenuReference))
  (Default|SetParentandMats _matsmenureference (Variables|Default|GetMats) self)
  (Default|SetMats _matsmenureference))