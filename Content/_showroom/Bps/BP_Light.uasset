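; BP_Light is a showroom light actor whose spotlight can be switched on and off.
; On BeginPlay it passes itself to the WB_Dot widget hosted in its Widget component, giving that widget a reference to the light.
; Its Interact event toggles the SpotLight's visibility based on the current state, without propagating to child components.
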(event EventBeginPlay
  (bind _aswb_dot (Utilities|Casting|CastToWB_Dot (UserInterface|GetWidget (Variables|Default|GetWidget))))
  (Default|SetLight _aswb_dot self))

(event EventInteract
  (bind _spotlight (Variables|Default|GetSpotLight))
  (if (Variables|/Script/Engine.SceneComponent|GetbVisible _spotlight)
    (Rendering|SetVisibility _spotlight false false)
    (else
      (Rendering|SetVisibility _spotlight true false))))

(fn ConstructionScript)