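; Showroom actor that displays a configurable static mesh and swaps between indexed sets of materials.
; The construction script assigns the chosen mesh to its StaticMesh component.
; ChangeMats picks a material set from Mats by index and applies it slot by slot to the StaticMesh of every entry in Meshes.
; Only when Meshes is empty does it apply the set to its own mesh, through the ChageMaterials function.
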(event EventBeginPlay)

(event Collision|EventActorBeginOverlap
  (params (OtherActor :type Actor%20Object%20Reference)))

(event EventTick
  (params (DeltaSeconds :type Float%20%28single-precision%29)))

(event EventChangeMats
  (params (Index :type Integer))
  (bind _mats (Variables|Default|GetMats))
  (bind _output (Utilities|Array|Get(acopy) _mats Index))
  (bind _materials (Utilities|Struct|BreakMatStruct _output))
  (if (Utilities|Array|IsNotEmpty (Variables|Default|GetMeshes))
    (for _array_element (Variables|Default|GetMeshes)
      (for (_array_element_2 _array_index) _materials
        (Rendering|Material|SetMaterial (Variables|BP_Changer_C|GetStaticMesh _array_element) _array_index _array_element_2)))
    (else
      (CallFunction|ChageMaterials _materials))))

(fn ConstructionScript
  (Components|StaticMesh|SetStaticMesh (Variables|Default|GetStaticMesh) (Variables|Default|GetMesh)))

(fn ChageMaterials
  (params (Array :type Array%20of%20Material%20Instance%20Object%20References))
  (for (_array_element _array_index) Array
    (Rendering|Material|SetMaterial (Variables|Default|GetStaticMesh) _array_index _array_element)))