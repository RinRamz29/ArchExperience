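; BP_Label is a showroom actor that shows a text label while the first-person character stands in its trigger box.
; On BeginPlay it hides its widget component and pushes its TextForLabel value into the WB_Label widget.
; Box overlap begin and end events, filtered to BP_FirstPersonCharacter, toggle the widget's visibility on and off.
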(event OnComponentBeginOverlap(Box)
  (params (OverlappedComponent :type Primitive%20Component%20Object%20Reference) (OtherActor :type Actor%20Object%20Reference) (OtherComp :type Primitive%20Component%20Object%20Reference) (OtherBodyIndex :type Integer) (bFromSweep :type Boolean) (SweepResult :type Hit%20Result%20Structure%20%28by%20ref%29))
  (Utilities|Casting|CastToBP_FirstPersonCharacter OtherActor)
  (Rendering|SetVisibility (Variables|Default|GetWidget) true true))

(event OnComponentEndOverlap(Box)
  (params (OverlappedComponent :type Primitive%20Component%20Object%20Reference) (OtherActor :type Actor%20Object%20Reference) (OtherComp :type Primitive%20Component%20Object%20Reference) (OtherBodyIndex :type Integer))
  (Utilities|Casting|CastToBP_FirstPersonCharacter OtherActor)
  (Rendering|SetVisibility (Variables|Default|GetWidget) false true))

(event EventBeginPlay
  (Rendering|SetVisibility (Variables|Default|GetWidget) false true)
  (bind _aswb_label (Utilities|Casting|CastToWB_Label (UserInterface|GetWidget (Variables|Default|GetWidget))))
  (Default|SetText _aswb_label (Variables|Default|GetTextForLabel)))

(fn ConstructionScript)