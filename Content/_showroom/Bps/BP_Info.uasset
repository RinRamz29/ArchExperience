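; BP_Info is a showroom info point that shows a text panel when the VR player comes near it.
; On BeginPlay it spawns an InfoUI actor targeted at its root, fills the WB_Info widget with its short and long texts, and registers it on the VRPawn.
; Tick measures distance to the VR origin, opening the menu once within range and closing it and resetting the DoOnce outside.
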(event EventTick
  (params (DeltaSeconds :type Float%20%28single-precision%29))
  (bind _infoui (Variables|Default|GetInfoUI))
  (if (<= (Math|Vector|VectorLength (- (Transformation|GetWorldLocation (Variables|/Game/VRTemplate/Blueprints/VRPawn.VRPawn_C|GetVROrigin (Variables|Default|GetPlayer))) (Transformation|GetWorldLocation (Variables|Default|GetDefaultSceneRoot)))) 5e+02)
    (Utilities|FlowControl|DoOnce false :!label _label
      (:Completed
        (Default|OpenMenu _infoui)))
    (else
      (Utilities|FlowControl|Sequence
        (:then_0
          (Default|CloseMenu _infoui))
        (:then_1
          (goto _label Reset))))))

(event EventBeginPlay
  (Utilities|FlowControl|Sequence
    (:then_0
      (bind _asvrpawn (Utilities|Casting|CastToVRPawn (Game|Player|GetPlayerPawn 0)))
      (Variables|Default|SetPlayer _asvrpawn))
    (:then_1
      (bind _returnvalue (Game|SpawnActorfromClass "/Game/_showroom/Bps/InfoUI.InfoUI_C" (Math|Transform|MakeTransform "0, 0, 0" "0, 0, 0" "1.000000,1.000000,1.000000") "Undefined" "MultiplyWithRoot" 0 true 0))
      (bind _output_get (Variables|Default|SetInfoUI _returnvalue))
      (Variables|/Game/_showroom/Bps/InfoUI.InfoUI_C|SetTarget _output_get (Variables|Default|GetDefaultSceneRoot))
      (Default|CloseMenu _output_get)
      (bind _aswb_info (Utilities|Casting|CastToWB_Info (UserInterface|GetWidget (Variables|/Game/_showroom/Bps/InfoUI.InfoUI_C|GetWidget _output_get))))
      (Default|SetText _aswb_info (Variables|Default|GetInfoShort) (Variables|Default|GetInfoLong)))
    (:then_2
      (Variables|/Game/VRTemplate/Blueprints/VRPawn.VRPawn_C|SetInfo%20UI (Variables|Default|GetPlayer) (Variables|Default|GetInfoUI)))))

(fn ConstructionScript)