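; BP_InfoPlaque is a configurable info plaque prop from the interior building kit, showing text on a plate mesh.
; Its construction script applies variables for text, text size and lateral text offset to the text render component, nudged slightly along X.
; It also sets the plate's static mesh and first material slot from variables.
; It has no runtime logic, as the event graph holds only disabled stub events.
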(event EventBeginPlay)

(event Collision|EventActorBeginOverlap
  (params (OtherActor :type Actor%20Object%20Reference)))

(event EventTick
  (params (DeltaSeconds :type Float%20%28single-precision%29)))

(fn ConstructionScript
  (Transformation|SetRelativeLocation (Variables|Default|GetTextRender) (Math|Vector|MakeVector 0.75 (Variables|Default|GetText%20Location%20offset) 0.0) false false)
  (Rendering|Components|TextRender|SetWorldSize (Variables|Default|GetTextRender) (Variables|Default|GetText%20Size))
  (Rendering|Components|TextRender|SetText (Variables|Default|GetTextRender) (Variables|Default|GetText))
  (Components|StaticMesh|SetStaticMesh (Variables|Default|GetSM_InfoPlate) (Variables|Default|GetNew%20Plaque%20Mesh))
  (Rendering|Material|SetMaterial (Variables|Default|GetSM_InfoPlate) 0 (Variables|Default|GetPlaque%20Material)))