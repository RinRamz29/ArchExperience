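; BP_Bed is a configurable bed prop, assembled entirely in its construction script from data tables.
; Frame type, bed size and variation indices pick meshes for frame, optional boxspring, mattress, pillows and blanket, falling back to the last row.
; Height values stack and Z-scale the layers, while per-size XY scales fit three mesh classes to nine bed sizes.
; Pillows can randomize materials, and a dynamic blanket material receives bounds and offsets from the assembled bed.
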(event EventBeginPlay)

(event Collision|EventActorBeginOverlap
  (params (OtherActor :type Actor%20Object%20Reference)))

(event EventTick
  (params (DeltaSeconds :type Float%20%28single-precision%29)))

(fn ConstructionScript
  (bind _returnvalue (Math|Random|RandomIntegerinRange 0 9))
  (bind _bed_size (Variables|Default|GetBed%20Size))
  (bind _bed_size_2 (Variables|Default|GetBed%20Size))
  (bind _mattress (Variables|Default|GetMattress))
  (bind _boxspring (Variables|Default|GetBoxspring))
  (bind _sm_bedframe (Variables|Default|GetSM_Bedframe))
  (bind _sm_pillow_02 (Variables|Default|GetSM_Pillow_02))
  (bind _sm_pillow_01 (Variables|Default|GetSM_Pillow_01))
  (bind _bed_size_3 (Variables|Default|GetBed%20Size))
  (bind _bed_size_4 (Variables|Default|GetBed%20Size))
  (bind _bed_size_5 (Variables|Default|GetBed%20Size))
  (bind _pillow_2___override_material (Variables|Default|GetPillow%202%20-%20Override%20Material))
  (bind _pillow_1___override_material (Variables|Default|GetPillow%201%20-%20Override%20Material))
  (bind _bedframe_material (Variables|Default|GetBedframe%20Material))
  (bind _blankets_material (Variables|Default|GetBlankets%20Material))
  (bind (_min _max) (Components|StaticMesh|GetLocalBounds _sm_bedframe))
  (bind _returnvalue_2 (Utilities|Select :Index _returnvalue :Option%200 "/Game/InteriorBuildingKit/Material/Bed/Pillows/MI_Pillow_01.MI_Pillow_01" :Option%201 "/Game/InteriorBuildingKit/Material/Bed/Pillows/MI_Pillow_02.MI_Pillow_02" :Option%202 "/Game/InteriorBuildingKit/Material/Bed/Pillows/MI_Pillow_03.MI_Pillow_03" :Option%203 "/Game/InteriorBuildingKit/Material/Bed/Pillows/MI_Pillow_04.MI_Pillow_04" :Option%204 "/Game/InteriorBuildingKit/Material/Bed/Pillows/MI_Pillow_05.MI_Pillow_05" :Option%205 "/Game/InteriorBuildingKit/Material/Bed/Pillows/MI_Pillow_06.MI_Pillow_06" :Option%206 "/Game/InteriorBuildingKit/Material/Bed/Pillows/MI_Pillow_07.MI_Pillow_07" :Option%207 "/Game/InteriorBuildingKit/Material/Bed/Pillows/MI_Pillow_08.MI_Pillow_08" :Option%208 "/Game/InteriorBuildingKit/Material/Bed/Pillows/MI_Pillow_09.MI_Pillow_09" :Option%209 "/Game/InteriorBuildingKit/Material/Bed/Pillows/MI_Pillow_10.MI_Pillow_10"))
  (bind _returnvalue_3 (Utilities|Select :Index _bed_size :NewEnumerator0 0.79 :NewEnumerator1 1.0 :NewEnumerator2 1.0 :NewEnumerator3 0.9 :NewEnumerator4 0.9 :NewEnumerator5 1.0 :NewEnumerator6 0.912 :NewEnumerator7 1.055 :NewEnumerator8 1.0))
  (bind _returnvalue_4 (Utilities|Select :Index _bed_size_2 :NewEnumerator0 0.935 :NewEnumerator1 0.935 :NewEnumerator2 1.0 :NewEnumerator3 0.935 :NewEnumerator4 1.0 :NewEnumerator5 1.0 :NewEnumerator6 0.95 :NewEnumerator7 0.95 :NewEnumerator8 1.0))
  (bind _returnvalue_5 (- _max _min))
  (switch Utilities|FlowControl|Switch|SwitchonBedFrameTypes_Enum (Variables|Default|GetBedframe%20Type)
    (:NewEnumerator1
      (bind _outrownames (DataTable|GetDataTableRowNames "/Game/InteriorBuildingKit/Struct/BedFrame_Wooden_DataTable.BedFrame_Wooden_DataTable"))
      (bind _returnvalue_6 (Utilities|GetDataTableRow "/Game/InteriorBuildingKit/Struct/BedFrame_Wooden_DataTable.BedFrame_Wooden_DataTable" (Utilities|Array|Get(acopy) _outrownames (Variables|Default|GetFrame%20Variation%20Option)) :!label _label)
        (:then
          (Components|StaticMesh|SetStaticMesh (Variables|Default|GetSM_Bedframe) (Utilities|Select :Index (Variables|Default|GetBed%20Size) :NewEnumerator0 (.smallframe _returnvalue_6) :NewEnumerator1 (.smallframe _returnvalue_6) :NewEnumerator2 (.smallframe _returnvalue_6) :NewEnumerator3 (.mediumframe _returnvalue_6) :NewEnumerator4 (.mediumframe _returnvalue_6) :NewEnumerator5 (.mediumframe _returnvalue_6) :NewEnumerator6 (.largeframe _returnvalue_6) :NewEnumerator7 (.largeframe _returnvalue_6) :NewEnumerator8 (.largeframe _returnvalue_6)))
          (bind _output_get (Variables|StoredVariables|SetBedframe%20Height (.frameheight _returnvalue_6)))
          (Transformation|SetRelativeLocation (Variables|Default|GetBoxspring%20Height) (Math|Vector|MakeVector 0.0 0.0 _output_get) false true))
        (:RowNotFound
          (Variables|Default|SetFrame%20Variation%20Option (- (Utilities|Array|Length _outrownames) 1))
          (goto _label))))
    (:NewEnumerator0
      (bind _outrownames_2 (DataTable|GetDataTableRowNames "/Game/InteriorBuildingKit/Struct/BedFrame_Metallic_DataTable.BedFrame_Metallic_DataTable"))
      (bind _returnvalue_7 (Utilities|GetDataTableRow "/Game/InteriorBuildingKit/Struct/BedFrame_Metallic_DataTable.BedFrame_Metallic_DataTable" (Utilities|Array|Get(acopy) _outrownames_2 (Variables|Default|GetFrame%20Variation%20Option)) :!label _label_2)
        (:then
          (Components|StaticMesh|SetStaticMesh (Variables|Default|GetSM_Bedframe) (Utilities|Select :Index (Variables|Default|GetBed%20Size) :NewEnumerator0 (.smallframe _returnvalue_7) :NewEnumerator1 (.smallframe _returnvalue_7) :NewEnumerator2 (.smallframe _returnvalue_7) :NewEnumerator3 (.mediumframe _returnvalue_7) :NewEnumerator4 (.mediumframe _returnvalue_7) :NewEnumerator5 (.mediumframe _returnvalue_7) :NewEnumerator6 (.largeframe _returnvalue_7) :NewEnumerator7 (.largeframe _returnvalue_7) :NewEnumerator8 (.largeframe _returnvalue_7)))
          (bind _output_get_2 (Variables|StoredVariables|SetBedframe%20Height (.frameheight _returnvalue_7)))
          (Transformation|SetRelativeLocation (Variables|Default|GetBoxspring%20Height) (Math|Vector|MakeVector 0.0 0.0 _output_get_2) false true))
        (:RowNotFound
          (Variables|Default|SetFrame%20Variation%20Option (- (Utilities|Array|Length _outrownames_2) 1))
          (goto _label_2)))))
  (Utilities|IsValid _bedframe_material
    (:Is%20Valid
      (Rendering|Material|SetMaterial (Variables|Default|GetSM_Bedframe) (Variables|Default|GetBedframe%20Material%20ID%20channel) _bedframe_material))
    (:Is%20Not%20Valid
      _))
  (if (Variables|Default|GetUse%20Boxspring?)
    (bind _outrownames_3 (DataTable|GetDataTableRowNames "/Game/InteriorBuildingKit/Struct/Boxsprings_DataTable.Boxsprings_DataTable"))
    (bind _returnvalue_8 (Utilities|GetDataTableRow "/Game/InteriorBuildingKit/Struct/Boxsprings_DataTable.Boxsprings_DataTable" (Utilities|Array|Get(acopy) _outrownames_3 (Variables|Default|GetBoxspring%20Variation%20Option)) :!label _label_3)
      (:then
        (Components|StaticMesh|SetStaticMesh _boxspring (Utilities|Select :Index (Variables|Default|GetBed%20Size) :NewEnumerator0 (.smallboxspring _returnvalue_8) :NewEnumerator1 (.smallboxspring _returnvalue_8) :NewEnumerator2 (.smallboxspring _returnvalue_8) :NewEnumerator3 (.mediumboxspring _returnvalue_8) :NewEnumerator4 (.mediumboxspring _returnvalue_8) :NewEnumerator5 (.mediumboxspring _returnvalue_8) :NewEnumerator6 (.largeboxspring _returnvalue_8) :NewEnumerator7 (.largeboxspring _returnvalue_8) :NewEnumerator8 (.largeboxspring _returnvalue_8)))
        (Transformation|SetRelativeScale3D _boxspring (Math|Vector|MakeVector 1.0 1.0 (/ (Variables|Default|GetBoxspring%20Height%20in%20Cm) (.boxspringheight _returnvalue_8))))
        (Transformation|SetRelativeLocation (Variables|Default|GetMattress%20Height) (Math|Vector|MakeVector 0.0 0.0 (+ (Variables|Default|GetBoxspring%20Height%20in%20Cm) (Variables|StoredVariables|GetBedframe%20Height))) false true))
      (:RowNotFound
        (Variables|Default|SetBoxspring%20Variation%20Option (- (Utilities|Array|Length _outrownames_3) 1))
        (goto _label_3)))
    (else
      (Components|DestroyComponent (Variables|Default|GetBoxspring))
      (Transformation|SetRelativeLocation (Variables|Default|GetMattress%20Height) (Math|Vector|MakeVector 0.0 0.0 (Variables|StoredVariables|GetBedframe%20Height)) false true)))
  (bind _outrownames_4 (DataTable|GetDataTableRowNames "/Game/InteriorBuildingKit/Struct/Mattress_DataTable.Mattress_DataTable"))
  (bind _returnvalue_9 (Utilities|GetDataTableRow "/Game/InteriorBuildingKit/Struct/Mattress_DataTable.Mattress_DataTable" (Utilities|Array|Get(acopy) _outrownames_4 (Variables|Default|GetMattress%20Variation%20Option)) :!label _label_4)
    (:then
      (Components|StaticMesh|SetStaticMesh _mattress (select (Variables|Default|GetUse%20Fitted%20Sheet?) (Utilities|Select :Index (Variables|Default|GetBed%20Size) :NewEnumerator0 (.smallfittedsheet _returnvalue_9) :NewEnumerator1 (.smallfittedsheet _returnvalue_9) :NewEnumerator2 (.smallfittedsheet _returnvalue_9) :NewEnumerator3 (.mediumfittedsheet _returnvalue_9) :NewEnumerator4 (.mediumfittedsheet _returnvalue_9) :NewEnumerator5 (.mediumfittedsheet _returnvalue_9) :NewEnumerator6 (.largefittedsheet _returnvalue_9) :NewEnumerator7 (.largefittedsheet _returnvalue_9) :NewEnumerator8 (.largefittedsheet _returnvalue_9)) (Utilities|Select :Index (Variables|Default|GetBed%20Size) :NewEnumerator0 (.smallmattress _returnvalue_9) :NewEnumerator1 (.smallmattress _returnvalue_9) :NewEnumerator2 (.smallmattress _returnvalue_9) :NewEnumerator3 (.mediummattress _returnvalue_9) :NewEnumerator4 (.mediummattress _returnvalue_9) :NewEnumerator5 (.mediummattress _returnvalue_9) :NewEnumerator6 (.largemattress _returnvalue_9) :NewEnumerator7 (.largemattress _returnvalue_9) :NewEnumerator8 (.largemattress _returnvalue_9))))
      (Transformation|SetRelativeScale3D _mattress (Math|Vector|MakeVector 1.0 1.0 (/ (Variables|Default|GetMattress%20Height%20in%20Cm) (.mattressheight _returnvalue_9))))
      (Transformation|SetRelativeLocation (Variables|Default|GetBlanket%20Height) (Math|Vector|MakeVector 0.0 0.0 (Variables|Default|GetMattress%20Height%20in%20Cm)) false true)
      (bind _outrownames_5 (DataTable|GetDataTableRowNames "/Game/InteriorBuildingKit/Struct/BedPillows_DataTable.BedPillows_DataTable"))
      (bind _returnvalue_10 (Utilities|GetDataTableRow "/Game/InteriorBuildingKit/Struct/BedPillows_DataTable.BedPillows_DataTable" (Utilities|Array|Get(acopy) _outrownames_5 (Variables|Default|GetPillow1%20Variation%20Option)) :!label _label_5)
        (:then
          (Components|StaticMesh|SetStaticMesh _sm_pillow_01 (.geometry _returnvalue_10))
          (Rendering|Material|SetMaterial _sm_pillow_01 0 (select (and (not (Utilities|IsValid _pillow_1___override_material)) (Variables|Default|GetPillow%201%20-%20Randomize%20Default%20Pillow%20Material?)) _returnvalue_2 _pillow_1___override_material))
          (bind _returnvalue_11 (Utilities|GetDataTableRow "/Game/InteriorBuildingKit/Struct/BedPillows_DataTable.BedPillows_DataTable" (Utilities|Array|Get(acopy) _outrownames_5 (Variables|Default|GetPillow2%20Variation%20Option)) :!label _label_6)
            (:then
              (Components|StaticMesh|SetStaticMesh _sm_pillow_02 (.geometry _returnvalue_11))
              (Rendering|Material|SetMaterial _sm_pillow_02 0 (select (and (not (Utilities|IsValid _pillow_2___override_material)) (Variables|Default|GetPillow%202%20-%20Randomize%20Default%20Pillow%20Material?)) _returnvalue_2 _pillow_2___override_material))
              (bind _outrownames_6 (DataTable|GetDataTableRowNames "/Game/InteriorBuildingKit/Struct/BedBlankets_DataTable.BedBlankets_DataTable"))
              (bind _returnvalue_12 (Utilities|GetDataTableRow "/Game/InteriorBuildingKit/Struct/BedBlankets_DataTable.BedBlankets_DataTable" (Utilities|Array|Get(acopy) _outrownames_6 (Variables|Default|GetBlanket%20Variation%20Option)) :!label _label_7)
                (:then
                  (Components|StaticMesh|SetStaticMesh (Variables|Default|GetBlanket) (Utilities|Select :Index (Variables|Default|GetBed%20Size) :NewEnumerator0 (.smallblanket _returnvalue_12) :NewEnumerator1 (.smallblanket _returnvalue_12) :NewEnumerator2 (.smallblanket _returnvalue_12) :NewEnumerator3 (.mediumblanket _returnvalue_12) :NewEnumerator4 (.mediumblanket _returnvalue_12) :NewEnumerator5 (.mediumblanket _returnvalue_12) :NewEnumerator6 (.largeblanket _returnvalue_12) :NewEnumerator7 (.largeblanket _returnvalue_12) :NewEnumerator8 (.largeblanket _returnvalue_12)))
                  (Utilities|FlowControl|Sequence
                    (:then_0
                      (if (Math|Boolean|ORBoolean (Utilities|Enum|Equal(Enum) _bed_size_4 "NewEnumerator0") (Utilities|Enum|Equal(Enum) _bed_size_4 "NewEnumerator1") (Utilities|Enum|Equal(Enum) _bed_size_4 "NewEnumerator2"))
                        (Transformation|SetRelativeLocation (Variables|Default|GetSM_Pillow_01) "0, 0, 0" false false)
                        (Components|DestroyComponent (Variables|Default|GetSM_Pillow_02))
                        (if (Variables|Default|GetUse%20Left%20Pillow%20-%20Main) :!label _label_8
                          _
                          (else
                            (Components|DestroyComponent (Variables|Default|GetSM_Pillow_01))))
                        (if (Variables|Default|GetUse%20Right%20Pillow%20-%20Main)
                          _
                          (else
                            (Components|DestroyComponent (Variables|Default|GetSM_Pillow_02))))
                        (if (Variables|Default|GetUse%20Blanket?)
                          _
                          (else
                            (Components|DestroyComponent (Variables|Default|GetBlanket))))
                        ;[1 1 1] Tweaks the scale to fit the desired bed size
                        (Transformation|SetRelativeScale3D (Variables|Default|GetSM_Bedframe) (Math|Vector|MakeVector _returnvalue_3 _returnvalue_4 1.0))
                        (bind _returnvalue_13 (Rendering|Material|CreateDynamicMaterialInstance (select (Utilities|IsValid _blankets_material) _blankets_material "/Game/InteriorBuildingKit/Material/Bed/Blankets/MI_BedBlanket_01.MI_BedBlanket_01") "None" "None" :!class /Script/Engine.KismetMaterialLibrary))
                        (bind _output_get_3 (Variables|StoredVariables|SetDynamic%20Material%20Instance _returnvalue_13))
                        (Rendering|Material|SetMaterial (Variables|Default|GetBlanket) 0 _output_get_3)
                        (Rendering|Material|SetVectorParameterValue _output_get_3 "Bounds" (Utilities|Struct|MakeLinearColor (* (.x _returnvalue_5) _returnvalue_3 3.0) (* (.y _returnvalue_5) _returnvalue_4 5.0) (* (Variables|StoredVariables|GetBedframe%20Height) 2.0) 1.0) :!class /Script/Engine.MaterialInstanceDynamic)
                        (Rendering|Material|SetVectorParameterValue _output_get_3 "Position Offset" (Utilities|Struct|MakeLinearColor 0.0 0.0 (+ (Variables|StoredVariables|GetBedframe%20Height) (select (Variables|Default|GetUse%20Boxspring?) (Variables|Default|GetBoxspring%20Height%20in%20Cm) 0.0) (Variables|Default|GetMattress%20Height%20in%20Cm)) 1.0) :!class /Script/Engine.MaterialInstanceDynamic)
                        (Rendering|Material|SetScalarParameterValue _output_get_3 "Offset Strength - Sides" (Variables|Default|GetBlanket%20Offsets%20-%20Side) :!class /Script/Engine.MaterialInstanceDynamic)
                        (Rendering|Material|SetScalarParameterValue _output_get_3 "Offset Strength - Bottom" (Variables|Default|GetBlanket%20Offsets%20-%20Bottom) :!class /Script/Engine.MaterialInstanceDynamic)))
                    (:then_1
                      (if (Math|Boolean|ORBoolean (Utilities|Enum|Equal(Enum) _bed_size_5 "NewEnumerator3") (Utilities|Enum|Equal(Enum) _bed_size_5 "NewEnumerator4") (Utilities|Enum|Equal(Enum) _bed_size_5 "NewEnumerator5"))
                        (Transformation|SetRelativeLocation (Variables|Default|GetSM_Pillow_01) "-35.000000, 0, 0" false false)
                        (Transformation|SetRelativeLocation (Variables|Default|GetSM_Pillow_02) "35.000000, 0, 0" false false)
                        (goto _label_8)))
                    (:then_2
                      (if (Math|Boolean|ORBoolean (Utilities|Enum|Equal(Enum) _bed_size_3 "NewEnumerator6") (Utilities|Enum|Equal(Enum) _bed_size_3 "NewEnumerator7") (Utilities|Enum|Equal(Enum) _bed_size_3 "NewEnumerator8"))
                        (Transformation|SetRelativeLocation (Variables|Default|GetSM_Pillow_01) "-40.000000, 0, 0" false false)
                        (Transformation|SetRelativeLocation (Variables|Default|GetSM_Pillow_02) "40.000000, 0, 0" false false)
                        (goto _label_8)))))
                (:RowNotFound
                  (Variables|Default|SetBlanket%20Variation%20Option (- (Utilities|Array|Length _outrownames_6) 1))
                  (goto _label_7))))
            (:RowNotFound
              (Variables|Default|SetPillow2%20Variation%20Option (- (Utilities|Array|Length _outrownames_5) 1))
              (goto _label_6))))
        (:RowNotFound
          (Variables|Default|SetPillow1%20Variation%20Option (- (Utilities|Array|Length _outrownames_5) 1))
          (goto _label_5))))
    (:RowNotFound
      (Variables|Default|SetMattress%20Variation%20Option (- (Utilities|Array|Length _outrownames_4) 1))
      (goto _label_4))))