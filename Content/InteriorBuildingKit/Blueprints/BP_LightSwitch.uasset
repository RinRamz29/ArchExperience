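; Configurable wall light switch prop from the interior building kit, with a single, double or triple plate.
; The Construction Script picks the plate mesh from NumberOfSwitches, spaces the rockers across it and destroys unused rocker components.
; Each rocker's roll is tilted up or down from its SwitchOn boolean.
; The visuals are construction-time only: no runtime logic or light control exists in these graphs.
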(event EventBeginPlay)

(event Collision|EventActorBeginOverlap
  (params (OtherActor :type Actor%20Object%20Reference)))

(event EventTick
  (params (DeltaSeconds :type Float%20%28single-precision%29)))

(fn ConstructionScript
  (Components|StaticMesh|SetStaticMesh (Variables|Default|GetSM_LightSwitch_Single) (Utilities|Select :Index (Variables|Default|GetNumber%20of%20switches) :Option%200 "/Game/InteriorBuildingKit/Geometry/Assets/WallDetails/SM_LightSwitch_Single.SM_LightSwitch_Single" :Option%201 "/Game/InteriorBuildingKit/Geometry/Assets/WallDetails/SM_LightSwitch_Single.SM_LightSwitch_Single" :Option%202 "/Game/InteriorBuildingKit/Geometry/Assets/WallDetails/SM_LightSwitch_Double.SM_LightSwitch_Double" :Option%203 "/Game/InteriorBuildingKit/Geometry/Assets/WallDetails/SM_LightSwitch_Tripple.SM_LightSwitch_Tripple"))
  (Utilities|FlowControl|Sequence
    (:then_0
      (if (== (Variables|Default|GetNumber%20of%20switches) 1)
        (Transformation|SetRelativeLocation (Variables|Default|GetSM_LightSwitch%201) "0, 0, 0" false false)
        (Components|DestroyComponent (Variables|Default|GetSM_LightSwitch%202))
        (Transformation|SetRelativeRotation (Variables|Default|GetSM_LightSwitch%201) (Math|Rotator|MakeRotator (Math|Float|SelectFloat -35.0 35.0 (Variables|Default|GetSwitch%201%20On?)) 0.0 0.0) false false)))
    (:then_1
      (if (== (Variables|Default|GetNumber%20of%20switches) 2)
        (Transformation|SetRelativeLocation (Variables|Default|GetSM_LightSwitch%201) "-2.500000, 0, 0" false false)
        (Transformation|SetRelativeLocation (Variables|Default|GetSM_LightSwitch%202) "2.500000, 0, 0" false false)
        (Components|DestroyComponent (Variables|Default|GetSM_LightSwitch%203))
        (Transformation|SetRelativeRotation (Variables|Default|GetSM_LightSwitch%201) (Math|Rotator|MakeRotator (Math|Float|SelectFloat -35.0 35.0 (Variables|Default|GetSwitch%201%20On?)) 0.0 0.0) false false)
        (Transformation|SetRelativeRotation (Variables|Default|GetSM_LightSwitch%202) (Math|Rotator|MakeRotator (Math|Float|SelectFloat -35.0 35.0 (Variables|Default|GetSwitch%202%20On?)) 0.0 0.0) false false)))
    (:then_2
      (if (== (Variables|Default|GetNumber%20of%20switches) 3)
        (Transformation|SetRelativeLocation (Variables|Default|GetSM_LightSwitch%201) "-5.000000, 0, 0" false false)
        (Transformation|SetRelativeLocation (Variables|Default|GetSM_LightSwitch%202) "0, 0, 0" false false)
        (Transformation|SetRelativeLocation (Variables|Default|GetSM_LightSwitch%203) "5.000000, 0, 0" false false)
        (Transformation|SetRelativeRotation (Variables|Default|GetSM_LightSwitch%201) (Math|Rotator|MakeRotator (Math|Float|SelectFloat -35.0 35.0 (Variables|Default|GetSwitch%201%20On?)) 0.0 0.0) false false)
        (Transformation|SetRelativeRotation (Variables|Default|GetSM_LightSwitch%202) (Math|Rotator|MakeRotator (Math|Float|SelectFloat -35.0 35.0 (Variables|Default|GetSwitch%202%20On?)) 0.0 0.0) false false)
        (Transformation|SetRelativeRotation (Variables|Default|GetSM_LightSwitch%203) (Math|Rotator|MakeRotator (Math|Float|SelectFloat -35.0 35.0 (Variables|Default|GetSwitch%203%20On?)) 0.0 0.0) false false)))))