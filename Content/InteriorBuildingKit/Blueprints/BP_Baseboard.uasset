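; Interior kit baseboard actor that builds trim along an editable list of Destination points in its construction script.
; Points are flattened in Z, and zeroed ones are offset from the previous point.
; Each segment takes a length-matched mesh from the TrimStyle data table row, stretched to fit and scaled by trim thickness and height.
; Optional start and end corner meshes come from the same row, with the end one mirrored.
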(event EventBeginPlay)

(event Collision|EventActorBeginOverlap
  (params (OtherActor :type Actor%20Object%20Reference)))

(event EventTick
  (params (DeltaSeconds :type Float%20%28single-precision%29)))

(fn ConstructionScript
  (bind _trim_thickness__ (Variables|Default|GetTrim%20thickness%20%25))
  (bind _destination (Variables|Default|GetDestination))
  (bind _destination_2 (Variables|Default|GetDestination))
  (bind _destination_3 (Variables|Default|GetDestination))
  (bind _destination_4 (Variables|Default|GetDestination))
  (bind _destination_5 (Variables|Default|GetDestination))
  (bind _trim_thickness___2 (Variables|Default|GetTrim%20thickness%20%25))
  (bind _destination_6 (Variables|Default|GetDestination))
  (bind _returnvalue (Utilities|Array|Length _destination))
  (bind _returnvalue_2 (Utilities|Array|Length _destination_5))
  (bind _returnvalue_3 (/ _trim_thickness___2 1e+02))
  (bind _returnvalue_4 (/ _trim_thickness__ 1e+02))
  (if (or (== _returnvalue 0) (== _returnvalue 1))
    (Utilities|Array|SetArrayElem :TargetArray _destination_2 :bSizeToFit true)
    (Utilities|Array|SetArrayElem _destination_2 1 "0,-100.000000,0" true))
  (for (_array_element _array_index) (Variables|Default|GetDestination)
    (bind _output_get (Variables|Tracking|SetArray%20Loop%20Counter _array_index))
    (Utilities|Array|SetArrayElem (Variables|Default|GetDestination) _output_get (Math|Vector|MakeVector (Math|Float|SelectFloat (.x (+ (Utilities|Array|Get(acopy) (Variables|Default|GetDestination) (Math|Integer|Clamp(Integer) (- _output_get 1) 0 (- _output_get 1))) "0,50.000000, 0")) (.X (Math|Vector|BreakVector _array_element)) (and (== (Math|Vector|VectorLength _array_element) 0.0) (> (Variables|Tracking|GetArray%20Loop%20Counter) 0))) (Math|Float|SelectFloat (.y (+ (Utilities|Array|Get(acopy) (Variables|Default|GetDestination) (Math|Integer|Clamp(Integer) (- _output_get 1) 0 (- _output_get 1))) "0,50.000000, 0")) (.Y (Math|Vector|BreakVector _array_element)) (and (== (Math|Vector|VectorLength _array_element) 0.0) (> (Variables|Tracking|GetArray%20Loop%20Counter) 0))) -0.01) true)
    (if (not (== (Variables|Tracking|GetArray%20Loop%20Counter) 0))
      (bind _outrownames (DataTable|GetDataTableRowNames "/Game/InteriorBuildingKit/Struct/BaseBoard_DataTable.BaseBoard_DataTable"))
      (bind _returnvalue_5 (Utilities|GetDataTableRow "/Game/InteriorBuildingKit/Struct/BaseBoard_DataTable.BaseBoard_DataTable" (Utilities|Array|Get(acopy) _outrownames (Variables|Default|GetTrim%20Style)) :!label _label)
        (:then
          (bind _returnvalue_6 (AddComponent|AddStaticMeshComponent false (Math|Transform|MakeTransform (Utilities|Array|Get(acopy) _destination_3 (Variables|Tracking|GetArray%20Loop%20Counter)) (Math|Rotator|CombineRotators (Math|Rotator|FindLookatRotation (Utilities|Array|Get(acopy) _destination_3 (Variables|Tracking|GetArray%20Loop%20Counter)) (Utilities|Array|Get(acopy) _destination_3 (- (Variables|Tracking|GetArray%20Loop%20Counter) 1))) "0,-90.000000, 0") "1.000000,1.000000,1.000000")))
          (Components|StaticMesh|SetStaticMesh _returnvalue_6 (Utilities|Array|Get(acopy) (.baseboardassets _returnvalue_5) (+ (Math|Conversions|ToInteger(Boolean) (> (Math|Vector|VectorLength (- (Utilities|Array|Get(acopy) _destination_3 (Variables|Tracking|GetArray%20Loop%20Counter)) (Utilities|Array|Get(acopy) _destination_3 (- (Variables|Tracking|GetArray%20Loop%20Counter) 1)))) 125.0)) (Math|Conversions|ToInteger(Boolean) (> (Math|Vector|VectorLength (- (Utilities|Array|Get(acopy) _destination_3 (Variables|Tracking|GetArray%20Loop%20Counter)) (Utilities|Array|Get(acopy) _destination_3 (- (Variables|Tracking|GetArray%20Loop%20Counter) 1)))) 175.0)) (Math|Conversions|ToInteger(Boolean) (> (Math|Vector|VectorLength (- (Utilities|Array|Get(acopy) _destination_3 (Variables|Tracking|GetArray%20Loop%20Counter)) (Utilities|Array|Get(acopy) _destination_3 (- (Variables|Tracking|GetArray%20Loop%20Counter) 1)))) 225.0)) (Math|Conversions|ToInteger(Boolean) (> (Math|Vector|VectorLength (- (Utilities|Array|Get(acopy) _destination_3 (Variables|Tracking|GetArray%20Loop%20Counter)) (Utilities|Array|Get(acopy) _destination_3 (- (Variables|Tracking|GetArray%20Loop%20Counter) 1)))) 275.0)) (Math|Conversions|ToInteger(Boolean) (> (Math|Vector|VectorLength (- (Utilities|Array|Get(acopy) _destination_3 (Variables|Tracking|GetArray%20Loop%20Counter)) (Utilities|Array|Get(acopy) _destination_3 (- (Variables|Tracking|GetArray%20Loop%20Counter) 1)))) 3.5e+02)) (Math|Conversions|ToInteger(Boolean) (> (Math|Vector|VectorLength (- (Utilities|Array|Get(acopy) _destination_3 (Variables|Tracking|GetArray%20Loop%20Counter)) (Utilities|Array|Get(acopy) _destination_3 (- (Variables|Tracking|GetArray%20Loop%20Counter) 1)))) 4.5e+02)) (Math|Conversions|ToInteger(Boolean) (> (Math|Vector|VectorLength (- (Utilities|Array|Get(acopy) _destination_3 (Variables|Tracking|GetArray%20Loop%20Counter)) (Utilities|Array|Get(acopy) _destination_3 (- (Variables|Tracking|GetArray%20Loop%20Counter) 1)))) 5.5e+02)) (Math|Conversions|ToInteger(Boolean) (> (Math|Vector|VectorLength (- (Utilities|Array|Get(acopy) _destination_3 (Variables|Tracking|GetArray%20Loop%20Counter)) (Utilities|Array|Get(acopy) _destination_3 (- (Variables|Tracking|GetArray%20Loop%20Counter) 1)))) 6.5e+02)) (Math|Conversions|ToInteger(Boolean) (> (Math|Vector|VectorLength (- (Utilities|Array|Get(acopy) _destination_3 (Variables|Tracking|GetArray%20Loop%20Counter)) (Utilities|Array|Get(acopy) _destination_3 (- (Variables|Tracking|GetArray%20Loop%20Counter) 1)))) 775.0)))))
          (Transformation|SetRelativeScale3D _returnvalue_6 (Math|Vector|MakeVector (/ (Variables|Default|GetTrim%20thickness%20%25) 1e+02) (/ (Math|Vector|VectorLength (- (Utilities|Array|Get(acopy) _destination_3 (Variables|Tracking|GetArray%20Loop%20Counter)) (Utilities|Array|Get(acopy) _destination_3 (- (Variables|Tracking|GetArray%20Loop%20Counter) 1)))) (.y (.Min (Components|StaticMesh|GetLocalBounds _returnvalue_6)))) (/ (Variables|Default|GetTrim%20Height%20%25) 1e+02)))
          (Rendering|Material|SetMaterial _returnvalue_6 0 (Variables|Default|GetMaterial)))
        (:RowNotFound
          (Variables|Default|SetTrim%20Style (- (Utilities|Array|Length _outrownames) 1))
          (goto _label)))))
  (bind _outrownames_2 (DataTable|GetDataTableRowNames "/Game/InteriorBuildingKit/Struct/BaseBoard_DataTable.BaseBoard_DataTable"))
  (bind _returnvalue_7 (Utilities|GetDataTableRow "/Game/InteriorBuildingKit/Struct/BaseBoard_DataTable.BaseBoard_DataTable" (Utilities|Array|Get(acopy) _outrownames_2 (Variables|Default|GetTrim%20Style)) :!label _label_2)
    (:then
      (Utilities|FlowControl|Sequence
        (:then_0
          (Variables|Default|SetCorner%20Type%20-%20Start (Math|Integer|Clamp(Integer) (select (>= (Variables|Default|GetCorner%20Type%20-%20Start) (Utilities|Array|Length (.baseboardcornerasset _returnvalue_7))) (- (Utilities|Array|Length (.baseboardcornerasset _returnvalue_7)) 1) (Variables|Default|GetCorner%20Type%20-%20Start)) 0 (select (>= (Variables|Default|GetCorner%20Type%20-%20Start) (Utilities|Array|Length (.baseboardcornerasset _returnvalue_7))) (- (Utilities|Array|Length (.baseboardcornerasset _returnvalue_7)) 1) (Variables|Default|GetCorner%20Type%20-%20Start))))
          (if (Variables|Default|GetApply%20corner%20at%20Start?)
            (Utilities|IsValid (Utilities|Array|Get(acopy) (.baseboardcornerasset _returnvalue_7) (Variables|Default|GetCorner%20Type%20-%20Start))
              (:Is%20Valid
                (bind _returnvalue_8 (AddComponent|AddStaticMeshComponent false (Math|Transform|MakeTransform (Utilities|Array|Get(acopy) (Variables|Default|GetDestination)) (Math|Rotator|CombineRotators (Math|Rotator|FindLookatRotation (Utilities|Array|Get(acopy) _destination_6 1) (Utilities|Array|Get(acopy) _destination_6)) "0,-90.000000, 0") (Math|Vector|MakeVector _returnvalue_4 _returnvalue_4 (/ (Variables|Default|GetTrim%20Height%20%25) 1e+02)))))
                (Components|StaticMesh|SetStaticMesh _returnvalue_8 (Utilities|Array|Get(acopy) (.baseboardcornerasset _returnvalue_7) (Variables|Default|GetCorner%20Type%20-%20Start)))
                (Rendering|Material|SetMaterial _returnvalue_8 0 (Variables|Default|GetMaterial))))))
        (:then_1
          (Variables|Default|SetCorner%20Type%20-%20End (Math|Integer|Clamp(Integer) (select (>= (Variables|Default|GetCorner%20Type%20-%20End) (Utilities|Array|Length (.baseboardcornerasset _returnvalue_7))) (- (Utilities|Array|Length (.baseboardcornerasset _returnvalue_7)) 1) (Variables|Default|GetCorner%20Type%20-%20End)) 0 (select (>= (Variables|Default|GetCorner%20Type%20-%20End) (Utilities|Array|Length (.baseboardcornerasset _returnvalue_7))) (- (Utilities|Array|Length (.baseboardcornerasset _returnvalue_7)) 1) (Variables|Default|GetCorner%20Type%20-%20End))))
          (if (Variables|Default|GetApply%20corner%20at%20End?)
            (Utilities|IsValid (Utilities|Array|Get(acopy) (.baseboardcornerasset _returnvalue_7) (Variables|Default|GetCorner%20Type%20-%20End))
              (:Is%20Valid
                (bind _returnvalue_9 (AddComponent|AddStaticMeshComponent false (Math|Transform|MakeTransform (Utilities|Array|Get(acopy) _destination_4 (- (Utilities|Array|Length _destination_4) 1)) (Math|Rotator|CombineRotators (Math|Rotator|FindLookatRotation (Utilities|Array|Get(acopy) _destination_5 (- _returnvalue_2 1)) (Utilities|Array|Get(acopy) _destination_5 (- _returnvalue_2 2))) "0,-90.000000, 0") (Math|Vector|MakeVector _returnvalue_3 (* _returnvalue_3 -1.0) (/ (Variables|Default|GetTrim%20Height%20%25) 1e+02)))))
                (Components|StaticMesh|SetStaticMesh _returnvalue_9 (Utilities|Array|Get(acopy) (.baseboardcornerasset _returnvalue_7) (Variables|Default|GetCorner%20Type%20-%20End)))
                (Rendering|Material|SetMaterial _returnvalue_9 0 (Variables|Default|GetMaterial))))))))
    (:RowNotFound
      (Variables|Default|SetTrim%20Style (- (Utilities|Array|Length _outrownames_2) 1))
      (goto _label_2))))