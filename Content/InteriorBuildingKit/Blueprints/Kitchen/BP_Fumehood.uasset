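; Kitchen fume hood prop from the interior building kit, with adjustable height and optional lighting.
; The construction script locks BaseLocation's X and Y, clamps its Z, and derives the main mesh's relative height from it.
; TurnOnLights applies the lit material to the mesh; when it is off, the script destroys the right top spot light.
; The event graph has no runtime logic.
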(event EventBeginPlay)

(event Collision|EventActorBeginOverlap
  (params (OtherActor :type Actor%20Object%20Reference)))

(event EventTick
  (params (DeltaSeconds :type Float%20%28single-precision%29)))

(fn ConstructionScript
  (Variables|Default|SetBase%20Location (Math|Vector|MakeVector 0.0 5e+01 (Math|Float|Clamp(Float) (.z (Variables|Default|GetBase%20Location)) -1.5e+02 -8e+01)))
  (Transformation|SetRelativeLocation (Variables|Default|GetSM_Fumehood1_Main) (Math|Vector|MakeVector 0.0 0.0 (+ (.z (Variables|Default|GetBase%20Location)) 8e+01)) false true)
  (if (Variables|Default|GetTurn%20on%20Lights?)
    (Rendering|Material|SetMaterial (Variables|Default|GetSM_Fumehood1_Main) 1 "/Game/InteriorBuildingKit/Material/Lighting/MI_FumehoodLights.MI_FumehoodLights")
    (else
      (Components|DestroyComponent (Variables|Default|GetSpotLight_Right%20Top)))))