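; Kitchen double-door fridge prop for the interior building kit, with four doors and six drawers posed by per-part open-state values.
; The construction script lerps door yaw and drawer slide from those values, so it has no runtime logic.
; When either upper door is open, the bulb gets a glow material and stops casting shadows; otherwise the point light is destroyed.
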(event EventBeginPlay)

(event Collision|EventActorBeginOverlap
  (params (OtherActor :type Actor%20Object%20Reference)))

(event EventTick
  (params (DeltaSeconds :type Float%20%28single-precision%29)))

(fn ConstructionScript
  (bind _sm_edisonbulbe3 (Variables|Default|GetSM_EdisonBulbe3))
  (Transformation|SetRelativeRotation (Variables|Default|GetSM_Fridge_DoubleDoor_Door_Upper%20Left) (Math|Rotator|MakeRotator 0.0 0.0 (Math|Float|Lerp 0.0 179.0 (Variables|Default|GetOpen%20State%20-%20Upper%20Left%20Door))) false false)
  (Transformation|SetRelativeRotation (Variables|Default|GetSM_Fridge_DoubleDoor_Door_Upper%20Right) (Math|Rotator|MakeRotator 0.0 0.0 (Math|Float|Lerp 0.0 -179.0 (Variables|Default|GetOpen%20State%20-%20Upper%20Right%20Door))) false false)
  (Transformation|SetRelativeRotation (Variables|Default|GetSM_Fridge_DoubleDoor_Door_Lower%20Left) (Math|Rotator|MakeRotator 0.0 0.0 (Math|Float|Lerp 0.0 179.0 (Variables|Default|GetOpen%20State%20-%20Lower%20Left%20Door))) false false)
  (Transformation|SetRelativeRotation (Variables|Default|GetSM_Fridge_DoubleDoor_Door_Lower%20Right) (Math|Rotator|MakeRotator 0.0 0.0 (Math|Float|Lerp 0.0 -179.0 (Variables|Default|GetOpen%20State%20-%20Lower%20Right%20Door))) false false)
  (Transformation|SetRelativeLocation (Variables|Default|GetSM_Fridge_DoubleDoor_DrawerL1) (Math|Vector|MakeVector 0.0 (Math|Float|Lerp 0.0 35.0 (Variables|Default|GetOpen%20State%20-%20Drawer%20Left%201)) 0.0) false true)
  (Transformation|SetRelativeLocation (Variables|Default|GetSM_Fridge_DoubleDoor_DrawerL2) (Math|Vector|MakeVector 0.0 (Math|Float|Lerp 0.0 35.0 (Variables|Default|GetOpen%20State%20-%20Drawer%20Left%202)) 15.0) false true)
  (Transformation|SetRelativeLocation (Variables|Default|GetSM_Fridge_DoubleDoor_DrawerL3) (Math|Vector|MakeVector 0.0 (Math|Float|Lerp 0.0 35.0 (Variables|Default|GetOpen%20State%20-%20Drawer%20Left%203)) 3e+01) false true)
  (Transformation|SetRelativeLocation (Variables|Default|GetSM_Fridge_DoubleDoor_DrawerR1) (Math|Vector|MakeVector 0.0 (Math|Float|Lerp 0.0 35.0 (Variables|Default|GetOpen%20State%20-%20Drawer%20Right%201)) 0.0) false true)
  (Transformation|SetRelativeLocation (Variables|Default|GetSM_Fridge_DoubleDoor_DrawerR2) (Math|Vector|MakeVector 0.0 (Math|Float|Lerp 0.0 35.0 (Variables|Default|GetOpen%20State%20-%20Drawer%20Right%202)) 15.0) false true)
  (Transformation|SetRelativeLocation (Variables|Default|GetSM_Fridge_DoubleDoor_DrawerR3) (Math|Vector|MakeVector 0.0 (Math|Float|Lerp 0.0 35.0 (Variables|Default|GetOpen%20State%20-%20Drawer%20Right%203)) 3e+01) false true)
  (if (or (> (Variables|Default|GetOpen%20State%20-%20Upper%20Left%20Door) 0.0) (> (Variables|Default|GetOpen%20State%20-%20Upper%20Right%20Door) 0.0))
    (Rendering|SetCastShadow _sm_edisonbulbe3 false)
    (Rendering|Material|SetMaterial _sm_edisonbulbe3 2 "/Game/InteriorBuildingKit/Material/Lighting/Defaults/MI_LightGlow_2500.MI_LightGlow_2500")
    (else
      (Components|DestroyComponent (Variables|Default|GetPointLight)))))