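; BP_Stove is a configurable kitchen stove prop that is posed entirely in its construction script.
; Open-state values lerp the door's rotation and slide the drawer.
; Slot indices snap each of the two racks to one of five heights, nudging the second rack to an adjacent slot if both match.
; The event graph holds only disabled placeholder events, so it adds no runtime behavior.
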(event EventBeginPlay)

(event Collision|EventActorBeginOverlap
  (params (OtherActor :type Actor%20Object%20Reference)))

(event EventTick
  (params (DeltaSeconds :type Float%20%28single-precision%29)))

(fn ConstructionScript
  (Transformation|SetRelativeRotation (Variables|Default|GetSM_Stove1_Door) (Math|Rotator|MakeRotator (Math|Float|Lerp 0.0 9e+01 (Variables|Default|GetOpen%20State%20-%20Door)) 0.0 0.0) false false)
  (Transformation|SetRelativeLocation (Variables|Default|GetSM_Stove1_Drawer) (Math|Vector|MakeVector 0.0 (Math|Float|Lerp 0.0 45.0 (Variables|Default|GetOpen%20State%20-%20Drawer)) 0.0) false false)
  (Transformation|SetRelativeLocation (Variables|Default|GetSM_Stove1_Rack1) (Math|Vector|MakeVector 0.0 0.0 (Utilities|Select :Index (Variables|Default|GetRack%201%20-%20Slot) :Option%200 51.200001 :Option%201 58.700001 :Option%202 66.0 :Option%203 73.5 :Option%204 80.849998)) false false)
  (bind _output_get (Variables|Default|SetRack%202%20-%20Slot (select (== (Variables|Default|GetRack%201%20-%20Slot) (Variables|Default|GetRack%202%20-%20Slot)) (select (== (Variables|Default|GetRack%201%20-%20Slot) 0) 1 (select (== (Variables|Default|GetRack%201%20-%20Slot) 4) 3 (+ (Variables|Default|GetRack%201%20-%20Slot) 1))) (Variables|Default|GetRack%202%20-%20Slot))))
  (Transformation|SetRelativeLocation (Variables|Default|GetSM_Stove1_Rack2) (Math|Vector|MakeVector 0.0 0.0 (Utilities|Select :Index _output_get :Option%200 51.200001 :Option%201 58.700001 :Option%202 66.0 :Option%203 73.5 :Option%204 80.849998)) false false))