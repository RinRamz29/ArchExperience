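; Configurable wall cupboard prop from an interior building kit, posed entirely in the Construction Script with no active runtime logic.
; A lights toggle either gives the under-light meshes a glow material or destroys both spotlights.
; Per-part open values drive the four doors' yaw through lerps, mirrored left to right, and slide four drawers along X.
; A mesh variable sets the books displayed.
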(event EventBeginPlay)

(event Collision|EventActorBeginOverlap
  (params (OtherActor :type Actor%20Object%20Reference)))

(event EventTick
  (params (DeltaSeconds :type Float%20%28single-precision%29)))

(fn ConstructionScript
  (if (Variables|Default|GetTurn%20on%20lights?)
    (Rendering|Material|SetMaterial (Variables|Default|GetSM_UnderLight_Right) 2 "/Game/InteriorBuildingKit/Material/Lighting/Defaults/MI_LightGlow_2500_Opaque.MI_LightGlow_2500_Opaque")
    (else
      (Components|DestroyComponent (Variables|Default|GetSpotLight_Left))))
  (Components|StaticMesh|SetStaticMesh (Variables|Default|GetSM_Books1) (Variables|Default|GetBood%20Reference))
  (Transformation|SetRelativeRotation (Variables|Default|GetSM_Cupboard%20-%20Top%20Left) (Math|Rotator|MakeRotator 0.0 0.0 (Math|Float|Lerp 0.0 1.7e+02 (Variables|Default|GetOpen%20rotation%20-%20Top%20Left%20cupboard))) false false)
  (Transformation|SetRelativeRotation (Variables|Default|GetSM_Cupboard%20-%20Top%20Right) (Math|Rotator|MakeRotator 0.0 0.0 (Math|Float|Lerp 0.0 -1.7e+02 (Variables|Default|GetOpen%20rotation%20-%20Top%20Right%20cupboard))) false false)
  (Transformation|SetRelativeRotation (Variables|Default|GetSM_Cupboard%20-%20Bottom%20Left) (Math|Rotator|MakeRotator 0.0 0.0 (Math|Float|Lerp 0.0 1.6e+02 (Variables|Default|GetOpen%20rotation%20-%20Bottom%20Left%20cupboard))) false false)
  (Transformation|SetRelativeRotation (Variables|Default|GetSM_Cupboard%20-%20Bottom%20Right) (Math|Rotator|MakeRotator 0.0 0.0 (Math|Float|Lerp 0.0 -1.6e+02 (Variables|Default|GetOpen%20rotation%20-%20Bottom%20Right%20cupboard))) false false)
  (Transformation|SetRelativeLocation (Variables|Default|GetSM_Drawer1) (Math|Vector|MakeVector (* (Variables|Default|GetOpen%20State%20-%20Drawer%201) 5e+01) 0.0 0.0) false false)
  (Transformation|SetRelativeLocation (Variables|Default|GetSM_Drawer2) (Math|Vector|MakeVector (* (Variables|Default|GetOpen%20State%20-%20Drawer%202) 5e+01) 0.0 0.0) false false)
  (Transformation|SetRelativeLocation (Variables|Default|GetSM_Drawer3) (Math|Vector|MakeVector (* (Variables|Default|GetOpen%20State%20-%20Drawer%203) 5e+01) 0.0 0.0) false false)
  (Transformation|SetRelativeLocation (Variables|Default|GetSM_Drawer4) (Math|Vector|MakeVector (* (Variables|Default|GetOpen%20State%20-%20Drawer%204) 5e+01) 0.0 0.0) false false))