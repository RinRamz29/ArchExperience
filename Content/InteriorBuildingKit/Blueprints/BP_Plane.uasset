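; BP_Plane is a construction-time plane actor in the interior building kit, sized by a Location vector.
; The construction script zeroes the vector's Z and divides X and Y by 100 to scale the PlaneCorner mesh, with a fixed Z scale.
; A LightmassResolution setting picks among mesh variants named by resolution, and the chosen material is applied to the first slot.
; The event graph holds no active logic.
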(event EventBeginPlay)

(event Collision|EventActorBeginOverlap
  (params (OtherActor :type Actor%20Object%20Reference)))

(event EventTick
  (params (DeltaSeconds :type Float%20%28single-precision%29)))

(fn ConstructionScript
  (Variables|Default|SetLocation (Math|Vector|MakeVector (.x (Variables|Default|GetLocation)) (.y (Variables|Default|GetLocation)) 0.0))
  (Components|StaticMesh|SetStaticMesh (Variables|Default|GetPlane_Corner) (Utilities|Select :Index (Variables|Default|GetLightmass%20resolution) :NewEnumerator5 "/Game/InteriorBuildingKit/Geometry/Assets/Shapes/SM_PlaneCorner_32.SM_PlaneCorner_32" :NewEnumerator4 "/Game/InteriorBuildingKit/Geometry/Assets/Shapes/SM_PlaneCorner_64.SM_PlaneCorner_64" :NewEnumerator0 "/Game/InteriorBuildingKit/Geometry/Assets/Shapes/SM_PlaneCorner_128.SM_PlaneCorner_128" :NewEnumerator1 "/Game/InteriorBuildingKit/Geometry/Assets/Shapes/SM_PlaneCorner_256.SM_PlaneCorner_256" :NewEnumerator2 "/Game/InteriorBuildingKit/Geometry/Assets/Shapes/SM_PlaneCorner_512.SM_PlaneCorner_512" :NewEnumerator3 "/Game/InteriorBuildingKit/Geometry/Assets/Shapes/SM_PlaneCorner_1024.SM_PlaneCorner_1024"))
  (Transformation|SetRelativeScale3D (Variables|Default|GetPlane_Corner) (Math|Vector|MakeVector (.x (/ (Variables|Default|GetLocation) 1e+02)) (.y (/ (Variables|Default|GetLocation) 1e+02)) 5.0))
  (Rendering|Material|SetMaterial (Variables|Default|GetPlane_Corner) 0 (Variables|Default|GetNew%20Material)))