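; Configurable double door for an interior building kit that, when movable, swings open as something enters its overlap volume and closes as it leaves.
; The construction script picks door and handle meshes from data tables, applies material overrides, poses the open angles and optionally adds a matching wall.
; At BeginPlay it can snap unlocked doors shut.
; One timeline drives both leaves, blending from their current yaw so interrupted swings stay smooth.
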(event OnComponentBeginOverlap(CharacterOverlapVolume)
  (params (OverlappedComponent :type Primitive%20Component%20Object%20Reference) (OtherActor :type Actor%20Object%20Reference) (OtherComp :type Primitive%20Component%20Object%20Reference) (OtherBodyIndex :type Integer) (bFromSweep :type Boolean) (SweepResult :type Hit%20Result%20Structure%20%28by%20ref%29))
  (if (Utilities|Enum|Equal(Enum) (Variables|Default|GetDoors%20Mobility) "Movable")
    (Utilities|FlowControl|Sequence
      (:then_0
        (Utilities|FlowControl|DoOnce false
          (:Completed
            (Utilities|FlowControl|Sequence
              (:then_0
                (bind (_direction _0_1) (Timeline|Animate%20Door%20Open-Closed Stop)
                  (:Update
                    (Transformation|SetRelativeRotation (Variables|Default|GetSM_Door_Left) (Math|Rotator|MakeRotator 0.0 0.0 (Utilities|Select :Index _direction :Forward (Math|Float|Lerp (Variables|Variables|GetStarting%20Position%20%28Left%20Door%20animations%29) (Variables|Default|GetDoor%20Open%20Angle%20-%20Left) _0_1) :Backward (Math|Float|Lerp 0.0 (Variables|Variables|GetStarting%20Position%20%28Left%20Door%20animations%29) _0_1))) false false)
                    (Transformation|SetRelativeRotation (Variables|Default|GetSM_Door_Right) (Math|Rotator|MakeRotator 0.0 0.0 (Utilities|Select :Index _direction :Forward (Math|Float|Lerp (Variables|Variables|GetStarting%20Position%20%28Right%20Door%20animations%29) (* (Variables|Default|GetDoor%20Open%20Angle%20-%20Right) -1.0) _0_1) :Backward (Math|Float|Lerp 0.0 (Variables|Variables|GetStarting%20Position%20%28Right%20Door%20animations%29) _0_1))) false false))))
              (:then_1
                (Variables|Variables|SetStarting%20Position%20%28Left%20Door%20animations%29 (.yaw (Variables|/Script/Engine.SceneComponent|GetRelativeRotation (Variables|Default|GetSM_Door_Left))))
                (Variables|Variables|SetStarting%20Position%20%28Right%20Door%20animations%29 (.yaw (Variables|/Script/Engine.SceneComponent|GetRelativeRotation (Variables|Default|GetSM_Door_Right))))
                (Timeline|Animate%20Door%20Open-Closed PlayFromStart))))))
      (:then_1
        (Utilities|FlowControl|DoOnce false) ; enters at Reset
      ))))

(event OnComponentEndOverlap(CharacterOverlapVolume)
  (params (OverlappedComponent :type Primitive%20Component%20Object%20Reference) (OtherActor :type Actor%20Object%20Reference) (OtherComp :type Primitive%20Component%20Object%20Reference) (OtherBodyIndex :type Integer))
  (if (Utilities|Enum|Equal(Enum) (Variables|Default|GetDoors%20Mobility) "Movable")
    (Utilities|FlowControl|Sequence
      (:then_0
        (Utilities|FlowControl|DoOnce false
          (:Completed
            (Utilities|FlowControl|Sequence
              (:then_0
                (bind (_direction _0_1) (Timeline|Animate%20Door%20Open-Closed Stop)
                  (:Update
                    (Transformation|SetRelativeRotation (Variables|Default|GetSM_Door_Left) (Math|Rotator|MakeRotator 0.0 0.0 (Utilities|Select :Index _direction :Forward (Math|Float|Lerp (Variables|Variables|GetStarting%20Position%20%28Left%20Door%20animations%29) (Variables|Default|GetDoor%20Open%20Angle%20-%20Left) _0_1) :Backward (Math|Float|Lerp 0.0 (Variables|Variables|GetStarting%20Position%20%28Left%20Door%20animations%29) _0_1))) false false)
                    (Transformation|SetRelativeRotation (Variables|Default|GetSM_Door_Right) (Math|Rotator|MakeRotator 0.0 0.0 (Utilities|Select :Index _direction :Forward (Math|Float|Lerp (Variables|Variables|GetStarting%20Position%20%28Right%20Door%20animations%29) (* (Variables|Default|GetDoor%20Open%20Angle%20-%20Right) -1.0) _0_1) :Backward (Math|Float|Lerp 0.0 (Variables|Variables|GetStarting%20Position%20%28Right%20Door%20animations%29) _0_1))) false false))))
              (:then_1
                (Variables|Variables|SetStarting%20Position%20%28Left%20Door%20animations%29 (.yaw (Variables|/Script/Engine.SceneComponent|GetRelativeRotation (Variables|Default|GetSM_Door_Left))))
                (Variables|Variables|SetStarting%20Position%20%28Right%20Door%20animations%29 (.yaw (Variables|/Script/Engine.SceneComponent|GetRelativeRotation (Variables|Default|GetSM_Door_Right))))
                (Timeline|Animate%20Door%20Open-Closed ReverseFromEnd))))))
      (:then_1
        (Utilities|FlowControl|DoOnce false) ; enters at Reset
      ))))

(event EventBeginPlay
  (Components|Timeline|SetPlayRate (Variables|Default|GetAnimate%20Door%20Open-Closed) (/ 1.0 (Variables|Default|GetDoor%20Opening%20Time)))
  (if (Utilities|Enum|Equal(Enum) (Variables|Default|GetDoors%20Mobility) "Movable")
    (if (Variables|Default|GetStart%20Colsed%20when%20game%20plays?)
      (if (not (Variables|Default|GetIs%20Door%20Locked?%20-%20For%20Moveable))
        (Transformation|SetRelativeRotation (Variables|Default|GetSM_Door_Left) (Math|Rotator|MakeRotator 0.0 0.0 0.0) false false)
        (Transformation|SetRelativeRotation (Variables|Default|GetSM_Door_Right) (Math|Rotator|MakeRotator 0.0 0.0 0.0) false false)))))

(fn ConstructionScript
  (bind _door_material (Variables|Default|GetDoor%20Material))
  (bind _frame_material (Variables|Default|GetFrame%20Material))
  (bind _wall_width (Variables|Default|GetWall%20Width))
  (bind _wall_type (Variables|Default|GetWall%20Type))
  (bind _wall_width_2 (Variables|Default|GetWall%20Width))
  (bind _wall_width_3 (Variables|Default|GetWall%20Width))
  (bind _handle_geometry_override___back (Variables|Default|GetHandle%20Geometry%20Override%20-%20Back))
  (bind _handle_geometry_override___front (Variables|Default|GetHandle%20Geometry%20Override%20-%20Front))
  (bind _handle_geometry_override___front_2 (Variables|Default|GetHandle%20Geometry%20Override%20-%20Front))
  (bind _handle_geometry_override___back_2 (Variables|Default|GetHandle%20Geometry%20Override%20-%20Back))
  (Transformation|SetRelativeTransform (Variables|Default|GetCharacter%20Overlap%20Volume) (Math|Transform|MakeTransform "75.000000, 0,120.000000" "0, 0, 0" "1.000000,1.000000,1.000000") false true)
  (Transformation|SetMobility (Variables|Default|GetSM_Door_Left) (Variables|Default|GetDoors%20Mobility))
  (if (or (Utilities|Enum|Equal(Enum) _wall_type "NewEnumerator0") (Utilities|Enum|Equal(Enum) _wall_type "NewEnumerator1"))
    _
    (else
      (Variables|Default|SetDoor%20Type "NewEnumerator2")))
  (Components|StaticMesh|SetStaticMesh (Variables|Default|GetSM_Doorframe) (Utilities|Select :Index (Variables|Default|GetDoor%20Type) :NewEnumerator2 "/Game/InteriorBuildingKit/Geometry/Building/Doors/Doors/Frames/SM_Doorframe_Double_Reg.SM_Doorframe_Double_Reg" :NewEnumerator0 "/Game/InteriorBuildingKit/Geometry/Building/Doors/Doors/Frames/SM_Doorframe_Double_Tall.SM_Doorframe_Double_Tall"))
  (Utilities|IsValid _frame_material
    (:Is%20Valid
      (Rendering|Material|SetMaterial (Variables|Default|GetSM_Doorframe) (Variables|Default|GetFrame%20Material%20ID) _frame_material))
    (:Is%20Not%20Valid
      _))
  (bind _outrownames (DataTable|GetDataTableRowNames "/Game/InteriorBuildingKit/Struct/DoorTypes_DataTable.DoorTypes_DataTable"))
  (bind _returnvalue (Utilities|GetDataTableRow "/Game/InteriorBuildingKit/Struct/DoorTypes_DataTable.DoorTypes_DataTable" (Utilities|Array|Get(acopy) _outrownames (Variables|Default|GetDoor%20Option)) :!label _label)
    (:then
      (Components|StaticMesh|SetStaticMesh (Variables|Default|GetSM_Door_Left) (Utilities|Select :Index (Variables|Default|GetDoor%20Type) :NewEnumerator2 (.modelreferencedoubleregleft _returnvalue) :NewEnumerator0 (.modelreferencedoubletallleft _returnvalue)))
      (Components|StaticMesh|SetStaticMesh (Variables|Default|GetSM_Door_Right) (Utilities|Select :Index (Variables|Default|GetDoor%20Type) :NewEnumerator2 (.modelreferencedoubleregright _returnvalue) :NewEnumerator0 (.modelreferencedoubletallright _returnvalue)))
      (Transformation|SetRelativeLocation (Variables|Default|GetSM_Door1Handle_Front%20%28Lock%29) (Utilities|Select :Index (Variables|Default|GetDoor%20Type) :NewEnumerator2 (.handlelocationdoubleregfront _returnvalue) :NewEnumerator0 (.handlelocationdoubletallfront _returnvalue)) false false)
      (Transformation|SetRelativeLocation (Variables|Default|GetSM_Door1Handle_Back) (Utilities|Select :Index (Variables|Default|GetDoor%20Type) :NewEnumerator2 (.handlelocationdoubleregback _returnvalue) :NewEnumerator0 (.handlelocationdoubletallback _returnvalue)) false false)
      (Transformation|SetRelativeLocation (Variables|Default|GetSM_Door2Handle_Front) (Utilities|Select :Index (Variables|Default|GetDoor%20Type) :NewEnumerator2 (* (.handlelocationdoubleregfront _returnvalue) "1.000000,-1.000000,1.000000") :NewEnumerator0 (* (.handlelocationdoubletallfront _returnvalue) "1.000000,-1.000000,1.000000")) false false)
      (Transformation|SetRelativeLocation (Variables|Default|GetSM_Door2Handle_Back%20%28Lock%29) (Utilities|Select :Index (Variables|Default|GetDoor%20Type) :NewEnumerator2 (* (.handlelocationdoubleregback _returnvalue) "1.000000,-1.000000,1.000000") :NewEnumerator0 (* (.handlelocationdoubletallback _returnvalue) "1.000000,-1.000000,1.000000")) false false)
      (Utilities|IsValid _door_material
        (:Is%20Valid
          (Rendering|Material|SetMaterial (Variables|Default|GetSM_Door_Left) (Variables|Default|GetDoor%20Material%20ID) _door_material))
        (:Is%20Not%20Valid
          _))
      (Transformation|SetRelativeRotation (Variables|Default|GetSM_Door_Left) (Math|Rotator|MakeRotator 0.0 0.0 (Variables|Default|GetDoor%20Open%20Angle%20-%20Left)) false false)
      (Transformation|SetRelativeRotation (Variables|Default|GetSM_Door_Right) (Math|Rotator|MakeRotator 0.0 0.0 (* (Variables|Default|GetDoor%20Open%20Angle%20-%20Right) -1.0)) false false)
      (bind _outrownames_2 (DataTable|GetDataTableRowNames "/Game/InteriorBuildingKit/Struct/DoorHandleTypes_DataTable.DoorHandleTypes_DataTable"))
      (bind _returnvalue_2 (Utilities|GetDataTableRow "/Game/InteriorBuildingKit/Struct/DoorHandleTypes_DataTable.DoorHandleTypes_DataTable" (Utilities|Array|Get(acopy) _outrownames_2 (Variables|Default|GetHandle%20Option)) :!label _label_2)
        (:then
          (Components|StaticMesh|SetStaticMesh (Variables|Default|GetSM_Door1Handle_Front%20%28Lock%29) (select (Utilities|IsValid _handle_geometry_override___front_2) _handle_geometry_override___front_2 (select (Variables|Default|GetLock%20On%20Front%20Handle?) (.versionwithalock _returnvalue_2) (.versionwithnolock _returnvalue_2))))
          (Components|StaticMesh|SetStaticMesh (Variables|Default|GetSM_Door2Handle_Back%20%28Lock%29) (select (Utilities|IsValid _handle_geometry_override___back_2) _handle_geometry_override___back_2 (select (Variables|Default|GetLock%20On%20Back%20Handle?) (.versionwithalock _returnvalue_2) (.versionwithnolock _returnvalue_2))))
          (Components|StaticMesh|SetStaticMesh (Variables|Default|GetSM_Door2Handle_Front) (select (Utilities|IsValid _handle_geometry_override___front) _handle_geometry_override___front (.versionwithnolock _returnvalue_2)))
          (Components|StaticMesh|SetStaticMesh (Variables|Default|GetSM_Door1Handle_Back) (select (Utilities|IsValid _handle_geometry_override___back) _handle_geometry_override___back (.versionwithnolock _returnvalue_2)))
          (Rendering|Material|SetMaterial (Variables|Default|GetSM_Door2Handle_Front) (Variables|Default|GetHandle%20Material%20Override%20-%20Base%20ID) (Variables|Default|GetHandle%20material%20override%20-%20Base))
          (Rendering|Material|SetMaterial (Variables|Default|GetSM_Door1Handle_Back) (Variables|Default|GetHandle%20Material%20Override%20-%20Handle%20ID) (Variables|Default|GetHandle%20material%20override%20-%20Handle))
          (if (Variables|Default|GetAdd%20Wall?)
            (bind _returnvalue_3 (AddComponent|AddStaticMeshComponent false (Math|Transform|MakeTransform "0, 0, 0" "0, 0, 0" (Math|Vector|MakeVector (/ (Math|Conversions|ToFloat(Integer) (Variables|Default|GetWall%20thickness%20-%20In%20units)) 25.0) 1.0 1.0))))
            (Components|StaticMesh|SetStaticMesh _returnvalue_3 (Utilities|Select :Index (Variables|Default|GetWall%20Type) :NewEnumerator0 (Utilities|Select :Index (Variables|Default|GetDoor%20Type) :NewEnumerator2 (Utilities|Select :Index _wall_width_2 :NewEnumerator3 "/Game/InteriorBuildingKit/Geometry/Building/Transition/Door/SM_TallFrame500_RegDoorDouble_NoTrim.SM_TallFrame500_RegDoorDouble_NoTrim" :NewEnumerator2 "/Game/InteriorBuildingKit/Geometry/Building/Transition/Door/SM_TallFrame400_RegDoorDouble_NoTrim.SM_TallFrame400_RegDoorDouble_NoTrim" :NewEnumerator5 "/Game/InteriorBuildingKit/Geometry/Building/Transition/Door/SM_TallFrame300_RegDoorDouble_NoTrim.SM_TallFrame300_RegDoorDouble_NoTrim" :NewEnumerator6 "/Game/InteriorBuildingKit/Geometry/Building/Transition/Door/SM_TallFrame250_RegDoorDouble_NoTrim.SM_TallFrame250_RegDoorDouble_NoTrim") :NewEnumerator0 (Utilities|Select :Index _wall_width_2 :NewEnumerator3 "/Game/InteriorBuildingKit/Geometry/Building/Transition/Door/SM_TallFrame500_TallDoorDouble_NoTrim.SM_TallFrame500_TallDoorDouble_NoTrim" :NewEnumerator2 "/Game/InteriorBuildingKit/Geometry/Building/Transition/Door/SM_TallFrame400_TallDoorDouble_NoTrim.SM_TallFrame400_TallDoorDouble_NoTrim" :NewEnumerator5 "/Game/InteriorBuildingKit/Geometry/Building/Transition/Door/SM_TallFrame300_TallDoorDouble_NoTrim.SM_TallFrame300_TallDoorDouble_NoTrim" :NewEnumerator6 "/Game/InteriorBuildingKit/Geometry/Building/Transition/Door/SM_TallFrame250_TallDoorDouble_NoTrim.SM_TallFrame250_TallDoorDouble_NoTrim")) :NewEnumerator1 (Utilities|Select :Index (Variables|Default|GetDoor%20Type) :NewEnumerator2 (Utilities|Select :Index _wall_width :NewEnumerator3 "/Game/InteriorBuildingKit/Geometry/Building/Transition/Door/SM_TallFrame500_RegDoorDouble_Trim.SM_TallFrame500_RegDoorDouble_Trim" :NewEnumerator2 "/Game/InteriorBuildingKit/Geometry/Building/Transition/Door/SM_TallFrame400_RegDoorDouble_Trim.SM_TallFrame400_RegDoorDouble_Trim" :NewEnumerator5 "/Game/InteriorBuildingKit/Geometry/Building/Transition/Door/SM_TallFrame300_RegDoorDouble_Trim.SM_TallFrame300_RegDoorDouble_Trim" :NewEnumerator6 "/Game/InteriorBuildingKit/Geometry/Building/Transition/Door/SM_TallFrame250_RegDoorDouble_Trim.SM_TallFrame250_RegDoorDouble_Trim") :NewEnumerator0 (Utilities|Select :Index _wall_width :NewEnumerator3 "/Game/InteriorBuildingKit/Geometry/Building/Transition/Door/SM_TallFrame500_TallDoorDouble_Trim.SM_TallFrame500_TallDoorDouble_Trim" :NewEnumerator2 "/Game/InteriorBuildingKit/Geometry/Building/Transition/Door/SM_TallFrame400_TallDoorDouble_Trim.SM_TallFrame400_TallDoorDouble_Trim" :NewEnumerator5 "/Game/InteriorBuildingKit/Geometry/Building/Transition/Door/SM_TallFrame300_TallDoorDouble_Trim.SM_TallFrame300_TallDoorDouble_Trim" :NewEnumerator6 "/Game/InteriorBuildingKit/Geometry/Building/Transition/Door/SM_TallFrame250_TallDoorDouble_Trim.SM_TallFrame250_TallDoorDouble_Trim")) :NewEnumerator5 (Utilities|Select :Index _wall_width_3 :NewEnumerator3 "/Game/InteriorBuildingKit/Geometry/Building/Transition/Door/SM_RegFrame500_RegDoorDouble_NoTrim.SM_RegFrame500_RegDoorDouble_NoTrim" :NewEnumerator2 "/Game/InteriorBuildingKit/Geometry/Building/Transition/Door/SM_RegFrame400_RegDoorDouble_NoTrim.SM_RegFrame400_RegDoorDouble_NoTrim" :NewEnumerator5 "/Game/InteriorBuildingKit/Geometry/Building/Transition/Door/SM_RegFrame300_RegDoorDouble_NoTrim.SM_RegFrame300_RegDoorDouble_NoTrim" :NewEnumerator6 "/Game/InteriorBuildingKit/Geometry/Building/Transition/Door/SM_RegFrame250_RegDoorDouble_NoTrim.SM_RegFrame250_RegDoorDouble_NoTrim") :NewEnumerator6 (Utilities|Select :Index _wall_width_3 :NewEnumerator3 "/Game/InteriorBuildingKit/Geometry/Building/Transition/Door/SM_RegFrame500_RegDoorDouble_Trim.SM_RegFrame500_RegDoorDouble_Trim" :NewEnumerator2 "/Game/InteriorBuildingKit/Geometry/Building/Transition/Door/SM_RegFrame400_RegDoorDouble_Trim.SM_RegFrame400_RegDoorDouble_Trim" :NewEnumerator5 "/Game/InteriorBuildingKit/Geometry/Building/Transition/Door/SM_RegFrame300_RegDoorDouble_Trim.SM_RegFrame300_RegDoorDouble_Trim" :NewEnumerator6 "/Game/InteriorBuildingKit/Geometry/Building/Transition/Door/SM_RegFrame250_RegDoorDouble_Trim.SM_RegFrame250_RegDoorDouble_Trim")))
            (Transformation|SetRelativeLocation _returnvalue_3 (Math|Vector|MakeVector 0.0 (/ (.y (.Max (Components|StaticMesh|GetLocalBounds _returnvalue_3))) -2.0) 0.0) false true)
            (if (not (or (== _returnvalue_3 "/Game/InteriorBuildingKit/Geometry/Building/Transition/Door/SM_RegFrame150_RegDoorSingle_Trim.SM_RegFrame150_RegDoorSingle_Trim") (== _returnvalue_3 "/Game/InteriorBuildingKit/Geometry/Building/Transition/Door/SM_RegFrame250_RegDoorDouble_Trim.SM_RegFrame250_RegDoorDouble_Trim")))
              (Rendering|Material|SetMaterial _returnvalue_3 0 (Variables|Default|GetWallpaper%20Material%20-%20Left%20Side))
              (Rendering|Material|SetMaterial _returnvalue_3 1 (Variables|Default|GetWallpaper%20Material%20-%20Right%20Side))
              (Rendering|Material|SetMaterial _returnvalue_3 (select (or (== _returnvalue_3 "/Game/InteriorBuildingKit/Geometry/Building/Transition/Door/SM_RegFrame150_RegDoorSingle_Trim.SM_RegFrame150_RegDoorSingle_Trim") (== _returnvalue_3 "/Game/InteriorBuildingKit/Geometry/Building/Transition/Door/SM_RegFrame250_RegDoorDouble_Trim.SM_RegFrame250_RegDoorDouble_Trim")) 1 3) (Variables|Default|GetEdge%20Material))
              (Rendering|Material|SetMaterial _returnvalue_3 (select (or (== _returnvalue_3 "/Game/InteriorBuildingKit/Geometry/Building/Transition/Door/SM_RegFrame150_RegDoorSingle_Trim.SM_RegFrame150_RegDoorSingle_Trim") (== _returnvalue_3 "/Game/InteriorBuildingKit/Geometry/Building/Transition/Door/SM_RegFrame250_RegDoorDouble_Trim.SM_RegFrame250_RegDoorDouble_Trim")) 0 2) (Variables|Default|GetTrim%20Material)))))
        (:RowNotFound
          (Variables|Default|SetHandle%20Option (- (Utilities|Array|Length _outrownames_2) 1))
          (goto _label_2))))
    (:RowNotFound
      (Variables|Default|SetDoor%20Option (- (Utilities|Array|Length _outrownames) 1))
      (goto _label))))