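; Configurable single interior door for a building kit that swings open when something enters its overlap volume and closes when it leaves, if set to Movable.
; The construction script picks frame, door and handle meshes from enums and data tables, clamping out-of-range options to the last row.
; It applies material overrides and can add a matching wall with optional siding.
; A timeline swings the door from its current yaw over a configurable opening time.
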(event OnComponentBeginOverlap(CharacterOverlapVolume)
  (params (OverlappedComponent :type Primitive%20Component%20Object%20Reference) (OtherActor :type Actor%20Object%20Reference) (OtherComp :type Primitive%20Component%20Object%20Reference) (OtherBodyIndex :type Integer) (bFromSweep :type Boolean) (SweepResult :type Hit%20Result%20Structure%20%28by%20ref%29))
  (if (Utilities|Enum|Equal(Enum) (Variables|Default|GetDoors%20Mobility) "Movable")
    (Utilities|FlowControl|Sequence
      (:then_0
        (Utilities|FlowControl|DoOnce false
          (:Completed
            (Utilities|FlowControl|Sequence
              (:then_0
                (bind (_direction _0_1) (Timeline|Animate%20Door%20Open-Closed Stop)
                  (:Update
                    (Transformation|SetRelativeRotation (Variables|Default|GetSM_Door) (Math|Rotator|MakeRotator 0.0 0.0 (Utilities|Select :Index _direction :Forward (Math|Float|Lerp (Variables|Variables|GetStarting%20Position%20%28Door%20animations%29) (Variables|Default|GetDoor%20Open%20Angle) _0_1) :Backward (Math|Float|Lerp 0.0 (Variables|Variables|GetStarting%20Position%20%28Door%20animations%29) _0_1))) false false))))
              (:then_1
                (Variables|Variables|SetStarting%20Position%20%28Door%20animations%29 (.yaw (Variables|/Script/Engine.SceneComponent|GetRelativeRotation (Variables|Default|GetSM_Door))))
                (Timeline|Animate%20Door%20Open-Closed PlayFromStart))))))
      (:then_1
        (Utilities|FlowControl|DoOnce false) ; enters at Reset
      ))))

(event OnComponentEndOverlap(CharacterOverlapVolume)
  (params (OverlappedComponent :type Primitive%20Component%20Object%20Reference) (OtherActor :type Actor%20Object%20Reference) (OtherComp :type Primitive%20Component%20Object%20Reference) (OtherBodyIndex :type Integer))
  (if (Utilities|Enum|Equal(Enum) (Variables|Default|GetDoors%20Mobility) "Movable")
    (Utilities|FlowControl|Sequence
      (:then_0
        (Utilities|FlowControl|DoOnce false
          (:Completed
            (Utilities|FlowControl|Sequence
              (:then_0
                (bind (_direction _0_1) (Timeline|Animate%20Door%20Open-Closed Stop)
                  (:Update
                    (Transformation|SetRelativeRotation (Variables|Default|GetSM_Door) (Math|Rotator|MakeRotator 0.0 0.0 (Utilities|Select :Index _direction :Forward (Math|Float|Lerp (Variables|Variables|GetStarting%20Position%20%28Door%20animations%29) (Variables|Default|GetDoor%20Open%20Angle) _0_1) :Backward (Math|Float|Lerp 0.0 (Variables|Variables|GetStarting%20Position%20%28Door%20animations%29) _0_1))) false false))))
              (:then_1
                (Variables|Variables|SetStarting%20Position%20%28Door%20animations%29 (.yaw (Variables|/Script/Engine.SceneComponent|GetRelativeRotation (Variables|Default|GetSM_Door))))
                (Timeline|Animate%20Door%20Open-Closed ReverseFromEnd))))))
      (:then_1
        (Utilities|FlowControl|DoOnce false) ; enters at Reset
      ))))

(event EventBeginPlay
  (Components|Timeline|SetPlayRate (Variables|Default|GetAnimate%20Door%20Open-Closed) (/ 1.0 (Variables|Default|GetDoor%20Opening%20Time)))
  (if (Utilities|Enum|Equal(Enum) (Variables|Default|GetDoors%20Mobility) "Movable")
    (if (Variables|Default|GetStart%20Colsed%20when%20game%20plays?)
      (if (not (Variables|Default|GetIs%20Door%20Locked?%20-%20For%20Moveable))
        (Transformation|SetRelativeRotation (Variables|Default|GetSM_Door) (Math|Rotator|MakeRotator 0.0 0.0 0.0) false false)))))

(fn ConstructionScript
  (bind _door_material (Variables|Default|GetDoor%20Material))
  (bind _wall_width (Variables|Default|GetWall%20Width))
  (bind _wall_width_2 (Variables|Default|GetWall%20Width))
  (bind _wall_width_3 (Variables|Default|GetWall%20Width))
  (bind _wall_width_4 (Variables|Default|GetWall%20Width))
  (bind _wall_type (Variables|Default|GetWall%20Type))
  (bind _frame_material (Variables|Default|GetFrame%20Material))
  (bind _handle_geometry_override___back (Variables|Default|GetHandle%20Geometry%20Override%20-%20Back))
  (bind _handle_geometry_override___front (Variables|Default|GetHandle%20Geometry%20Override%20-%20Front))
  (bind _returnvalue (Utilities|Select :Index _wall_width_4 :NewEnumerator3 "/Game/InteriorBuildingKit/Geometry/Building/Siding/Doors/SM_RegFrame500_RegDoorSingle_Ext01.SM_RegFrame500_RegDoorSingle_Ext01" :NewEnumerator2 "/Game/InteriorBuildingKit/Geometry/Building/Siding/Doors/SM_RegFrame400_RegDoorSingle_Ext01.SM_RegFrame400_RegDoorSingle_Ext01" :NewEnumerator5 "/Game/InteriorBuildingKit/Geometry/Building/Siding/Doors/SM_RegFrame300_RegDoorSingle_Ext01.SM_RegFrame300_RegDoorSingle_Ext01" :NewEnumerator6 "/Game/InteriorBuildingKit/Geometry/Building/Siding/Doors/SM_RegFrame200_RegDoorSingle_Ext01.SM_RegFrame200_RegDoorSingle_Ext01" :NewEnumerator7 "/Game/InteriorBuildingKit/Geometry/Building/Transition/Door/SM_RegFrame150_RegDoorSingle_NoTrim.SM_RegFrame150_RegDoorSingle_NoTrim"))
  (Transformation|SetRelativeTransform (Variables|Default|GetCharacter%20Overlap%20Volume) (Math|Transform|MakeTransform "75.000000, 0,120.000000" "0, 0, 0" "1.000000,1.000000,1.000000") false true)
  (Transformation|SetMobility (Variables|Default|GetSM_Door) (Variables|Default|GetDoors%20Mobility))
  (if (or (Utilities|Enum|Equal(Enum) _wall_type "NewEnumerator0") (Utilities|Enum|Equal(Enum) _wall_type "NewEnumerator1"))
    _
    (else
      (Variables|Default|SetDoor%20Type "NewEnumerator2")))
  (Components|StaticMesh|SetStaticMesh (Variables|Default|GetSM_Doorframe) (Utilities|Select :Index (Variables|Default|GetDoor%20Type) :NewEnumerator2 "/Game/InteriorBuildingKit/Geometry/Building/Doors/Doors/Frames/SM_Doorframe_Single_Reg.SM_Doorframe_Single_Reg" :NewEnumerator0 "/Game/InteriorBuildingKit/Geometry/Building/Doors/Doors/Frames/SM_Doorframe_Single_Tall.SM_Doorframe_Single_Tall"))
  (Utilities|IsValid _frame_material
    (:Is%20Valid
      (Rendering|Material|SetMaterial (Variables|Default|GetSM_Doorframe) (Variables|Default|GetFrame%20Material%20ID) _frame_material))
    (:Is%20Not%20Valid
      _))
  (bind _outrownames (DataTable|GetDataTableRowNames "/Game/InteriorBuildingKit/Struct/DoorTypes_DataTable.DoorTypes_DataTable"))
  (bind _returnvalue_2 (Utilities|GetDataTableRow "/Game/InteriorBuildingKit/Struct/DoorTypes_DataTable.DoorTypes_DataTable" (Utilities|Array|Get(acopy) _outrownames (Variables|Default|GetDoor%20Option)) :!label _label)
    (:then
      (Components|StaticMesh|SetStaticMesh (Variables|Default|GetSM_Door) (Utilities|Select :Index (Variables|Default|GetDoor%20Type) :NewEnumerator2 (.modelreferencesinglereg _returnvalue_2) :NewEnumerator0 (.modelreferencesingletall _returnvalue_2)))
      (Transformation|SetRelativeLocation (Variables|Default|GetSM_DoorHandle_Front) (Utilities|Select :Index (Variables|Default|GetDoor%20Type) :NewEnumerator2 (.handlelocationsingleregfront _returnvalue_2) :NewEnumerator0 (.handlelocationsingletallfront _returnvalue_2)) false false)
      (Transformation|SetRelativeLocation (Variables|Default|GetSM_DoorHandle_Back) (Utilities|Select :Index (Variables|Default|GetDoor%20Type) :NewEnumerator2 (.handlelocationsingleregback _returnvalue_2) :NewEnumerator0 (.handlelocationsingletallback _returnvalue_2)) false false)
      (Utilities|IsValid _door_material
        (:Is%20Valid
          (Rendering|Material|SetMaterial (Variables|Default|GetSM_Door) (Variables|Default|GetDoor%20Material%20ID) _door_material))
        (:Is%20Not%20Valid
          _))
      (Transformation|SetRelativeRotation (Variables|Default|GetSM_Door) (Math|Rotator|MakeRotator 0.0 0.0 (Variables|Default|GetDoor%20Open%20Angle)) false false)
      (bind _outrownames_2 (DataTable|GetDataTableRowNames "/Game/InteriorBuildingKit/Struct/DoorHandleTypes_DataTable.DoorHandleTypes_DataTable"))
      (bind _returnvalue_3 (Utilities|GetDataTableRow "/Game/InteriorBuildingKit/Struct/DoorHandleTypes_DataTable.DoorHandleTypes_DataTable" (Utilities|Array|Get(acopy) _outrownames_2 (Variables|Default|GetHandle%20Option)) :!label _label_2)
        (:then
          (Components|StaticMesh|SetStaticMesh (Variables|Default|GetSM_DoorHandle_Front) (select (Utilities|IsValid _handle_geometry_override___front) _handle_geometry_override___front (select (Variables|Default|GetLock%20On%20Front%20Handle?) (.versionwithalock _returnvalue_3) (.versionwithnolock _returnvalue_3))))
          (Components|StaticMesh|SetStaticMesh (Variables|Default|GetSM_DoorHandle_Back) (select (Utilities|IsValid _handle_geometry_override___back) _handle_geometry_override___back (select (Variables|Default|GetLock%20On%20Back%20Handle?) (.versionwithalock _returnvalue_3) (.versionwithnolock _returnvalue_3))))
          (Rendering|Material|SetMaterial (Variables|Default|GetSM_DoorHandle_Front) (Variables|Default|GetHandle%20Material%20Override%20-%20Base%20ID) (Variables|Default|GetHandle%20material%20override%20-%20Base))
          (Rendering|Material|SetMaterial (Variables|Default|GetSM_DoorHandle_Front) (Variables|Default|GetHandle%20Material%20Override%20-%20Handle%20ID) (Variables|Default|GetHandle%20material%20override%20-%20Handle))
          (if (Variables|Default|GetAdd%20Wall?)
            (bind _returnvalue_4 (AddComponent|AddStaticMeshComponent false (Math|Transform|MakeTransform "0, 0, 0" "0, 0, 0" (Math|Vector|MakeVector (/ (Math|Conversions|ToFloat(Integer) (Variables|Default|GetWall%20thickness%20-%20In%20units)) 25.0) 1.0 1.0))))
            (Components|StaticMesh|SetStaticMesh _returnvalue_4 (Utilities|Select :Index (Variables|Default|GetWall%20Type) :NewEnumerator0 (Utilities|Select :Index (Variables|Default|GetDoor%20Type) :NewEnumerator2 (Utilities|Select :Index _wall_width_3 :NewEnumerator3 "/Game/InteriorBuildingKit/Geometry/Building/Transition/Door/SM_TallFrame500_RegDoorSingle_NoTrim.SM_TallFrame500_RegDoorSingle_NoTrim" :NewEnumerator2 "/Game/InteriorBuildingKit/Geometry/Building/Transition/Door/SM_TallFrame400_RegDoorSingle_NoTrim.SM_TallFrame400_RegDoorSingle_NoTrim" :NewEnumerator5 "/Game/InteriorBuildingKit/Geometry/Building/Transition/Door/SM_TallFrame300_RegDoorSingle_NoTrim.SM_TallFrame300_RegDoorSingle_NoTrim" :NewEnumerator6 "/Game/InteriorBuildingKit/Geometry/Building/Transition/Door/SM_TallFrame200_RegDoorSingle_NoTrim.SM_TallFrame200_RegDoorSingle_NoTrim" :NewEnumerator7 "/Game/InteriorBuildingKit/Geometry/Building/Transition/Door/SM_TallFrame150_RegDoorSingle_NoTrim.SM_TallFrame150_RegDoorSingle_NoTrim") :NewEnumerator0 (Utilities|Select :Index _wall_width_3 :NewEnumerator3 "/Game/InteriorBuildingKit/Geometry/Building/Transition/Door/SM_TallFrame500_TallDoorSingle_NoTrim.SM_TallFrame500_TallDoorSingle_NoTrim" :NewEnumerator2 "/Game/InteriorBuildingKit/Geometry/Building/Transition/Door/SM_TallFrame400_TallDoorSingle_NoTrim.SM_TallFrame400_TallDoorSingle_NoTrim" :NewEnumerator5 "/Game/InteriorBuildingKit/Geometry/Building/Transition/Door/SM_TallFrame300_TallDoorSingle_NoTrim.SM_TallFrame300_TallDoorSingle_NoTrim" :NewEnumerator6 "/Game/InteriorBuildingKit/Geometry/Building/Transition/Door/SM_TallFrame200_TallDoorSingle_NoTrim.SM_TallFrame200_TallDoorSingle_NoTrim" :NewEnumerator7 "/Game/InteriorBuildingKit/Geometry/Building/Transition/Door/SM_TallFrame150_TallDoorSingle_NoTrim.SM_TallFrame150_TallDoorSingle_NoTrim")) :NewEnumerator1 (Utilities|Select :Index (Variables|Default|GetDoor%20Type) :NewEnumerator2 (Utilities|Select :Index _wall_width :NewEnumerator3 "/Game/InteriorBuildingKit/Geometry/Building/Transition/Door/SM_TallFrame500_RegDoorSingle_Trim.SM_TallFrame500_RegDoorSingle_Trim" :NewEnumerator2 "/Game/InteriorBuildingKit/Geometry/Building/Transition/Door/SM_TallFrame400_RegDoorSingle_Trim.SM_TallFrame400_RegDoorSingle_Trim" :NewEnumerator5 "/Game/InteriorBuildingKit/Geometry/Building/Transition/Door/SM_TallFrame300_RegDoorSingle_Trim.SM_TallFrame300_RegDoorSingle_Trim" :NewEnumerator6 "/Game/InteriorBuildingKit/Geometry/Building/Transition/Door/SM_TallFrame200_RegDoorSingle_Trim.SM_TallFrame200_RegDoorSingle_Trim" :NewEnumerator7 "/Game/InteriorBuildingKit/Geometry/Building/Transition/Door/SM_TallFrame150_RegDoorSingle_Trim.SM_TallFrame150_RegDoorSingle_Trim") :NewEnumerator0 (Utilities|Select :Index _wall_width :NewEnumerator3 "/Game/InteriorBuildingKit/Geometry/Building/Transition/Door/SM_TallFrame500_TallDoorSingle_Trim.SM_TallFrame500_TallDoorSingle_Trim" :NewEnumerator2 "/Game/InteriorBuildingKit/Geometry/Building/Transition/Door/SM_TallFrame400_TallDoorSingle_Trim.SM_TallFrame400_TallDoorSingle_Trim" :NewEnumerator5 "/Game/InteriorBuildingKit/Geometry/Building/Transition/Door/SM_TallFrame300_TallDoorSingle_Trim.SM_TallFrame300_TallDoorSingle_Trim" :NewEnumerator6 "/Game/InteriorBuildingKit/Geometry/Building/Transition/Door/SM_TallFrame200_TallDoorSingle_NoTrim.SM_TallFrame200_TallDoorSingle_NoTrim" :NewEnumerator7 "/Game/InteriorBuildingKit/Geometry/Building/Transition/Door/SM_TallFrame150_TallDoorSingle_Trim.SM_TallFrame150_TallDoorSingle_Trim")) :NewEnumerator5 (Utilities|Select :Index _wall_width_2 :NewEnumerator3 "/Game/InteriorBuildingKit/Geometry/Building/Transition/Door/SM_RegFrame500_RegDoorSingle_NoTrim.SM_RegFrame500_RegDoorSingle_NoTrim" :NewEnumerator2 "/Game/InteriorBuildingKit/Geometry/Building/Transition/Door/SM_RegFrame400_RegDoorSingle_NoTrim.SM_RegFrame400_RegDoorSingle_NoTrim" :NewEnumerator5 "/Game/InteriorBuildingKit/Geometry/Building/Transition/Door/SM_RegFrame300_RegDoorSingle_NoTrim.SM_RegFrame300_RegDoorSingle_NoTrim" :NewEnumerator6 "/Game/InteriorBuildingKit/Geometry/Building/Transition/Door/SM_RegFrame200_RegDoorSingle_NoTrim.SM_RegFrame200_RegDoorSingle_NoTrim" :NewEnumerator7 "/Game/InteriorBuildingKit/Geometry/Building/Transition/Door/SM_RegFrame150_RegDoorSingle_NoTrim.SM_RegFrame150_RegDoorSingle_NoTrim") :NewEnumerator6 (Utilities|Select :Index _wall_width_2 :NewEnumerator3 "/Game/InteriorBuildingKit/Geometry/Building/Transition/Door/SM_RegFrame500_RegDoorSingle_Trim.SM_RegFrame500_RegDoorSingle_Trim" :NewEnumerator2 "/Game/InteriorBuildingKit/Geometry/Building/Transition/Door/SM_RegFrame400_RegDoorSingle_Trim.SM_RegFrame400_RegDoorSingle_Trim" :NewEnumerator5 "/Game/InteriorBuildingKit/Geometry/Building/Transition/Door/SM_RegFrame300_RegDoorSingle_Trim.SM_RegFrame300_RegDoorSingle_Trim" :NewEnumerator6 "/Game/InteriorBuildingKit/Geometry/Building/Transition/Door/SM_RegFrame200_RegDoorSingle_Trim.SM_RegFrame200_RegDoorSingle_Trim" :NewEnumerator7 "/Game/InteriorBuildingKit/Geometry/Building/Transition/Door/SM_RegFrame150_RegDoorSingle_Trim.SM_RegFrame150_RegDoorSingle_Trim")))
            (Transformation|SetRelativeLocation _returnvalue_4 (Math|Vector|MakeVector 0.0 (/ (.y (.Max (Components|StaticMesh|GetLocalBounds _returnvalue_4))) -2.0) 0.0) false true)
            (Utilities|FlowControl|Sequence
              (:then_0
                (if (not (or (== _returnvalue_4 "/Game/InteriorBuildingKit/Geometry/Building/Transition/Door/SM_RegFrame150_RegDoorSingle_Trim.SM_RegFrame150_RegDoorSingle_Trim") (== _returnvalue_4 "/Game/InteriorBuildingKit/Geometry/Building/Transition/Door/SM_RegFrame250_RegDoorDouble_Trim.SM_RegFrame250_RegDoorDouble_Trim")))
                  (Rendering|Material|SetMaterial _returnvalue_4 0 (Variables|Default|GetWallpaper%20Material%20-%20Left%20Side))
                  (Rendering|Material|SetMaterial _returnvalue_4 1 (Variables|Default|GetWallpaper%20Material%20-%20Right%20Side))
                  (Rendering|Material|SetMaterial _returnvalue_4 (select (or (== _returnvalue_4 "/Game/InteriorBuildingKit/Geometry/Building/Transition/Door/SM_RegFrame150_RegDoorSingle_Trim.SM_RegFrame150_RegDoorSingle_Trim") (== _returnvalue_4 "/Game/InteriorBuildingKit/Geometry/Building/Transition/Door/SM_RegFrame250_RegDoorDouble_Trim.SM_RegFrame250_RegDoorDouble_Trim")) 1 3) (Variables|Default|GetEdge%20Material))
                  (Rendering|Material|SetMaterial _returnvalue_4 (select (or (== _returnvalue_4 "/Game/InteriorBuildingKit/Geometry/Building/Transition/Door/SM_RegFrame150_RegDoorSingle_Trim.SM_RegFrame150_RegDoorSingle_Trim") (== _returnvalue_4 "/Game/InteriorBuildingKit/Geometry/Building/Transition/Door/SM_RegFrame250_RegDoorDouble_Trim.SM_RegFrame250_RegDoorDouble_Trim")) 0 2) (Variables|Default|GetTrim%20Material))))
              (:then_1
                (Utilities|FlowControl|Sequence
                  (:then_0
                    (if (Variables|Default|GetAdd%20siding%20on%20Left%20side?)
                      (bind _returnvalue_5 (AddComponent|AddStaticMeshComponent false))
                      (bind _output_get (Variables|Default|SetExterior%20Reference%20-%20Left%20Side _returnvalue_5))
                      (Components|StaticMesh|SetStaticMesh _output_get (Utilities|Select :Index (Variables|Default|GetWall%20Type) :NewEnumerator0 (Utilities|Select :Index (Variables|Default|GetDoor%20Type) :NewEnumerator2 (Utilities|Select :Index _wall_width_4 :NewEnumerator3 "/Game/InteriorBuildingKit/Geometry/Building/Siding/Doors/SM_TallFrame500_RegDoorSingle_Ext01.SM_TallFrame500_RegDoorSingle_Ext01" :NewEnumerator2 "/Game/InteriorBuildingKit/Geometry/Building/Siding/Doors/SM_TallFrame400_RegDoorSingle_Ext01.SM_TallFrame400_RegDoorSingle_Ext01" :NewEnumerator5 "/Game/InteriorBuildingKit/Geometry/Building/Siding/Doors/SM_TallFrame300_RegDoorSingle_Ext01.SM_TallFrame300_RegDoorSingle_Ext01" :NewEnumerator6 "/Game/InteriorBuildingKit/Geometry/Building/Siding/Doors/SM_TallFrame200_RegDoorSingle_Ext01.SM_TallFrame200_RegDoorSingle_Ext01" :NewEnumerator7 "/Game/InteriorBuildingKit/Geometry/Building/Siding/Doors/SM_TallFrame150_RegDoorSingle_Ext01.SM_TallFrame150_RegDoorSingle_Ext01") :NewEnumerator0 (Utilities|Select :Index _wall_width_4 :NewEnumerator3 "/Game/InteriorBuildingKit/Geometry/Building/Siding/Doors/SM_TallFrame500_TallDoorSingle_Ext01.SM_TallFrame500_TallDoorSingle_Ext01" :NewEnumerator2 "/Game/InteriorBuildingKit/Geometry/Building/Siding/Doors/SM_TallFrame400_TallDoorSingle_Ext01.SM_TallFrame400_TallDoorSingle_Ext01" :NewEnumerator5 "/Game/InteriorBuildingKit/Geometry/Building/Siding/Doors/SM_TallFrame300_TallDoorSingle_Ext01.SM_TallFrame300_TallDoorSingle_Ext01" :NewEnumerator6 "/Game/InteriorBuildingKit/Geometry/Building/Siding/Doors/SM_TallFrame200_TallDoorSingle_Ext01.SM_TallFrame200_TallDoorSingle_Ext01" :NewEnumerator7 "/Game/InteriorBuildingKit/Geometry/Building/Siding/Doors/SM_TallFrame150_TallDoorSingle_Ext01.SM_TallFrame150_TallDoorSingle_Ext01")) :NewEnumerator1 (Utilities|Select :Index (Variables|Default|GetDoor%20Type) :NewEnumerator2 (Utilities|Select :Index _wall_width_4 :NewEnumerator3 "/Game/InteriorBuildingKit/Geometry/Building/Siding/Doors/SM_TallFrame500_RegDoorSingle_Ext01.SM_TallFrame500_RegDoorSingle_Ext01" :NewEnumerator2 "/Game/InteriorBuildingKit/Geometry/Building/Siding/Doors/SM_TallFrame400_RegDoorSingle_Ext01.SM_TallFrame400_RegDoorSingle_Ext01" :NewEnumerator5 "/Game/InteriorBuildingKit/Geometry/Building/Siding/Doors/SM_TallFrame300_RegDoorSingle_Ext01.SM_TallFrame300_RegDoorSingle_Ext01" :NewEnumerator6 "/Game/InteriorBuildingKit/Geometry/Building/Siding/Doors/SM_TallFrame200_RegDoorSingle_Ext01.SM_TallFrame200_RegDoorSingle_Ext01" :NewEnumerator7 "/Game/InteriorBuildingKit/Geometry/Building/Siding/Doors/SM_TallFrame150_RegDoorSingle_Ext01.SM_TallFrame150_RegDoorSingle_Ext01") :NewEnumerator0 (Utilities|Select :Index _wall_width_4 :NewEnumerator3 "/Game/InteriorBuildingKit/Geometry/Building/Siding/Doors/SM_TallFrame500_TallDoorSingle_Ext01.SM_TallFrame500_TallDoorSingle_Ext01" :NewEnumerator2 "/Game/InteriorBuildingKit/Geometry/Building/Siding/Doors/SM_TallFrame400_TallDoorSingle_Ext01.SM_TallFrame400_TallDoorSingle_Ext01" :NewEnumerator5 "/Game/InteriorBuildingKit/Geometry/Building/Siding/Doors/SM_TallFrame300_TallDoorSingle_Ext01.SM_TallFrame300_TallDoorSingle_Ext01" :NewEnumerator6 "/Game/InteriorBuildingKit/Geometry/Building/Siding/Doors/SM_TallFrame200_TallDoorSingle_Ext01.SM_TallFrame200_TallDoorSingle_Ext01" :NewEnumerator7 "/Game/InteriorBuildingKit/Geometry/Building/Siding/Doors/SM_TallFrame150_TallDoorSingle_Ext01.SM_TallFrame150_TallDoorSingle_Ext01")) :NewEnumerator5 _returnvalue :NewEnumerator6 _returnvalue))
                      (Transformation|SetRelativeLocation _output_get (Math|Vector|MakeVector -15.0 (/ (.y (.Max (Components|StaticMesh|GetLocalBounds _returnvalue_4))) 2.0) 0.0) false true)))
                  (:then_1
                    (if (Variables|Default|GetAdd%20siding%20on%20Right%20Side?)
                      (bind _returnvalue_6 (AddComponent|AddStaticMeshComponent false (Math|Transform|MakeTransform "0, 0, 0" "0, 0, 0" "-1.000000,1,1")))
                      (bind _output_get_2 (Variables|Default|SetExterior%20Reference%20-%20Right%20Side _returnvalue_6))
                      (Components|StaticMesh|SetStaticMesh _output_get_2 (Utilities|Select :Index (Variables|Default|GetWall%20Type) :NewEnumerator0 (Utilities|Select :Index (Variables|Default|GetDoor%20Type) :NewEnumerator2 (Utilities|Select :Index _wall_width_4 :NewEnumerator3 "/Game/InteriorBuildingKit/Geometry/Building/Siding/Doors/SM_TallFrame500_RegDoorSingle_Ext01.SM_TallFrame500_RegDoorSingle_Ext01" :NewEnumerator2 "/Game/InteriorBuildingKit/Geometry/Building/Siding/Doors/SM_TallFrame400_RegDoorSingle_Ext01.SM_TallFrame400_RegDoorSingle_Ext01" :NewEnumerator5 "/Game/InteriorBuildingKit/Geometry/Building/Siding/Doors/SM_TallFrame300_RegDoorSingle_Ext01.SM_TallFrame300_RegDoorSingle_Ext01" :NewEnumerator6 "/Game/InteriorBuildingKit/Geometry/Building/Siding/Doors/SM_TallFrame200_RegDoorSingle_Ext01.SM_TallFrame200_RegDoorSingle_Ext01" :NewEnumerator7 "/Game/InteriorBuildingKit/Geometry/Building/Siding/Doors/SM_TallFrame150_RegDoorSingle_Ext01.SM_TallFrame150_RegDoorSingle_Ext01") :NewEnumerator0 (Utilities|Select :Index _wall_width_4 :NewEnumerator3 "/Game/InteriorBuildingKit/Geometry/Building/Siding/Doors/SM_TallFrame500_TallDoorSingle_Ext01.SM_TallFrame500_TallDoorSingle_Ext01" :NewEnumerator2 "/Game/InteriorBuildingKit/Geometry/Building/Siding/Doors/SM_TallFrame400_TallDoorSingle_Ext01.SM_TallFrame400_TallDoorSingle_Ext01" :NewEnumerator5 "/Game/InteriorBuildingKit/Geometry/Building/Siding/Doors/SM_TallFrame300_TallDoorSingle_Ext01.SM_TallFrame300_TallDoorSingle_Ext01" :NewEnumerator6 "/Game/InteriorBuildingKit/Geometry/Building/Siding/Doors/SM_TallFrame200_TallDoorSingle_Ext01.SM_TallFrame200_TallDoorSingle_Ext01" :NewEnumerator7 "/Game/InteriorBuildingKit/Geometry/Building/Siding/Doors/SM_TallFrame150_TallDoorSingle_Ext01.SM_TallFrame150_TallDoorSingle_Ext01")) :NewEnumerator1 (Utilities|Select :Index (Variables|Default|GetDoor%20Type) :NewEnumerator2 (Utilities|Select :Index _wall_width_4 :NewEnumerator3 "/Game/InteriorBuildingKit/Geometry/Building/Siding/Doors/SM_TallFrame500_RegDoorSingle_Ext01.SM_TallFrame500_RegDoorSingle_Ext01" :NewEnumerator2 "/Game/InteriorBuildingKit/Geometry/Building/Siding/Doors/SM_TallFrame400_RegDoorSingle_Ext01.SM_TallFrame400_RegDoorSingle_Ext01" :NewEnumerator5 "/Game/InteriorBuildingKit/Geometry/Building/Siding/Doors/SM_TallFrame300_RegDoorSingle_Ext01.SM_TallFrame300_RegDoorSingle_Ext01" :NewEnumerator6 "/Game/InteriorBuildingKit/Geometry/Building/Siding/Doors/SM_TallFrame200_RegDoorSingle_Ext01.SM_TallFrame200_RegDoorSingle_Ext01" :NewEnumerator7 "/Game/InteriorBuildingKit/Geometry/Building/Siding/Doors/SM_TallFrame150_RegDoorSingle_Ext01.SM_TallFrame150_RegDoorSingle_Ext01") :NewEnumerator0 (Utilities|Select :Index _wall_width_4 :NewEnumerator3 "/Game/InteriorBuildingKit/Geometry/Building/Siding/Doors/SM_TallFrame500_TallDoorSingle_Ext01.SM_TallFrame500_TallDoorSingle_Ext01" :NewEnumerator2 "/Game/InteriorBuildingKit/Geometry/Building/Siding/Doors/SM_TallFrame400_TallDoorSingle_Ext01.SM_TallFrame400_TallDoorSingle_Ext01" :NewEnumerator5 "/Game/InteriorBuildingKit/Geometry/Building/Siding/Doors/SM_TallFrame300_TallDoorSingle_Ext01.SM_TallFrame300_TallDoorSingle_Ext01" :NewEnumerator6 "/Game/InteriorBuildingKit/Geometry/Building/Siding/Doors/SM_TallFrame200_TallDoorSingle_Ext01.SM_TallFrame200_TallDoorSingle_Ext01" :NewEnumerator7 "/Game/InteriorBuildingKit/Geometry/Building/Siding/Doors/SM_TallFrame150_TallDoorSingle_Ext01.SM_TallFrame150_TallDoorSingle_Ext01")) :NewEnumerator5 _returnvalue :NewEnumerator6 _returnvalue))
                      (Transformation|SetRelativeLocation _output_get_2 (Math|Vector|MakeVector 0.0 (/ (.y (.Max (Components|StaticMesh|GetLocalBounds _returnvalue_4))) 2.0) 0.0) false true))))))))
        (:RowNotFound
          (Variables|Default|SetHandle%20Option (- (Utilities|Array|Length _outrownames_2) 1))
          (goto _label_2))))
    (:RowNotFound
      (Variables|Default|SetDoor%20Option (- (Utilities|Array|Length _outrownames) 1))
      (goto _label))))