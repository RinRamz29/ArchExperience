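; Configurable dresser prop from an interior building kit, assembled entirely in the construction script.
; DresserType and DresserOption pick a row from the Narrow, Wide or Tall data table, supplying body, optional mirror and up to eight drawer meshes and positions.
; Per-drawer open amounts are capped at the row's pull-out limit and offset drawers along Y; unused components are destroyed.
; Handle meshes come from a handle-type table, with separate dresser and handle materials.
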(event EventBeginPlay)

(event Collision|EventActorBeginOverlap
  (params (OtherActor :type Actor%20Object%20Reference)))

(event EventTick
  (params (DeltaSeconds :type Float%20%28single-precision%29)))

(fn ConstructionScript
  (bind _sm_dresser_drawer8 (Variables|Default|GetSM_Dresser_Drawer8))
  (bind _sm_dresser_drawer1 (Variables|Default|GetSM_Dresser_Drawer1))
  (bind _sm_dresser_drawer3 (Variables|Default|GetSM_Dresser_Drawer3))
  (bind _sm_dresser_drawer4 (Variables|Default|GetSM_Dresser_Drawer4))
  (bind _sm_dresser_mirrors (Variables|Default|GetSM_Dresser_Mirrors))
  (bind _sm_dresser_drawer2 (Variables|Default|GetSM_Dresser_Drawer2))
  (bind _sm_dresser_drawer7 (Variables|Default|GetSM_Dresser_Drawer7))
  (bind _sm_handle_drawer3 (Variables|Default|GetSM_Handle_Drawer3))
  (bind _sm_handle_drawer4 (Variables|Default|GetSM_Handle_Drawer4))
  (bind _sm_handle_drawer2 (Variables|Default|GetSM_Handle_Drawer2))
  (bind _sm_handle_drawer7 (Variables|Default|GetSM_Handle_Drawer7))
  (bind _sm_handle_drawer8 (Variables|Default|GetSM_Handle_Drawer8))
  (bind _sm_handle_drawer1 (Variables|Default|GetSM_Handle_Drawer1))
  (bind _sm_dresser_base (Variables|Default|GetSM_Dresser_Base))
  (bind _dresser_type (Variables|Default|GetDresser%20Type))
  (bind _sm_dresser_drawer5 (Variables|Default|GetSM_Dresser_Drawer5))
  (bind _sm_dresser_drawer6 (Variables|Default|GetSM_Dresser_Drawer6))
  (bind _sm_handle_drawer5 (Variables|Default|GetSM_Handle_Drawer5))
  (bind _sm_handle_drawer6 (Variables|Default|GetSM_Handle_Drawer6))
  (switch Utilities|FlowControl|Switch|SwitchonDresserTypes_Enum (Variables|Default|GetDresser%20Type)
    (:NewEnumerator2
      (bind _outrownames (DataTable|GetDataTableRowNames "/Game/InteriorBuildingKit/Struct/Dressers_Narrow_DataTable.Dressers_Narrow_DataTable"))
      (bind _returnvalue (Utilities|GetDataTableRow "/Game/InteriorBuildingKit/Struct/Dressers_Narrow_DataTable.Dressers_Narrow_DataTable" (Utilities|Array|Get(acopy) _outrownames (Variables|Default|GetDresser%20Option)) :!label _label)
        (:then
          (Variables|Variables|SetDrawer%201%20-%20Location (.drawer1startinglocation _returnvalue))
          (Variables|Variables|SetDrawer%202%20-%20Location (.drawer2startinglocation _returnvalue))
          (Variables|Variables|SetDrawer%203%20-%20Location (.drawer3startinglocation _returnvalue))
          (Variables|Variables|SetDrawer%204%20-%20Location (.drawer4startinglocation _returnvalue))
          (Variables|Variables|SetDrawer%205%20-%20Location (.drawer5startinglocation _returnvalue))
          (Variables|Variables|SetDrawer%206%20-%20Location (.drawer6startinglocation _returnvalue))
          (Variables|Variables|SetDrawer%207%20-%20Location (.drawer7startinglocation _returnvalue))
          (Variables|Variables|SetDrawer%208%20-%20Location (.drawer8startinglocation _returnvalue))
          (Variables|Variables|SetOpen%20State%20Draw%20Distance%20%28Temp%29 (.maxdrawerpulloutdistanceglobal _returnvalue)))
        (:RowNotFound
          (Variables|Default|SetDresser%20Option (- (Utilities|Array|Length _outrownames) 1))
          (goto _label))))
    (:NewEnumerator0
      (bind _outrownames_2 (DataTable|GetDataTableRowNames "/Game/InteriorBuildingKit/Struct/Dressers_Wide_DataTable.Dressers_Wide_DataTable"))
      (bind _returnvalue_2 (Utilities|GetDataTableRow "/Game/InteriorBuildingKit/Struct/Dressers_Wide_DataTable.Dressers_Wide_DataTable" (Utilities|Array|Get(acopy) _outrownames_2 (Variables|Default|GetDresser%20Option)) :!label _label_2)
        (:then
          (Variables|Variables|SetDrawer%201%20-%20Location (.drawer1startinglocation _returnvalue_2))
          (Variables|Variables|SetDrawer%202%20-%20Location (.drawer2startinglocation _returnvalue_2))
          (Variables|Variables|SetDrawer%203%20-%20Location (.drawer3startinglocation _returnvalue_2))
          (Variables|Variables|SetDrawer%204%20-%20Location (.drawer4startinglocation _returnvalue_2))
          (Variables|Variables|SetDrawer%205%20-%20Location (.drawer5startinglocation _returnvalue_2))
          (Variables|Variables|SetDrawer%206%20-%20Location (.drawer6startinglocation _returnvalue_2))
          (Variables|Variables|SetDrawer%207%20-%20Location (.drawer7startinglocation _returnvalue_2))
          (Variables|Variables|SetDrawer%208%20-%20Location (.drawer8startinglocation _returnvalue_2))
          (Variables|Variables|SetOpen%20State%20Draw%20Distance%20%28Temp%29 (.maxdrawerpulloutdistanceglobal _returnvalue_2)))
        (:RowNotFound
          (Variables|Default|SetDresser%20Option (- (Utilities|Array|Length _outrownames_2) 1))
          (goto _label_2))))
    (:NewEnumerator1
      (bind _outrownames_3 (DataTable|GetDataTableRowNames "/Game/InteriorBuildingKit/Struct/Dressers_Tall_DataTable.Dressers_Tall_DataTable"))
      (bind _returnvalue_3 (Utilities|GetDataTableRow "/Game/InteriorBuildingKit/Struct/Dressers_Tall_DataTable.Dressers_Tall_DataTable" (Utilities|Array|Get(acopy) _outrownames_3 (Variables|Default|GetDresser%20Option)) :!label _label_3)
        (:then
          (Variables|Variables|SetDrawer%201%20-%20Location (.drawer1startinglocation _returnvalue_3))
          (Variables|Variables|SetDrawer%202%20-%20Location (.drawer2startinglocation _returnvalue_3))
          (Variables|Variables|SetDrawer%203%20-%20Location (.drawer3startinglocation _returnvalue_3))
          (Variables|Variables|SetDrawer%204%20-%20Location (.drawer4startinglocation _returnvalue_3))
          (Variables|Variables|SetDrawer%205%20-%20Location (.drawer5startinglocation _returnvalue_3))
          (Variables|Variables|SetDrawer%206%20-%20Location (.drawer6startinglocation _returnvalue_3))
          (Variables|Variables|SetDrawer%207%20-%20Location (.drawer7startinglocation _returnvalue_3))
          (Variables|Variables|SetDrawer%208%20-%20Location (.drawer8startinglocation _returnvalue_3))
          (Variables|Variables|SetOpen%20State%20Draw%20Distance%20%28Temp%29 (.maxdrawerpulloutdistanceglobal _returnvalue_3)))
        (:RowNotFound
          (Variables|Default|SetDresser%20Option (- (Utilities|Array|Length _outrownames_3) 1))
          (goto _label_3)))))
  (Utilities|FlowControl|Sequence
    (:then_0
      (if (> (Variables|Default|GetOpen%20State%20-%20Drawer%201) (Variables|Variables|GetOpen%20State%20Draw%20Distance%20%28Temp%29))
        (Variables|Default|SetOpen%20State%20-%20Drawer%201 (Variables|Variables|GetOpen%20State%20Draw%20Distance%20%28Temp%29))))
    (:then_1
      (if (> (Variables|Default|GetOpen%20State%20-%20Drawer%202) (Variables|Variables|GetOpen%20State%20Draw%20Distance%20%28Temp%29))
        (Variables|Default|SetOpen%20State%20-%20Drawer%202 (Variables|Variables|GetOpen%20State%20Draw%20Distance%20%28Temp%29))))
    (:then_2
      (if (> (Variables|Default|GetOpen%20State%20-%20Drawer%203) (Variables|Variables|GetOpen%20State%20Draw%20Distance%20%28Temp%29))
        (Variables|Default|SetOpen%20State%20-%20Drawer%203 (Variables|Variables|GetOpen%20State%20Draw%20Distance%20%28Temp%29))))
    (:then_3
      (if (> (Variables|Default|GetOpen%20State%20-%20Drawer%204) (Variables|Variables|GetOpen%20State%20Draw%20Distance%20%28Temp%29))
        (Variables|Default|SetOpen%20State%20-%20Drawer%204 (Variables|Variables|GetOpen%20State%20Draw%20Distance%20%28Temp%29))))
    (:then_4
      (if (> (Variables|Default|GetOpen%20State%20-%20Drawer%205) (Variables|Variables|GetOpen%20State%20Draw%20Distance%20%28Temp%29))
        (Variables|Default|SetOpen%20State%20-%20Drawer%205 (Variables|Variables|GetOpen%20State%20Draw%20Distance%20%28Temp%29))))
    (:then_5
      (if (> (Variables|Default|GetOpen%20State%20-%20Drawer%206) (Variables|Variables|GetOpen%20State%20Draw%20Distance%20%28Temp%29))
        (Variables|Default|SetOpen%20State%20-%20Drawer%206 (Variables|Variables|GetOpen%20State%20Draw%20Distance%20%28Temp%29))))
    (:then_6
      (if (> (Variables|Default|GetOpen%20State%20-%20Drawer%207) (Variables|Variables|GetOpen%20State%20Draw%20Distance%20%28Temp%29))
        (Variables|Default|SetOpen%20State%20-%20Drawer%207 (Variables|Variables|GetOpen%20State%20Draw%20Distance%20%28Temp%29))))
    (:then_7
      (if (> (Variables|Default|GetOpen%20State%20-%20Drawer%208) (Variables|Variables|GetOpen%20State%20Draw%20Distance%20%28Temp%29))
        (Variables|Default|SetOpen%20State%20-%20Drawer%208 (Variables|Variables|GetOpen%20State%20Draw%20Distance%20%28Temp%29))))
    (:then_8
      (Components|StaticMesh|SetStaticMesh _sm_dresser_base (Utilities|Select :Index _dresser_type :NewEnumerator2 (.maindrawermesh _returnvalue) :NewEnumerator0 (.maindrawermesh _returnvalue_2) :NewEnumerator1 (.maindrawermesh _returnvalue_3)))
      (Rendering|Material|SetMaterial _sm_dresser_base 0 (Variables|Default|GetNew%20Dresser%20Material))
      (if (Variables|Default|GetUse%20Mirror%20if%20applicable?)
        (Utilities|IsValid (Utilities|Select :Index _dresser_type :NewEnumerator2 (.dressermirrormeshifapplicable _returnvalue) :NewEnumerator0 (.dressermirrormeshifapplicable _returnvalue_2) :NewEnumerator1 (.dressermirrormeshifapplicable _returnvalue_3))
          (:Is%20Valid
            (Components|StaticMesh|SetStaticMesh _sm_dresser_mirrors (Utilities|Select :Index _dresser_type :NewEnumerator2 (.dressermirrormeshifapplicable _returnvalue) :NewEnumerator0 (.dressermirrormeshifapplicable _returnvalue_2) :NewEnumerator1 (.dressermirrormeshifapplicable _returnvalue_3)))
            (Rendering|Material|SetMaterial _sm_dresser_mirrors 0 (Variables|Default|GetNew%20Dresser%20Material)))
          (:Is%20Not%20Valid
            (Components|DestroyComponent _sm_dresser_mirrors :!label _label_4)))
        (else
          (goto _label_4)))
      (Utilities|IsValid (Utilities|Select :Index _dresser_type :NewEnumerator2 (.drawer1mesh _returnvalue) :NewEnumerator0 (.drawer1mesh _returnvalue_2) :NewEnumerator1 (.drawer1mesh _returnvalue_3))
        (:Is%20Valid
          (Components|StaticMesh|SetStaticMesh _sm_dresser_drawer1 (Utilities|Select :Index _dresser_type :NewEnumerator2 (.drawer1mesh _returnvalue) :NewEnumerator0 (.drawer1mesh _returnvalue_2) :NewEnumerator1 (.drawer1mesh _returnvalue_3)))
          (Transformation|SetRelativeLocation _sm_dresser_drawer1 (+ (Variables|Variables|GetDrawer%201%20-%20Location) (Math|Vector|MakeVector 0.0 (Variables|Default|GetOpen%20State%20-%20Drawer%201) 0.0)) false true)
          (Rendering|Material|SetMaterial _sm_dresser_drawer1 0 (Variables|Default|GetNew%20Dresser%20Material)))
        (:Is%20Not%20Valid
          (Components|DestroyComponent _sm_dresser_drawer1)))
      (Utilities|IsValid (Utilities|Select :Index _dresser_type :NewEnumerator2 (.drawer2mesh _returnvalue) :NewEnumerator0 (.drawer2mesh _returnvalue_2) :NewEnumerator1 (.drawer2mesh _returnvalue_3))
        (:Is%20Valid
          (Components|StaticMesh|SetStaticMesh _sm_dresser_drawer2 (Utilities|Select :Index _dresser_type :NewEnumerator2 (.drawer2mesh _returnvalue) :NewEnumerator0 (.drawer2mesh _returnvalue_2) :NewEnumerator1 (.drawer2mesh _returnvalue_3)))
          (Transformation|SetRelativeLocation _sm_dresser_drawer2 (+ (Variables|Variables|GetDrawer%202%20-%20Location) (Math|Vector|MakeVector 0.0 (Variables|Default|GetOpen%20State%20-%20Drawer%202) 0.0)) false true)
          (Rendering|Material|SetMaterial _sm_dresser_drawer2 0 (Variables|Default|GetNew%20Dresser%20Material)))
        (:Is%20Not%20Valid
          (Components|DestroyComponent _sm_dresser_drawer2)))
      (Utilities|IsValid (Utilities|Select :Index _dresser_type :NewEnumerator2 (.drawer3mesh _returnvalue) :NewEnumerator0 (.drawer3mesh _returnvalue_2) :NewEnumerator1 (.drawer3mesh _returnvalue_3))
        (:Is%20Valid
          (Components|StaticMesh|SetStaticMesh _sm_dresser_drawer3 (Utilities|Select :Index _dresser_type :NewEnumerator2 (.drawer3mesh _returnvalue) :NewEnumerator0 (.drawer3mesh _returnvalue_2) :NewEnumerator1 (.drawer3mesh _returnvalue_3)))
          (Transformation|SetRelativeLocation _sm_dresser_drawer3 (+ (Variables|Variables|GetDrawer%203%20-%20Location) (Math|Vector|MakeVector 0.0 (Variables|Default|GetOpen%20State%20-%20Drawer%203) 0.0)) false true)
          (Rendering|Material|SetMaterial _sm_dresser_drawer3 0 (Variables|Default|GetNew%20Dresser%20Material)))
        (:Is%20Not%20Valid
          (Components|DestroyComponent _sm_dresser_drawer3)))
      (Utilities|IsValid (Utilities|Select :Index _dresser_type :NewEnumerator2 (.drawer4mesh _returnvalue) :NewEnumerator0 (.drawer4mesh _returnvalue_2) :NewEnumerator1 (.drawer4mesh _returnvalue_3))
        (:Is%20Valid
          (Components|StaticMesh|SetStaticMesh _sm_dresser_drawer4 (Utilities|Select :Index _dresser_type :NewEnumerator2 (.drawer4mesh _returnvalue) :NewEnumerator0 (.drawer4mesh _returnvalue_2) :NewEnumerator1 (.drawer4mesh _returnvalue_3)))
          (Transformation|SetRelativeLocation _sm_dresser_drawer4 (+ (Variables|Variables|GetDrawer%204%20-%20Location) (Math|Vector|MakeVector 0.0 (Variables|Default|GetOpen%20State%20-%20Drawer%204) 0.0)) false true)
          (Rendering|Material|SetMaterial _sm_dresser_drawer4 0 (Variables|Default|GetNew%20Dresser%20Material)))
        (:Is%20Not%20Valid
          (Components|DestroyComponent _sm_dresser_drawer4)))
      (Utilities|IsValid (Utilities|Select :Index _dresser_type :NewEnumerator2 (.drawer5mesh _returnvalue) :NewEnumerator0 (.drawer5mesh _returnvalue_2) :NewEnumerator1 (.drawer5mesh _returnvalue_3))
        (:Is%20Valid
          (Components|StaticMesh|SetStaticMesh _sm_dresser_drawer5 (Utilities|Select :Index _dresser_type :NewEnumerator2 (.drawer5mesh _returnvalue) :NewEnumerator0 (.drawer5mesh _returnvalue_2) :NewEnumerator1 (.drawer5mesh _returnvalue_3)))
          (Transformation|SetRelativeLocation _sm_dresser_drawer5 (+ (Variables|Variables|GetDrawer%205%20-%20Location) (Math|Vector|MakeVector 0.0 (Variables|Default|GetOpen%20State%20-%20Drawer%205) 0.0)) false true)
          (Rendering|Material|SetMaterial _sm_dresser_drawer5 0 (Variables|Default|GetNew%20Dresser%20Material)))
        (:Is%20Not%20Valid
          (Components|DestroyComponent _sm_dresser_drawer5)))
      (Utilities|IsValid (Utilities|Select :Index _dresser_type :NewEnumerator2 (.drawer6mesh _returnvalue) :NewEnumerator0 (.drawer6mesh _returnvalue_2) :NewEnumerator1 (.drawer6mesh _returnvalue_3))
        (:Is%20Valid
          (Components|StaticMesh|SetStaticMesh _sm_dresser_drawer6 (Utilities|Select :Index _dresser_type :NewEnumerator2 (.drawer6mesh _returnvalue) :NewEnumerator0 (.drawer6mesh _returnvalue_2) :NewEnumerator1 (.drawer6mesh _returnvalue_3)))
          (Transformation|SetRelativeLocation _sm_dresser_drawer6 (+ (Variables|Variables|GetDrawer%206%20-%20Location) (Math|Vector|MakeVector 0.0 (Variables|Default|GetOpen%20State%20-%20Drawer%206) 0.0)) false true)
          (Rendering|Material|SetMaterial _sm_dresser_drawer6 0 (Variables|Default|GetNew%20Dresser%20Material)))
        (:Is%20Not%20Valid
          (Components|DestroyComponent _sm_dresser_drawer6)))
      (Utilities|IsValid (Utilities|Select :Index _dresser_type :NewEnumerator2 (.drawer7mesh _returnvalue) :NewEnumerator0 (.drawer7mesh _returnvalue_2) :NewEnumerator1 (.drawer7mesh _returnvalue_3))
        (:Is%20Valid
          (Components|StaticMesh|SetStaticMesh _sm_dresser_drawer7 (Utilities|Select :Index _dresser_type :NewEnumerator2 (.drawer7mesh _returnvalue) :NewEnumerator0 (.drawer7mesh _returnvalue_2) :NewEnumerator1 (.drawer7mesh _returnvalue_3)))
          (Transformation|SetRelativeLocation _sm_dresser_drawer7 (+ (Variables|Variables|GetDrawer%207%20-%20Location) (Math|Vector|MakeVector 0.0 (Variables|Default|GetOpen%20State%20-%20Drawer%207) 0.0)) false true)
          (Rendering|Material|SetMaterial _sm_dresser_drawer7 0 (Variables|Default|GetNew%20Dresser%20Material)))
        (:Is%20Not%20Valid
          (Components|DestroyComponent _sm_dresser_drawer7)))
      (Utilities|IsValid (Utilities|Select :Index _dresser_type :NewEnumerator2 (.drawer8mesh _returnvalue) :NewEnumerator0 (.drawer8mesh _returnvalue_2) :NewEnumerator1 (.drawer8mesh _returnvalue_3))
        (:Is%20Valid
          (Components|StaticMesh|SetStaticMesh _sm_dresser_drawer8 (Utilities|Select :Index _dresser_type :NewEnumerator2 (.drawer8mesh _returnvalue) :NewEnumerator0 (.drawer8mesh _returnvalue_2) :NewEnumerator1 (.drawer8mesh _returnvalue_3)))
          (Transformation|SetRelativeLocation _sm_dresser_drawer8 (+ (Variables|Variables|GetDrawer%208%20-%20Location) (Math|Vector|MakeVector 0.0 (Variables|Default|GetOpen%20State%20-%20Drawer%208) 0.0)) false true)
          (Rendering|Material|SetMaterial _sm_dresser_drawer8 0 (Variables|Default|GetNew%20Dresser%20Material)))
        (:Is%20Not%20Valid
          (Components|DestroyComponent _sm_dresser_drawer8)))
      (bind _returnvalue_4 (Utilities|GetDataTableRow "/Game/InteriorBuildingKit/Struct/CounterHandleTypes_DataTable.CounterHandleTypes_DataTable" (Utilities|String|StringToName (Utilities|String|EnumtoString (Variables|Default|GetHandle%20Type))))
        (:then
          (if (>= (Variables|Default|GetHandle%20Option) (Utilities|Array|Length (.handletype _returnvalue_4)))
            (Variables|Default|SetHandle%20Option (- (Utilities|Array|Length (.handletype _returnvalue_4)) 1)))
          (Utilities|IsValid _sm_handle_drawer1
            (:Is%20Valid
              (Components|StaticMesh|SetStaticMesh _sm_handle_drawer1 (Utilities|Array|Get(acopy) (.handletype _returnvalue_4) (Variables|Default|GetHandle%20Option)))
              (Rendering|Material|SetMaterial _sm_handle_drawer1 0 (Variables|Default|GetNew%20Handle%20Material)))
            (:Is%20Not%20Valid
              _))
          (Utilities|IsValid _sm_handle_drawer2
            (:Is%20Valid
              (Components|StaticMesh|SetStaticMesh _sm_handle_drawer2 (Utilities|Array|Get(acopy) (.handletype _returnvalue_4) (Variables|Default|GetHandle%20Option)))
              (Rendering|Material|SetMaterial _sm_handle_drawer2 0 (Variables|Default|GetNew%20Handle%20Material)))
            (:Is%20Not%20Valid
              _))
          (Utilities|IsValid _sm_handle_drawer3
            (:Is%20Valid
              (Components|StaticMesh|SetStaticMesh _sm_handle_drawer3 (Utilities|Array|Get(acopy) (.handletype _returnvalue_4) (Variables|Default|GetHandle%20Option)))
              (Rendering|Material|SetMaterial _sm_handle_drawer3 0 (Variables|Default|GetNew%20Handle%20Material)))
            (:Is%20Not%20Valid
              _))
          (Utilities|IsValid _sm_handle_drawer4
            (:Is%20Valid
              (Components|StaticMesh|SetStaticMesh _sm_handle_drawer4 (Utilities|Array|Get(acopy) (.handletype _returnvalue_4) (Variables|Default|GetHandle%20Option)))
              (Rendering|Material|SetMaterial _sm_handle_drawer4 0 (Variables|Default|GetNew%20Handle%20Material)))
            (:Is%20Not%20Valid
              _))
          (Utilities|IsValid _sm_handle_drawer5
            (:Is%20Valid
              (Components|StaticMesh|SetStaticMesh _sm_handle_drawer5 (Utilities|Array|Get(acopy) (.handletype _returnvalue_4) (Variables|Default|GetHandle%20Option)))
              (Rendering|Material|SetMaterial _sm_handle_drawer5 0 (Variables|Default|GetNew%20Handle%20Material)))
            (:Is%20Not%20Valid
              _))
          (Utilities|IsValid _sm_handle_drawer6
            (:Is%20Valid
              (Components|StaticMesh|SetStaticMesh _sm_handle_drawer6 (Utilities|Array|Get(acopy) (.handletype _returnvalue_4) (Variables|Default|GetHandle%20Option)))
              (Rendering|Material|SetMaterial _sm_handle_drawer6 0 (Variables|Default|GetNew%20Handle%20Material)))
            (:Is%20Not%20Valid
              _))
          (Utilities|IsValid _sm_handle_drawer7
            (:Is%20Valid
              (Components|StaticMesh|SetStaticMesh _sm_handle_drawer7 (Utilities|Array|Get(acopy) (.handletype _returnvalue_4) (Variables|Default|GetHandle%20Option)))
              (Rendering|Material|SetMaterial _sm_handle_drawer7 0 (Variables|Default|GetNew%20Handle%20Material)))
            (:Is%20Not%20Valid
              _))
          (Utilities|IsValid _sm_handle_drawer8
            (:Is%20Valid
              (Components|StaticMesh|SetStaticMesh _sm_handle_drawer8 (Utilities|Array|Get(acopy) (.handletype _returnvalue_4) (Variables|Default|GetHandle%20Option)))
              (Rendering|Material|SetMaterial _sm_handle_drawer8 0 (Variables|Default|GetNew%20Handle%20Material)))))))))