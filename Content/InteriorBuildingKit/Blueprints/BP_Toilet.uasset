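; BP_Toilet is a toilet prop from the interior building kit with an adjustable lid, seat and water mesh.
; The Construction Script rotates lid and seat on roll from their open-strength values, raising the lid value to at least the seat's so the seat never opens past the lid.
; WaterOption selects between two water meshes.
; The event graph is empty, so the asset has no runtime logic.
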(event EventBeginPlay)

(event Collision|EventActorBeginOverlap
  (params (OtherActor :type Actor%20Object%20Reference)))

(event EventTick
  (params (DeltaSeconds :type Float%20%28single-precision%29)))

(fn ConstructionScript
  (if (> (Variables|Default|GetSeat%20Open%20Strength) (Variables|Default|GetLid%20Open%20Strength))
    (Variables|Default|SetLid%20Open%20Strength (Variables|Default|GetSeat%20Open%20Strength)))
  (Transformation|SetRelativeRotation (Variables|Default|GetSM_Toilet01_Lid) (Math|Rotator|MakeRotator (Math|Float|Lerp 0.0 -1e+02 (Variables|Default|GetLid%20Open%20Strength)) 0.0 0.0) false false)
  (Transformation|SetRelativeRotation (Variables|Default|GetSM_Toilet01_Seat) (Math|Rotator|MakeRotator (Math|Float|Lerp 0.0 -1e+02 (Variables|Default|GetSeat%20Open%20Strength)) 0.0 0.0) false false)
  (Components|StaticMesh|SetStaticMesh (Variables|Default|GetSM_Toilet01_Water) (Utilities|Select :Index (Variables|Default|GetWater%20Option) :Option%200 "/Game/InteriorBuildingKit/Geometry/Assets/Bathroom/Toilets/SM_Toilet01_Water2.SM_Toilet01_Water2" :Option%201 "/Game/InteriorBuildingKit/Geometry/Assets/Bathroom/Toilets/SM_Toilet01_Water1.SM_Toilet01_Water1")))