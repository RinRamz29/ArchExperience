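; BP_Desk_01 is a desk prop from the interior building kit with individually adjustable drawers and a secret door.
; The Construction Script slides each left, middle and right drawer along its relative X axis in proportion to its open-state variable.
; The secret door instead swings in yaw, interpolated by its own open state.
; Poses are set only at construction, as the event graph has no active runtime logic.
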(event EventBeginPlay)

(event Collision|EventActorBeginOverlap
  (params (OtherActor :type Actor%20Object%20Reference)))

(event EventTick
  (params (DeltaSeconds :type Float%20%28single-precision%29)))

(fn ConstructionScript
  (Transformation|SetRelativeLocation (Variables|Default|GetSM_Desk_Door_L1) (Math|Vector|MakeVector (* (Variables|Default|GetOpen%20State%20-%20Drawer%20L1) -5e+01) 0.0 0.0) false false)
  (Transformation|SetRelativeLocation (Variables|Default|GetSM_Desk_Door_L2) (Math|Vector|MakeVector (* (Variables|Default|GetOpen%20State%20-%20Drawer%20L2) -5e+01) 0.0 0.0) false false)
  (Transformation|SetRelativeLocation (Variables|Default|GetSM_Desk_Door_L3) (Math|Vector|MakeVector (* (Variables|Default|GetOpen%20State%20-%20Drawer%20L3) -5e+01) 0.0 0.0) false false)
  (Transformation|SetRelativeLocation (Variables|Default|GetSM_Desk_Door_L4) (Math|Vector|MakeVector (* (Variables|Default|GetOpen%20State%20-%20Drawer%20L4) -5e+01) 0.0 0.0) false false)
  (Transformation|SetRelativeLocation (Variables|Default|GetSM_Desk_Door_M1) (Math|Vector|MakeVector (* (Variables|Default|GetOpen%20State%20-%20Drawer%20M1) -5e+01) 0.0 0.0) false false)
  (Transformation|SetRelativeRotation (Variables|Default|GetSM_Desk_SecretDoor) (Math|Rotator|MakeRotator 0.0 0.0 (Math|Float|Lerp -9e+01 -179.0 (Variables|Default|GetOpen%20State%20-%20Drawer%20Secret))) false false)
  (Transformation|SetRelativeLocation (Variables|Default|GetSM_Desk_Door_R1) (Math|Vector|MakeVector (* (Variables|Default|GetOpen%20State%20-%20Drawer%20R1) -5e+01) 0.0 0.0) false false)
  (Transformation|SetRelativeLocation (Variables|Default|GetSM_Desk_Door_R2) (Math|Vector|MakeVector (* (Variables|Default|GetOpen%20State%20-%20Drawer%20R2) -5e+01) 0.0 0.0) false false)
  (Transformation|SetRelativeLocation (Variables|Default|GetSM_Desk_Door_R3) (Math|Vector|MakeVector (* (Variables|Default|GetOpen%20State%20-%20Drawer%20R3) -5e+01) 0.0 0.0) false false)
  (Transformation|SetRelativeLocation (Variables|Default|GetSM_Desk_Door_R4) (Math|Vector|MakeVector (* (Variables|Default|GetOpen%20State%20-%20Drawer%20R4) -5e+01) 0.0 0.0) false false))