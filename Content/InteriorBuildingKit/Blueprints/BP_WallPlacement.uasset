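; Interior-kit wall actor that builds itself in the construction script from a clamped Destination end point.
; Height and window options pick a data table, and length buckets select the trim or plain mesh, plus optional exterior siding per side.
; Window meshes spawn at table-stored transforms, with out-of-range variation indices reset to the last row.
; The wall and siding then optionally scale to snap to Destination, and the wall gets wallpaper, edge and trim materials.
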(event EventBeginPlay)

(event Collision|EventActorBeginOverlap
  (params (OtherActor :type Actor%20Object%20Reference)))

(event EventTick
  (params (DeltaSeconds :type Float%20%28single-precision%29)))

(fn ConstructionScript
  (bind _sm_wall (Variables|Default|GetSM_Wall))
  (bind (_min _max) (Components|StaticMesh|GetLocalBounds _sm_wall))
  (Variables|Default|SetDestination (Math|Vector|MakeVector 0.0 (Math|Float|Clamp(Float) (.y (Variables|Default|GetDestination)) -1.5e+03 -5e+01) (Math|Float|Clamp(Float) (.z (Variables|Default|GetDestination)) 5e+01 1.5e+03)))
  (if (Variables|Default|GetDoes%20wall%20have%20windows?) ; Has Windows?
    (if (> (.z (Variables|Default|GetDestination)) 328.0) ; Is tall?
      (bind _outrownames (DataTable|GetDataTableRowNames "/Game/InteriorBuildingKit/Struct/WallsWindowed_Tall_DataTable.WallsWindowed_Tall_DataTable"))
      (bind _returnvalue (Utilities|GetDataTableRow "/Game/InteriorBuildingKit/Struct/WallsWindowed_Tall_DataTable.WallsWindowed_Tall_DataTable" (Utilities|Array|Get(acopy) _outrownames (Variables|Default|GetWindow%20Cuttout%20Variation)) :!label _label)
        (:then
          (Components|StaticMesh|SetStaticMesh (Variables|Default|GetSM_Wall) (Utilities|Select :Index (Variables|Default|GetWall%20Type) :NewEnumerator0 (Utilities|Select :Index (+ (Math|Conversions|ToInteger(Boolean) (> (* (.y (Variables|Default|GetDestination)) -1.0) 3e+02)) (Math|Conversions|ToInteger(Boolean) (> (* (.y (Variables|Default|GetDestination)) -1.0) 5e+02)) (Math|Conversions|ToInteger(Boolean) (> (* (.y (Variables|Default|GetDestination)) -1.0) 725.0))) :Option%200 (.withtrim-mesh200 _returnvalue) :Option%201 (.withtrim-mesh400 _returnvalue) :Option%202 (.withtrim-mesh600 _returnvalue) :Option%203 (.withtrim-mesh850 _returnvalue)) :NewEnumerator1 (Utilities|Select :Index (+ (Math|Conversions|ToInteger(Boolean) (> (* (.y (Variables|Default|GetDestination)) -1.0) 3e+02)) (Math|Conversions|ToInteger(Boolean) (> (* (.y (Variables|Default|GetDestination)) -1.0) 5e+02)) (Math|Conversions|ToInteger(Boolean) (> (* (.y (Variables|Default|GetDestination)) -1.0) 725.0))) :Option%200 (.withouttrim-mesh200 _returnvalue) :Option%201 (.withouttrim-mesh400 _returnvalue) :Option%202 (.withouttrim-mesh600 _returnvalue) :Option%203 (.withouttrim-mesh850 _returnvalue))))
          (Variables|Variables|SetWindow%20Location%20Array (select (Utilities|Enum|Equal(Enum) (Variables|Default|GetWall%20Type) "NewEnumerator0") (Utilities|Select :Index (+ (Math|Conversions|ToInteger(Boolean) (> (* (.y (Variables|Default|GetDestination)) -1.0) 3e+02)) (Math|Conversions|ToInteger(Boolean) (> (* (.y (Variables|Default|GetDestination)) -1.0) 5e+02)) (Math|Conversions|ToInteger(Boolean) (> (* (.y (Variables|Default|GetDestination)) -1.0) 725.0))) :Option%200 (.windowlocations-withtrim-mesh200 _returnvalue) :Option%201 (.windowlocations-withtrim-mesh400 _returnvalue) :Option%202 (.windowlocations-withtrim-mesh600 _returnvalue) :Option%203 (.windowlocations-withtrim-mesh850 _returnvalue)) (Utilities|Select :Index (+ (Math|Conversions|ToInteger(Boolean) (> (* (.y (Variables|Default|GetDestination)) -1.0) 3e+02)) (Math|Conversions|ToInteger(Boolean) (> (* (.y (Variables|Default|GetDestination)) -1.0) 5e+02)) (Math|Conversions|ToInteger(Boolean) (> (* (.y (Variables|Default|GetDestination)) -1.0) 725.0))) :Option%200 (.windowlocations-withouttrim-mesh200 _returnvalue) :Option%201 (.windowlocations-withouttrim-mesh400 _returnvalue) :Option%202 (.windowlocations-withouttrim-mesh600 _returnvalue) :Option%203 (.windowlocations-withouttrim-mesh850 _returnvalue))))
          (Utilities|FlowControl|Sequence
            (:then_0
              (if (Variables|Default|GetAdd%20siding%20on%20Left%20side?)
                (bind _returnvalue_2 (AddComponent|AddStaticMeshComponent false (Math|Transform|MakeTransform (Math|Vector|MakeVector (* (Variables|Default|GetWall%20thickness%20%28In%20units%29) -1.0) 0.0 0.0) "0, 0, 0" "1.000000,1.000000,1.000000")))
                (bind _output_get (Variables|Default|SetExterior%20Reference%20-%20Left%20Side _returnvalue_2))
                (Components|StaticMesh|SetStaticMesh _output_get (Utilities|Select :Index (+ (Math|Conversions|ToInteger(Boolean) (> (* (.y (Variables|Default|GetDestination)) -1.0) 3e+02)) (Math|Conversions|ToInteger(Boolean) (> (* (.y (Variables|Default|GetDestination)) -1.0) 5e+02)) (Math|Conversions|ToInteger(Boolean) (> (* (.y (Variables|Default|GetDestination)) -1.0) 725.0))) :Option%200 (.exterior-mesh200 _returnvalue) :Option%201 (.exterior-mesh400 _returnvalue) :Option%202 (.exterior-mesh600 _returnvalue) :Option%203 (.exterior-mesh850 _returnvalue)))))
            (:then_1
              (if (Variables|Default|GetAdd%20siding%20on%20Right%20Side?)
                (bind _returnvalue_3 (AddComponent|AddStaticMeshComponent false))
                (bind _output_get_2 (Variables|Default|SetExterior%20Reference%20-%20Right%20Side _returnvalue_3))
                (Components|StaticMesh|SetStaticMesh _output_get_2 (Utilities|Select :Index (+ (Math|Conversions|ToInteger(Boolean) (> (* (.y (Variables|Default|GetDestination)) -1.0) 3e+02)) (Math|Conversions|ToInteger(Boolean) (> (* (.y (Variables|Default|GetDestination)) -1.0) 5e+02)) (Math|Conversions|ToInteger(Boolean) (> (* (.y (Variables|Default|GetDestination)) -1.0) 725.0))) :Option%200 (.exterior-mesh200 _returnvalue) :Option%201 (.exterior-mesh400 _returnvalue) :Option%202 (.exterior-mesh600 _returnvalue) :Option%203 (.exterior-mesh850 _returnvalue)))))
            (:then_2
              (bind _outrownames_2 (DataTable|GetDataTableRowNames "/Game/InteriorBuildingKit/Struct/WallsWindowVariations_DataTable.WallsWindowVariations_DataTable" :!label _label_2))
              (bind _returnvalue_4 (Utilities|GetDataTableRow "/Game/InteriorBuildingKit/Struct/WallsWindowVariations_DataTable.WallsWindowVariations_DataTable" (Utilities|Array|Get(acopy) _outrownames_2 (Variables|Default|GetWindow%20Variation)) :!label _label_3)
                (:then
                  (for _array_element (Variables|Variables|GetWindow%20Location%20Array)
                    (bind _returnvalue_5 (AddComponent|AddStaticMeshComponent false _array_element))
                    (Components|StaticMesh|SetStaticMesh _returnvalue_5 (Utilities|Select :Index (Variables|Default|GetWindow%20Cuttout%20Variation) :Option%200 (.windowvariation1 _returnvalue_4) :Option%201 (.windowvariation2 _returnvalue_4) :Option%202 (.windowvariation3 _returnvalue_4) :Option%203 (.windowvariation4 _returnvalue_4)))
                    (Transformation|AttachComponentToComponent _returnvalue_5 (Variables|Default|GetSM_Wall) "None" "KeepRelative" "KeepRelative" "KeepRelative" true))
                  (Transformation|SetRelativeScale3D (Variables|Default|GetSM_Wall) (Math|Vector|MakeVector (/ (Math|Conversions|ToFloat(Integer) (Variables|Default|GetWall%20thickness%20%28In%20units%29)) 25.0) (select (Variables|Default|GetSnap%20Length%20to%20end%20point?) (/ (.y (Variables|Default|GetDestination)) (.y _min)) 1.0) (select (Variables|Default|GetSnap%20height%20to%20end%20point?) (/ (.z (Variables|Default|GetDestination)) (.z _max)) 1.0)) :!label _label_4)
                  (Utilities|IsValid (Variables|Default|GetExterior%20Reference%20-%20Left%20Side)
                    (:Is%20Valid
                      (Transformation|SetRelativeScale3D (Variables|Default|GetExterior%20Reference%20-%20Left%20Side) (Math|Vector|MakeVector 1.0 (select (Variables|Default|GetSnap%20Length%20to%20end%20point?) (/ (.y (Variables|Default|GetDestination)) (.y _min)) 1.0) (select (Variables|Default|GetSnap%20height%20to%20end%20point?) (/ (.z (Variables|Default|GetDestination)) (.z _max)) 1.0))))
                    (:Is%20Not%20Valid
                      _))
                  (Utilities|IsValid (Variables|Default|GetExterior%20Reference%20-%20Right%20Side)
                    (:Is%20Valid
                      (Transformation|SetRelativeScale3D (Variables|Default|GetExterior%20Reference%20-%20Right%20Side) (Math|Vector|MakeVector -1.0 (select (Variables|Default|GetSnap%20Length%20to%20end%20point?) (/ (.y (Variables|Default|GetDestination)) (.y _min)) 1.0) (select (Variables|Default|GetSnap%20height%20to%20end%20point?) (/ (.z (Variables|Default|GetDestination)) (.z _max)) 1.0))))
                    (:Is%20Not%20Valid
                      _))
                  (Rendering|Material|SetMaterial (Variables|Default|GetSM_Wall) (select (Variables|Default|GetDoes%20wall%20have%20windows?) 2 (Utilities|Select :Index (Variables|Default|GetWall%20Type) :NewEnumerator0 2 :NewEnumerator1 1)) (Variables|Default|GetWallpaper%20Material%20-%20Left%20Side))
                  (Rendering|Material|SetMaterial (Variables|Default|GetSM_Wall) (select (Variables|Default|GetDoes%20wall%20have%20windows?) 3 (Utilities|Select :Index (Variables|Default|GetWall%20Type) :NewEnumerator0 3 :NewEnumerator1 2)) (Variables|Default|GetWallpaper%20Material%20-%20%20Right%20Side))
                  (Rendering|Material|SetMaterial (Variables|Default|GetSM_Wall) (select (Variables|Default|GetDoes%20wall%20have%20windows?) 1 (Utilities|Select :Index (Variables|Default|GetWall%20Type) :NewEnumerator0 1 :NewEnumerator1 0)) (Variables|Default|GetEdge%20Material))
                  (if (Utilities|Enum|Equal(Enum) (Variables|Default|GetWall%20Type) "NewEnumerator0")
                    (Rendering|Material|SetMaterial (Variables|Default|GetSM_Wall) 0 (Variables|Default|GetTrim%20Material))))
                (:RowNotFound
                  (Variables|Default|SetWindow%20Variation (- (Utilities|Array|Length _outrownames_2) 1))
                  (goto _label_3))))))
        (:RowNotFound
          (Variables|Default|SetWindow%20Cuttout%20Variation (- (Utilities|Array|Length _outrownames) 1))
          (goto _label)))
      (else
        (bind _outrownames_3 (DataTable|GetDataTableRowNames "/Game/InteriorBuildingKit/Struct/WallsWindowed_Reg_DataTable.WallsWindowed_Reg_DataTable"))
        (bind _returnvalue_6 (Utilities|GetDataTableRow "/Game/InteriorBuildingKit/Struct/WallsWindowed_Reg_DataTable.WallsWindowed_Reg_DataTable" (Utilities|Array|Get(acopy) _outrownames_3 (Variables|Default|GetWindow%20Cuttout%20Variation)) :!label _label_5)
          (:then
            (Components|StaticMesh|SetStaticMesh (Variables|Default|GetSM_Wall) (Utilities|Select :Index (Variables|Default|GetWall%20Type) :NewEnumerator0 (Utilities|Select :Index (+ (Math|Conversions|ToInteger(Boolean) (> (* (.y (Variables|Default|GetDestination)) -1.0) 3e+02)) (Math|Conversions|ToInteger(Boolean) (> (* (.y (Variables|Default|GetDestination)) -1.0) 5e+02)) (Math|Conversions|ToInteger(Boolean) (> (* (.y (Variables|Default|GetDestination)) -1.0) 725.0))) :Option%200 (.withtrim-mesh200 _returnvalue_6) :Option%201 (.withtrim-mesh400 _returnvalue_6) :Option%202 (.withtrim-mesh600 _returnvalue_6) :Option%203 (.withtrim-mesh850 _returnvalue_6)) :NewEnumerator1 (Utilities|Select :Index (+ (Math|Conversions|ToInteger(Boolean) (> (* (.y (Variables|Default|GetDestination)) -1.0) 3e+02)) (Math|Conversions|ToInteger(Boolean) (> (* (.y (Variables|Default|GetDestination)) -1.0) 5e+02)) (Math|Conversions|ToInteger(Boolean) (> (* (.y (Variables|Default|GetDestination)) -1.0) 725.0))) :Option%200 (.withouttrim-mesh200 _returnvalue_6) :Option%201 (.withouttrim-mesh400 _returnvalue_6) :Option%202 (.withouttrim-mesh600 _returnvalue_6) :Option%203 (.withouttrim-mesh850 _returnvalue_6))))
            (Variables|Variables|SetWindow%20Location%20Array (select (Utilities|Enum|Equal(Enum) (Variables|Default|GetWall%20Type) "NewEnumerator0") (Utilities|Select :Index (+ (Math|Conversions|ToInteger(Boolean) (> (* (.y (Variables|Default|GetDestination)) -1.0) 3e+02)) (Math|Conversions|ToInteger(Boolean) (> (* (.y (Variables|Default|GetDestination)) -1.0) 5e+02)) (Math|Conversions|ToInteger(Boolean) (> (* (.y (Variables|Default|GetDestination)) -1.0) 725.0))) :Option%200 (.windowlocations-withtrim-mesh200 _returnvalue_6) :Option%201 (.windowlocations-withtrim-mesh400 _returnvalue_6) :Option%202 (.windowlocations-withtrim-mesh600 _returnvalue_6) :Option%203 (.windowlocations-withtrim-mesh850 _returnvalue_6)) (Utilities|Select :Index (+ (Math|Conversions|ToInteger(Boolean) (> (* (.y (Variables|Default|GetDestination)) -1.0) 3e+02)) (Math|Conversions|ToInteger(Boolean) (> (* (.y (Variables|Default|GetDestination)) -1.0) 5e+02)) (Math|Conversions|ToInteger(Boolean) (> (* (.y (Variables|Default|GetDestination)) -1.0) 725.0))) :Option%200 (.windowlocations-withouttrim-mesh200 _returnvalue_6) :Option%201 (.windowlocations-withouttrim-mesh400 _returnvalue_6) :Option%202 (.windowlocations-withouttrim-mesh600 _returnvalue_6) :Option%203 (.windowlocations-withouttrim-mesh850 _returnvalue_6))))
            (Utilities|FlowControl|Sequence
              (:then_0
                (if (Variables|Default|GetAdd%20siding%20on%20Left%20side?)
                  (bind _returnvalue_7 (AddComponent|AddStaticMeshComponent false (Math|Transform|MakeTransform (Math|Vector|MakeVector (* (Variables|Default|GetWall%20thickness%20%28In%20units%29) -1.0) 0.0 0.0) "0, 0, 0" "1.000000,1.000000,1.000000")))
                  (bind _output_get_3 (Variables|Default|SetExterior%20Reference%20-%20Left%20Side _returnvalue_7))
                  (Components|StaticMesh|SetStaticMesh _output_get_3 (Utilities|Select :Index (+ (Math|Conversions|ToInteger(Boolean) (> (* (.y (Variables|Default|GetDestination)) -1.0) 3e+02)) (Math|Conversions|ToInteger(Boolean) (> (* (.y (Variables|Default|GetDestination)) -1.0) 5e+02)) (Math|Conversions|ToInteger(Boolean) (> (* (.y (Variables|Default|GetDestination)) -1.0) 725.0))) :Option%200 (.exterior-mesh200 _returnvalue_6) :Option%201 (.exterior-mesh400 _returnvalue_6) :Option%202 (.exterior-mesh600 _returnvalue_6) :Option%203 (.exterior-mesh850 _returnvalue_6)))))
              (:then_1
                (if (Variables|Default|GetAdd%20siding%20on%20Right%20Side?)
                  (bind _returnvalue_8 (AddComponent|AddStaticMeshComponent false))
                  (bind _output_get_4 (Variables|Default|SetExterior%20Reference%20-%20Right%20Side _returnvalue_8))
                  (Components|StaticMesh|SetStaticMesh _output_get_4 (Utilities|Select :Index (+ (Math|Conversions|ToInteger(Boolean) (> (* (.y (Variables|Default|GetDestination)) -1.0) 3e+02)) (Math|Conversions|ToInteger(Boolean) (> (* (.y (Variables|Default|GetDestination)) -1.0) 5e+02)) (Math|Conversions|ToInteger(Boolean) (> (* (.y (Variables|Default|GetDestination)) -1.0) 725.0))) :Option%200 (.exterior-mesh200 _returnvalue_6) :Option%201 (.exterior-mesh400 _returnvalue_6) :Option%202 (.exterior-mesh600 _returnvalue_6) :Option%203 (.exterior-mesh850 _returnvalue_6)))))
              (:then_2
                (goto _label_2))))
          (:RowNotFound
            (Variables|Default|SetWindow%20Cuttout%20Variation (- (Utilities|Array|Length _outrownames_3) 1))
            (goto _label_5)))))
    (elif (> (.z (Variables|Default|GetDestination)) 328.0) ; Is tall?
      (bind _outrownames_4 (DataTable|GetDataTableRowNames "/Game/InteriorBuildingKit/Struct/WallsBlank_Tall_DataTable.WallsBlank_Tall_DataTable"))
      (bind _returnvalue_9 (Utilities|GetDataTableRow "/Game/InteriorBuildingKit/Struct/WallsBlank_Tall_DataTable.WallsBlank_Tall_DataTable" (Utilities|Array|Get(acopy) _outrownames_4))
        (:then
          (Components|StaticMesh|SetStaticMesh (Variables|Default|GetSM_Wall) (Utilities|Select :Index (Variables|Default|GetWall%20Type) :NewEnumerator0 (Utilities|Select :Index (+ (Math|Conversions|ToInteger(Boolean) (> (* (.y (Variables|Default|GetDestination)) -1.0) 125.0)) (Math|Conversions|ToInteger(Boolean) (> (* (.y (Variables|Default|GetDestination)) -1.0) 175.0)) (Math|Conversions|ToInteger(Boolean) (> (* (.y (Variables|Default|GetDestination)) -1.0) 225.0)) (Math|Conversions|ToInteger(Boolean) (> (* (.y (Variables|Default|GetDestination)) -1.0) 275.0)) (Math|Conversions|ToInteger(Boolean) (> (* (.y (Variables|Default|GetDestination)) -1.0) 3.5e+02)) (Math|Conversions|ToInteger(Boolean) (> (* (.y (Variables|Default|GetDestination)) -1.0) 4.5e+02)) (Math|Conversions|ToInteger(Boolean) (> (* (.y (Variables|Default|GetDestination)) -1.0) 5.5e+02)) (Math|Conversions|ToInteger(Boolean) (> (* (.y (Variables|Default|GetDestination)) -1.0) 6.5e+02)) (Math|Conversions|ToInteger(Boolean) (> (* (.y (Variables|Default|GetDestination)) -1.0) 775.0))) :Option%200 (.withtrim-mesh100 _returnvalue_9) :Option%201 (.withtrim-mesh150 _returnvalue_9) :Option%202 (.withtrim-mesh200 _returnvalue_9) :Option%203 (.withtrim-mesh250 _returnvalue_9) :Option%204 (.withtrim-mesh300 _returnvalue_9) :Option%205 (.withtrim-mesh400 _returnvalue_9) :Option%206 (.withtrim-mesh500 _returnvalue_9) :Option%207 (.withtrim-mesh600 _returnvalue_9) :Option%208 (.withtrim-mesh700 _returnvalue_9) :Option%209 (.withtrim-mesh850 _returnvalue_9)) :NewEnumerator1 (Utilities|Select :Index (+ (Math|Conversions|ToInteger(Boolean) (> (* (.y (Variables|Default|GetDestination)) -1.0) 125.0)) (Math|Conversions|ToInteger(Boolean) (> (* (.y (Variables|Default|GetDestination)) -1.0) 175.0)) (Math|Conversions|ToInteger(Boolean) (> (* (.y (Variables|Default|GetDestination)) -1.0) 225.0)) (Math|Conversions|ToInteger(Boolean) (> (* (.y (Variables|Default|GetDestination)) -1.0) 275.0)) (Math|Conversions|ToInteger(Boolean) (> (* (.y (Variables|Default|GetDestination)) -1.0) 3.5e+02)) (Math|Conversions|ToInteger(Boolean) (> (* (.y (Variables|Default|GetDestination)) -1.0) 4.5e+02)) (Math|Conversions|ToInteger(Boolean) (> (* (.y (Variables|Default|GetDestination)) -1.0) 5.5e+02)) (Math|Conversions|ToInteger(Boolean) (> (* (.y (Variables|Default|GetDestination)) -1.0) 6.5e+02)) (Math|Conversions|ToInteger(Boolean) (> (* (.y (Variables|Default|GetDestination)) -1.0) 775.0))) :Option%200 (.withouttrim-mesh100 _returnvalue_9) :Option%201 (.withouttrim-mesh150 _returnvalue_9) :Option%202 (.withouttrim-mesh200 _returnvalue_9) :Option%203 (.withouttrim-mesh250 _returnvalue_9) :Option%204 (.withouttrim-mesh300 _returnvalue_9) :Option%205 (.withouttrim-mesh400 _returnvalue_9) :Option%206 (.withouttrim-mesh500 _returnvalue_9) :Option%207 (.withouttrim-mesh600 _returnvalue_9) :Option%208 (.withouttrim-mesh700 _returnvalue_9) :Option%209 (.withouttrim-mesh850 _returnvalue_9))))
          (Utilities|FlowControl|Sequence
            (:then_0
              (if (Variables|Default|GetAdd%20siding%20on%20Left%20side?)
                (bind _returnvalue_10 (AddComponent|AddStaticMeshComponent false (Math|Transform|MakeTransform (Math|Vector|MakeVector (* (Variables|Default|GetWall%20thickness%20%28In%20units%29) -1.0) 0.0 0.0) "0, 0, 0" "1.000000,1.000000,1.000000")))
                (bind _output_get_5 (Variables|Default|SetExterior%20Reference%20-%20Left%20Side _returnvalue_10))
                (Components|StaticMesh|SetStaticMesh _output_get_5 (Utilities|Select :Index (+ (Math|Conversions|ToInteger(Boolean) (> (* (.y (Variables|Default|GetDestination)) -1.0) 125.0)) (Math|Conversions|ToInteger(Boolean) (> (* (.y (Variables|Default|GetDestination)) -1.0) 175.0)) (Math|Conversions|ToInteger(Boolean) (> (* (.y (Variables|Default|GetDestination)) -1.0) 225.0)) (Math|Conversions|ToInteger(Boolean) (> (* (.y (Variables|Default|GetDestination)) -1.0) 275.0)) (Math|Conversions|ToInteger(Boolean) (> (* (.y (Variables|Default|GetDestination)) -1.0) 3.5e+02)) (Math|Conversions|ToInteger(Boolean) (> (* (.y (Variables|Default|GetDestination)) -1.0) 4.5e+02)) (Math|Conversions|ToInteger(Boolean) (> (* (.y (Variables|Default|GetDestination)) -1.0) 5.5e+02)) (Math|Conversions|ToInteger(Boolean) (> (* (.y (Variables|Default|GetDestination)) -1.0) 6.5e+02)) (Math|Conversions|ToInteger(Boolean) (> (* (.y (Variables|Default|GetDestination)) -1.0) 775.0))) :Option%200 (.exterior-mesh100 _returnvalue_9) :Option%201 (.exterior-mesh150 _returnvalue_9) :Option%202 (.exterior-mesh200 _returnvalue_9) :Option%203 (.exterior-mesh250 _returnvalue_9) :Option%204 (.exterior-mesh300 _returnvalue_9) :Option%205 (.exterior-mesh400 _returnvalue_9) :Option%206 (.exterior-mesh500 _returnvalue_9) :Option%207 (.exterior-mesh600 _returnvalue_9) :Option%208 (.exterior-mesh700 _returnvalue_9) :Option%209 (.exterior-mesh850 _returnvalue_9)))))
            (:then_1
              (if (Variables|Default|GetAdd%20siding%20on%20Right%20Side?)
                (bind _returnvalue_11 (AddComponent|AddStaticMeshComponent false))
                (bind _output_get_6 (Variables|Default|SetExterior%20Reference%20-%20Right%20Side _returnvalue_11))
                (Components|StaticMesh|SetStaticMesh _output_get_6 (Utilities|Select :Index (+ (Math|Conversions|ToInteger(Boolean) (> (* (.y (Variables|Default|GetDestination)) -1.0) 125.0)) (Math|Conversions|ToInteger(Boolean) (> (* (.y (Variables|Default|GetDestination)) -1.0) 175.0)) (Math|Conversions|ToInteger(Boolean) (> (* (.y (Variables|Default|GetDestination)) -1.0) 225.0)) (Math|Conversions|ToInteger(Boolean) (> (* (.y (Variables|Default|GetDestination)) -1.0) 275.0)) (Math|Conversions|ToInteger(Boolean) (> (* (.y (Variables|Default|GetDestination)) -1.0) 3.5e+02)) (Math|Conversions|ToInteger(Boolean) (> (* (.y (Variables|Default|GetDestination)) -1.0) 4.5e+02)) (Math|Conversions|ToInteger(Boolean) (> (* (.y (Variables|Default|GetDestination)) -1.0) 5.5e+02)) (Math|Conversions|ToInteger(Boolean) (> (* (.y (Variables|Default|GetDestination)) -1.0) 6.5e+02)) (Math|Conversions|ToInteger(Boolean) (> (* (.y (Variables|Default|GetDestination)) -1.0) 775.0))) :Option%200 (.exterior-mesh100 _returnvalue_9) :Option%201 (.exterior-mesh150 _returnvalue_9) :Option%202 (.exterior-mesh200 _returnvalue_9) :Option%203 (.exterior-mesh250 _returnvalue_9) :Option%204 (.exterior-mesh300 _returnvalue_9) :Option%205 (.exterior-mesh400 _returnvalue_9) :Option%206 (.exterior-mesh500 _returnvalue_9) :Option%207 (.exterior-mesh600 _returnvalue_9) :Option%208 (.exterior-mesh700 _returnvalue_9) :Option%209 (.exterior-mesh850 _returnvalue_9)))))
            (:then_2
              (goto _label_4)))))
      (else
        (bind _outrownames_5 (DataTable|GetDataTableRowNames "/Game/InteriorBuildingKit/Struct/WallsBlank_Reg_DataTable.WallsBlank_Reg_DataTable"))
        (bind _returnvalue_12 (Utilities|GetDataTableRow "/Game/InteriorBuildingKit/Struct/WallsBlank_Reg_DataTable.WallsBlank_Reg_DataTable" (Utilities|Array|Get(acopy) _outrownames_5))
          (:then
            (Components|StaticMesh|SetStaticMesh (Variables|Default|GetSM_Wall) (Utilities|Select :Index (Variables|Default|GetWall%20Type) :NewEnumerator0 (Utilities|Select :Index (+ (Math|Conversions|ToInteger(Boolean) (> (* (.y (Variables|Default|GetDestination)) -1.0) 125.0)) (Math|Conversions|ToInteger(Boolean) (> (* (.y (Variables|Default|GetDestination)) -1.0) 175.0)) (Math|Conversions|ToInteger(Boolean) (> (* (.y (Variables|Default|GetDestination)) -1.0) 225.0)) (Math|Conversions|ToInteger(Boolean) (> (* (.y (Variables|Default|GetDestination)) -1.0) 275.0)) (Math|Conversions|ToInteger(Boolean) (> (* (.y (Variables|Default|GetDestination)) -1.0) 3.5e+02)) (Math|Conversions|ToInteger(Boolean) (> (* (.y (Variables|Default|GetDestination)) -1.0) 4.5e+02)) (Math|Conversions|ToInteger(Boolean) (> (* (.y (Variables|Default|GetDestination)) -1.0) 5.5e+02)) (Math|Conversions|ToInteger(Boolean) (> (* (.y (Variables|Default|GetDestination)) -1.0) 6.5e+02)) (Math|Conversions|ToInteger(Boolean) (> (* (.y (Variables|Default|GetDestination)) -1.0) 775.0))) :Option%200 (.withtrim-mesh100 _returnvalue_12) :Option%201 (.withtrim-mesh150 _returnvalue_12) :Option%202 (.withtrim-mesh200 _returnvalue_12) :Option%203 (.withtrim-mesh250 _returnvalue_12) :Option%204 (.withtrim-mesh300 _returnvalue_12) :Option%205 (.withtrim-mesh400 _returnvalue_12) :Option%206 (.withtrim-mesh500 _returnvalue_12) :Option%207 (.withtrim-mesh600 _returnvalue_12) :Option%208 (.withtrim-mesh700 _returnvalue_12) :Option%209 (.withtrim-mesh850 _returnvalue_12)) :NewEnumerator1 (Utilities|Select :Index (+ (Math|Conversions|ToInteger(Boolean) (> (* (.y (Variables|Default|GetDestination)) -1.0) 125.0)) (Math|Conversions|ToInteger(Boolean) (> (* (.y (Variables|Default|GetDestination)) -1.0) 175.0)) (Math|Conversions|ToInteger(Boolean) (> (* (.y (Variables|Default|GetDestination)) -1.0) 225.0)) (Math|Conversions|ToInteger(Boolean) (> (* (.y (Variables|Default|GetDestination)) -1.0) 275.0)) (Math|Conversions|ToInteger(Boolean) (> (* (.y (Variables|Default|GetDestination)) -1.0) 3.5e+02)) (Math|Conversions|ToInteger(Boolean) (> (* (.y (Variables|Default|GetDestination)) -1.0) 4.5e+02)) (Math|Conversions|ToInteger(Boolean) (> (* (.y (Variables|Default|GetDestination)) -1.0) 5.5e+02)) (Math|Conversions|ToInteger(Boolean) (> (* (.y (Variables|Default|GetDestination)) -1.0) 6.5e+02)) (Math|Conversions|ToInteger(Boolean) (> (* (.y (Variables|Default|GetDestination)) -1.0) 775.0))) :Option%200 (.withouttrim-mesh100 _returnvalue_12) :Option%201 (.withouttrim-mesh150 _returnvalue_12) :Option%202 (.withouttrim-mesh200 _returnvalue_12) :Option%203 (.withouttrim-mesh250 _returnvalue_12) :Option%204 (.withouttrim-mesh300 _returnvalue_12) :Option%205 (.withouttrim-mesh400 _returnvalue_12) :Option%206 (.withouttrim-mesh500 _returnvalue_12) :Option%207 (.withouttrim-mesh600 _returnvalue_12) :Option%208 (.withouttrim-mesh700 _returnvalue_12) :Option%209 (.withouttrim-mesh850 _returnvalue_12))))
            (Utilities|FlowControl|Sequence
              (:then_0
                (if (Variables|Default|GetAdd%20siding%20on%20Left%20side?)
                  (bind _returnvalue_13 (AddComponent|AddStaticMeshComponent false (Math|Transform|MakeTransform (Math|Vector|MakeVector (* (Variables|Default|GetWall%20thickness%20%28In%20units%29) -1.0) 0.0 0.0) "0, 0, 0" "1.000000,1.000000,1.000000")))
                  (bind _output_get_7 (Variables|Default|SetExterior%20Reference%20-%20Left%20Side _returnvalue_13))
                  (Components|StaticMesh|SetStaticMesh _output_get_7 (Utilities|Select :Index (+ (Math|Conversions|ToInteger(Boolean) (> (* (.y (Variables|Default|GetDestination)) -1.0) 125.0)) (Math|Conversions|ToInteger(Boolean) (> (* (.y (Variables|Default|GetDestination)) -1.0) 175.0)) (Math|Conversions|ToInteger(Boolean) (> (* (.y (Variables|Default|GetDestination)) -1.0) 225.0)) (Math|Conversions|ToInteger(Boolean) (> (* (.y (Variables|Default|GetDestination)) -1.0) 275.0)) (Math|Conversions|ToInteger(Boolean) (> (* (.y (Variables|Default|GetDestination)) -1.0) 3.5e+02)) (Math|Conversions|ToInteger(Boolean) (> (* (.y (Variables|Default|GetDestination)) -1.0) 4.5e+02)) (Math|Conversions|ToInteger(Boolean) (> (* (.y (Variables|Default|GetDestination)) -1.0) 5.5e+02)) (Math|Conversions|ToInteger(Boolean) (> (* (.y (Variables|Default|GetDestination)) -1.0) 6.5e+02)) (Math|Conversions|ToInteger(Boolean) (> (* (.y (Variables|Default|GetDestination)) -1.0) 775.0))) :Option%200 (.exterior-mesh100 _returnvalue_12) :Option%201 (.exterior-mesh150 _returnvalue_12) :Option%202 (.exterior-mesh200 _returnvalue_12) :Option%203 (.exterior-mesh250 _returnvalue_12) :Option%204 (.exterior-mesh300 _returnvalue_12) :Option%205 (.exterior-mesh400 _returnvalue_12) :Option%206 (.exterior-mesh500 _returnvalue_12) :Option%207 (.exterior-mesh600 _returnvalue_12) :Option%208 (.exterior-mesh700 _returnvalue_12) :Option%209 (.exterior-mesh850 _returnvalue_12)))))
              (:then_1
                (if (Variables|Default|GetAdd%20siding%20on%20Right%20Side?)
                  (bind _returnvalue_14 (AddComponent|AddStaticMeshComponent false))
                  (bind _output_get_8 (Variables|Default|SetExterior%20Reference%20-%20Right%20Side _returnvalue_14))
                  (Components|StaticMesh|SetStaticMesh _output_get_8 (Utilities|Select :Index (+ (Math|Conversions|ToInteger(Boolean) (> (* (.y (Variables|Default|GetDestination)) -1.0) 125.0)) (Math|Conversions|ToInteger(Boolean) (> (* (.y (Variables|Default|GetDestination)) -1.0) 175.0)) (Math|Conversions|ToInteger(Boolean) (> (* (.y (Variables|Default|GetDestination)) -1.0) 225.0)) (Math|Conversions|ToInteger(Boolean) (> (* (.y (Variables|Default|GetDestination)) -1.0) 275.0)) (Math|Conversions|ToInteger(Boolean) (> (* (.y (Variables|Default|GetDestination)) -1.0) 3.5e+02)) (Math|Conversions|ToInteger(Boolean) (> (* (.y (Variables|Default|GetDestination)) -1.0) 4.5e+02)) (Math|Conversions|ToInteger(Boolean) (> (* (.y (Variables|Default|GetDestination)) -1.0) 5.5e+02)) (Math|Conversions|ToInteger(Boolean) (> (* (.y (Variables|Default|GetDestination)) -1.0) 6.5e+02)) (Math|Conversions|ToInteger(Boolean) (> (* (.y (Variables|Default|GetDestination)) -1.0) 775.0))) :Option%200 (.exterior-mesh100 _returnvalue_12) :Option%201 (.exterior-mesh150 _returnvalue_12) :Option%202 (.exterior-mesh200 _returnvalue_12) :Option%203 (.exterior-mesh250 _returnvalue_12) :Option%204 (.exterior-mesh300 _returnvalue_12) :Option%205 (.exterior-mesh400 _returnvalue_12) :Option%206 (.exterior-mesh500 _returnvalue_12) :Option%207 (.exterior-mesh600 _returnvalue_12) :Option%208 (.exterior-mesh700 _returnvalue_12) :Option%209 (.exterior-mesh850 _returnvalue_12)))))
              (:then_2
                (goto _label_4)))))))))