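; A TV prop actor that plays a playlist of video URLs on its screen, in a wall or floor mounted variant.
; The construction script takes mesh and screen transform from the first TV_DataTable row and constructs a MediaPlayer and MediaTexture per instance.
; BeginPlay feeds that texture into a dynamic screen material and links the sound.
; When a video ends, the next plays sequentially with wraparound or at random without immediate repeats.
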(event Custom|Video%20Ended
  (bind _media_player (Variables|StoredComponents|GetMedia%20Player))
  (bind _url_to_load_videos (Variables|Default|GetURL%20to%20load%20videos))
  (bind _returnvalue (Utilities|Array|Length _url_to_load_videos))
  (if (Variables|Default|GetRandomize%20Playback%20position?)
    (if (> _returnvalue 1)
      (bind _output_get (Variables|Counter|SetURL%20Counter%20%28Random%20Check%29 (Math|Random|RandomIntegerinRange 0 (- _returnvalue 1)) :!label _label))
      (if (== _output_get (Variables|Counter|GetURL%20Counter))
        (Utilities|FlowControl|Delay 0.1)
        (goto _label)
        (else
          (Variables|Counter|SetURL%20Counter _output_get))))
    (elif (== (Variables|Counter|GetURL%20Counter) (- (Utilities|Array|Length (Variables|Default|GetURL%20to%20load%20videos)) 1))
      (Variables|Counter|SetURL%20Counter 0)
      (else
        (Variables|Counter|SetURL%20Counter (+ (Variables|Counter|GetURL%20Counter) 1)))))
  (Class|MediaPlayer|OpenUrl _media_player (Utilities|Array|Get(acopy) (Variables|Default|GetURL%20to%20load%20videos) (Variables|Counter|GetURL%20Counter)))
  (Media|MediaPlayer|Play _media_player :!class /Script/MediaAssets.MediaPlayer))

(event EventBeginPlay
  (bind _media_player (Variables|StoredComponents|GetMedia%20Player))
  (if (not (== (Utilities|Array|Length (Variables|Default|GetURL%20to%20load%20videos)) 0))
    (Rendering|SetVisibility (Variables|Default|GetScreen) true false)
    (Audio|Components|Audio|SetVolumeMultiplier (Variables|Default|GetMediaSound) (Variables|Default|GetMaster%20Volume) :!class /Script/AudioMixer.SynthComponent)
    (bind _returnvalue (Rendering|Material|CreateDynamicMaterialInstance "/Game/InteriorBuildingKit/Material/Base/M_TV_Base.M_TV_Base" "None" "None" :!class /Script/Engine.KismetMaterialLibrary))
    (Variables|StoredComponents|SetDynamic%20Material%20Instance _returnvalue)
    (Rendering|Material|SetMaterial (Variables|Default|GetScreen) 0 (Variables|StoredComponents|GetDynamic%20Material%20Instance))
    (Rendering|Material|SetTextureParameterValue (Variables|StoredComponents|GetDynamic%20Material%20Instance) "Image" (Variables|StoredComponents|GetMedia%20Texture))
    (EventDispatchers|AssignOnEndReached (Variables|StoredComponents|GetMedia%20Player) (delegate Custom|Video%20Ended))
    (Variables|/Script/MediaAssets.MediaPlayer|SetPlayOnOpen _media_player true)
    (Media|MediaSoundComponent|SetMediaPlayer (Variables|Default|GetMediaSound) _media_player)
    (Media|MediaSoundComponent|SetMediaPlayer (Variables|StoredComponents|GetMedia%20Texture) _media_player)
    (Class|MediaPlayer|OpenUrl _media_player (Utilities|Array|Get(acopy) (Variables|Default|GetURL%20to%20load%20videos) (Math|Integer|SelectInt (Math|Random|RandomIntegerinRange 0 (- (Utilities|Array|Length (Variables|Default|GetURL%20to%20load%20videos)) 1)) 0 (Variables|Default|GetRandomize%20Playback%20Start%20position?))))
    (Media|MediaPlayer|Play _media_player :!class /Script/MediaAssets.MediaPlayer)))

(event Collision|EventActorBeginOverlap
  (params (OtherActor :type Actor%20Object%20Reference)))

(event EventTick
  (params (DeltaSeconds :type Float%20%28single-precision%29)))

(fn ConstructionScript
  (bind _is_this_a_wall_mounted_tv_ (Variables|Default|GetIs%20this%20a%20wall%20mounted%20TV?))
  (bind _outrownames (DataTable|GetDataTableRowNames "/Game/InteriorBuildingKit/Struct/TV_DataTable.TV_DataTable"))
  (bind _returnvalue (Utilities|GetDataTableRow "/Game/InteriorBuildingKit/Struct/TV_DataTable.TV_DataTable" (Utilities|Array|Get(acopy) _outrownames))
    (:then
      (Components|StaticMesh|SetStaticMesh (Variables|Default|GetSM_TV) (select _is_this_a_wall_mounted_tv_ (.wallmountedmesh _returnvalue) (.floormountedmesh _returnvalue)))
      (Transformation|SetRelativeTransform (Variables|Default|GetScreen) (Math|Transform|SelectTransform (.wallmountedtvscreentransform _returnvalue) (.floormountedtvscreentransform _returnvalue) _is_this_a_wall_mounted_tv_) false false)
      (bind _returnvalue_2 (Game|ConstructObjectfromClass self "/Script/MediaAssets.MediaPlayer"))
      (Variables|StoredComponents|SetMedia%20Player _returnvalue_2)
      (bind _returnvalue_3 (Game|ConstructObjectfromClass self "/Script/MediaAssets.MediaTexture"))
      (Variables|StoredComponents|SetMedia%20Texture _returnvalue_3))))