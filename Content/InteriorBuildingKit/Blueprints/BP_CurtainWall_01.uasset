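; Modular curtain wall piece for an interior building kit, configured entirely in the construction script with no active runtime logic.
; CurtainType picks one of three curtain meshes and destroys the rope components that do not match that style.
; FlipCurtains mirrors the curtain through negative Y scale and swaps which side's rope is up or down for the middle style.
; Optional material overrides apply to the wall and curtain when set.
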(event EventBeginPlay)

(event Collision|EventActorBeginOverlap
  (params (OtherActor :type Actor%20Object%20Reference)))

(event EventTick
  (params (DeltaSeconds :type Float%20%28single-precision%29)))

(fn ConstructionScript
  (bind _curtain_type (Variables|Default|GetCurtain%20Type))
  (Utilities|FlowControl|Sequence
    (:then_0
      (if (== _curtain_type 0)
        (Components|DestroyComponent (Variables|Default|GetSM_CurtainRope_Down-Left))))
    (:then_1
      (if (== _curtain_type 1)
        (if (Variables|Default|GetFlip%20Curtains?)
          (Components|DestroyComponent (Variables|Default|GetSM_CurtainRope_Up-Left))
          (else
            (Components|DestroyComponent (Variables|Default|GetSM_CurtainRope_Down-Left))))))
    (:then_2
      (if (== _curtain_type 2)
        (Components|DestroyComponent (Variables|Default|GetSM_CurtainRope_Up-Right))))
    (:then_3
      (Components|StaticMesh|SetStaticMesh (Variables|Default|GetCurtain) (Utilities|Select :Index (Variables|Default|GetCurtain%20Type) :Option%200 "/Game/InteriorBuildingKit/Geometry/Assets/Curtains/SM_CurtainsB.SM_CurtainsB" :Option%201 "/Game/InteriorBuildingKit/Geometry/Assets/Curtains/SM_Curtains2B.SM_Curtains2B" :Option%202 "/Game/InteriorBuildingKit/Geometry/Assets/Curtains/SM_Curtains3.SM_Curtains3"))
      (Transformation|SetRelativeScale3D (Variables|Default|GetCurtain) (Math|Vector|MakeVector 1.0 (Math|Float|SelectFloat -0.785 0.785 (Variables|Default|GetFlip%20Curtains?)) 1.125))
      (Utilities|FlowControl|Sequence
        (:then_0
          (Utilities|IsValid (Variables|Default|GetWall%20Material)
            (:Is%20Valid
              (Rendering|Material|SetMaterial (Variables|Default|GetWall) (Variables|Default|GetWall%20Material%20ID) (Variables|Default|GetWall%20Material)))))
        (:then_1
          (Utilities|IsValid (Variables|Default|GetCurtain%20Material)
            (:Is%20Valid
              (Rendering|Material|SetMaterial (Variables|Default|GetCurtain) 0 (Variables|Default|GetCurtain%20Material)))))))))