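; BP_LightMaskingBox is a resizable box from an interior building kit, evidently for masking light, with individually toggleable sides.
; The construction script sizes and places six BoxCorner components from the Location vector divided by 100, destroying hidden sides.
; Sides are thin slabs, using negative scale on far faces to extend inward.
; With all six sides shown, it keeps only the bottom component, scaled into one solid box.
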(event EventBeginPlay)

(event Collision|EventActorBeginOverlap
  (params (OtherActor :type Actor%20Object%20Reference)))

(event EventTick
  (params (DeltaSeconds :type Float%20%28single-precision%29)))

(fn ConstructionScript
  (bind _box_corner_right (Variables|Default|GetBox_Corner-Right))
  (bind _location (Variables|Default|GetLocation))
  (bind _box_corner_top (Variables|Default|GetBox_Corner-Top))
  (bind _location_2 (Variables|Default|GetLocation))
  (bind _box_corner_left (Variables|Default|GetBox_Corner-Left))
  (bind _location_3 (Variables|Default|GetLocation))
  (bind _box_corner_back (Variables|Default|GetBox_Corner-Back))
  (bind _location_4 (Variables|Default|GetLocation))
  (bind _location_5 (Variables|Default|GetLocation))
  (bind _box_corner_front (Variables|Default|GetBox_Corner-Front))
  (bind _location_6 (Variables|Default|GetLocation))
  (bind _box_corner_bottom (Variables|Default|GetBox_Corner-Bottom))
  (bind _returnvalue (/ _location_4 1e+02))
  (bind _returnvalue_2 (/ _location_2 1e+02))
  (bind _returnvalue_3 (/ _location_3 1e+02))
  (bind _returnvalue_4 (/ _location 1e+02))
  (bind _returnvalue_5 (/ _location_5 1e+02))
  (bind _returnvalue_6 (/ _location_6 1e+02))
  (if (Math|Boolean|ANDBoolean (Variables|Default|GetShow%20Top) (Variables|Default|GetShow%20Bottom) (Variables|Default|GetShow%20Left) (Variables|Default|GetShow%20Right) (Variables|Default|GetShow%20Front) (Variables|Default|GetShow%20Back))
    (Components|DestroyComponent (Variables|Default|GetBox_Corner-Top))
    (Transformation|SetRelativeScale3D (Variables|Default|GetBox_Corner-Bottom) (/ (Variables|Default|GetLocation) 1e+02))
    (else
      (if (Variables|Default|GetShow%20Right)
        (Transformation|SetRelativeTransform _box_corner_right (Math|Transform|MakeTransform (Math|Vector|MakeVector 0.0 0.0 0.0) "0, 0, 0" (Math|Vector|MakeVector 0.1 (.y _returnvalue) (.z _returnvalue))) false true)
        (else
          (Components|DestroyComponent _box_corner_right)))
      (if (Variables|Default|GetShow%20Left)
        (Transformation|SetRelativeTransform _box_corner_left (Math|Transform|MakeTransform (Math|Vector|MakeVector (.x (Variables|Default|GetLocation)) 0.0 0.0) "0, 0, 0" (Math|Vector|MakeVector -0.1 (.y _returnvalue_3) (.z _returnvalue_3))) false true)
        (else
          (Components|DestroyComponent _box_corner_left)))
      (if (Variables|Default|GetShow%20Front)
        (Transformation|SetRelativeTransform _box_corner_front (Math|Transform|MakeTransform (Math|Vector|MakeVector 0.0 (.y (Variables|Default|GetLocation)) 0.0) "0, 0, 0" (Math|Vector|MakeVector (.x _returnvalue_6) -0.1 (.z _returnvalue_6))) false true)
        (else
          (Components|DestroyComponent _box_corner_front)))
      (if (Variables|Default|GetShow%20Back)
        (Transformation|SetRelativeTransform _box_corner_back (Math|Transform|MakeTransform (Math|Vector|MakeVector 0.0 0.0 0.0) "0, 0, 0" (Math|Vector|MakeVector (.x _returnvalue_5) 0.1 (.z _returnvalue_5))) false true)
        (else
          (Components|DestroyComponent _box_corner_back)))
      (if (Variables|Default|GetShow%20Top)
        (Transformation|SetRelativeTransform _box_corner_top (Math|Transform|MakeTransform (Math|Vector|MakeVector 0.0 0.0 (.z (Variables|Default|GetLocation))) "0, 0, 0" (Math|Vector|MakeVector (.x _returnvalue_2) (.y _returnvalue_2) -0.1)) false true)
        (else
          (Components|DestroyComponent _box_corner_top)))
      (if (Variables|Default|GetShow%20Bottom)
        (Transformation|SetRelativeScale3D _box_corner_bottom (Math|Vector|MakeVector (.x _returnvalue_4) (.y _returnvalue_4) 0.1))
        (else
          (Components|DestroyComponent _box_corner_bottom))))))