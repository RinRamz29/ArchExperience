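; Configurable pantry storage unit prop for interiors, with four doors, twelve drawers and optional under-lights, set up entirely in the construction script.
; TurnOnLights either applies the lit material to the under-light meshes or destroys the spot lights.
; Per-part open-state values lerp door yaw and drawer offset.
; A data table row picked by HandleType supplies every handle mesh, with HandleOption capped to the array; the material override reaches only drawer handles.
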(event EventBeginPlay)

(event Collision|EventActorBeginOverlap
  (params (OtherActor :type Actor%20Object%20Reference)))

(event EventTick
  (params (DeltaSeconds :type Float%20%28single-precision%29)))

(fn ConstructionScript
  (if (Variables|Default|GetTurn%20on%20lights?)
    (Rendering|Material|SetMaterial (Variables|Default|GetSM_UnderLight_Left%20Top) 2 "/Game/InteriorBuildingKit/Material/Lighting/Defaults/MI_LightsOn_Default.MI_LightsOn_Default")
    (else
      (Components|DestroyComponent (Variables|Default|GetSpotLight_Right%20Top))))
  (Transformation|SetRelativeRotation (Variables|Default|GetSM_Pantry1_Door1%20Left) (Math|Rotator|MakeRotator 0.0 0.0 (Math|Float|Lerp 0.0 179.0 (Variables|Default|GetOpen%20State%20Door%201%20-%20Left))) false false)
  (Transformation|SetRelativeRotation (Variables|Default|GetSM_Pantry1_Door1%20Right) (Math|Rotator|MakeRotator 0.0 0.0 (Math|Float|Lerp 0.0 -179.0 (Variables|Default|GetOpen%20State%20Door%201%20-%20Right))) false false)
  (Transformation|SetRelativeRotation (Variables|Default|GetSM_Pantry1_Door2%20Left) (Math|Rotator|MakeRotator 0.0 0.0 (Math|Float|Lerp 0.0 179.0 (Variables|Default|GetOpen%20State%20Door%202%20-%20Left))) false false)
  (Transformation|SetRelativeRotation (Variables|Default|GetSM_Pantry1_Door2%20Right) (Math|Rotator|MakeRotator 0.0 0.0 (Math|Float|Lerp 0.0 -179.0 (Variables|Default|GetOpen%20State%20Door%202%20-%20Right))) false false)
  (Transformation|SetRelativeLocation (Variables|Default|GetSM_Pantry1_Drawer1%20A) (Math|Vector|MakeVector -113.5 (Math|Float|Lerp 0.0 35.0 (Variables|Default|GetOpen%20State%20Drawer%201%20-%20A)) 66.25) false true)
  (Transformation|SetRelativeLocation (Variables|Default|GetSM_Pantry1_Drawer1%20B) (Math|Vector|MakeVector -113.5 (Math|Float|Lerp 0.0 35.0 (Variables|Default|GetOpen%20State%20Drawer%201%20-%20B)) 35.650002) false true)
  (Transformation|SetRelativeLocation (Variables|Default|GetSM_Pantry1_Drawer1%20C) (Math|Vector|MakeVector -113.5 (Math|Float|Lerp 0.0 35.0 (Variables|Default|GetOpen%20State%20Drawer%201%20-%20C)) 5.1) false true)
  (Transformation|SetRelativeLocation (Variables|Default|GetSM_Pantry1_Drawer2%20A) (Math|Vector|MakeVector -37.5 (Math|Float|Lerp 0.0 35.0 (Variables|Default|GetOpen%20State%20Drawer%202%20-%20A)) 66.25) false true)
  (Transformation|SetRelativeLocation (Variables|Default|GetSM_Pantry1_Drawer2%20B) (Math|Vector|MakeVector -37.5 (Math|Float|Lerp 0.0 35.0 (Variables|Default|GetOpen%20State%20Drawer%202%20-%20B)) 35.650002) false true)
  (Transformation|SetRelativeLocation (Variables|Default|GetSM_Pantry1_Drawer2%20C) (Math|Vector|MakeVector -37.5 (Math|Float|Lerp 0.0 35.0 (Variables|Default|GetOpen%20State%20Drawer%202%20-%20C)) 5.1) false true)
  (Transformation|SetRelativeLocation (Variables|Default|GetSM_Pantry1_Drawer3%20A) (Math|Vector|MakeVector 37.5 (Math|Float|Lerp 0.0 35.0 (Variables|Default|GetOpen%20State%20Drawer%203%20-%20A)) 66.25) false true)
  (Transformation|SetRelativeLocation (Variables|Default|GetSM_Pantry1_Drawer3%20B) (Math|Vector|MakeVector 37.5 (Math|Float|Lerp 0.0 35.0 (Variables|Default|GetOpen%20State%20Drawer%203%20-%20B)) 35.650002) false true)
  (Transformation|SetRelativeLocation (Variables|Default|GetSM_Pantry1_Drawer3%20C) (Math|Vector|MakeVector 37.5 (Math|Float|Lerp 0.0 35.0 (Variables|Default|GetOpen%20State%20Drawer%203%20-%20C)) 5.1) false true)
  (Transformation|SetRelativeLocation (Variables|Default|GetSM_Pantry1_Drawer4%20A) (Math|Vector|MakeVector 113.5 (Math|Float|Lerp 0.0 35.0 (Variables|Default|GetOpen%20State%20Drawer%204%20-%20A)) 66.25) false true)
  (Transformation|SetRelativeLocation (Variables|Default|GetSM_Pantry1_Drawer4%20B) (Math|Vector|MakeVector 113.5 (Math|Float|Lerp 0.0 35.0 (Variables|Default|GetOpen%20State%20Drawer%204%20-%20B)) 35.650002) false true)
  (Transformation|SetRelativeLocation (Variables|Default|GetSM_Pantry1_Drawer4%20C) (Math|Vector|MakeVector 113.5 (Math|Float|Lerp 0.0 35.0 (Variables|Default|GetOpen%20State%20Drawer%204%20-%20C)) 5.1) false true)
  (bind _returnvalue (Utilities|GetDataTableRow "/Game/InteriorBuildingKit/Struct/CounterHandleTypes_DataTable.CounterHandleTypes_DataTable" (Utilities|String|StringToName (Utilities|String|EnumtoString (Variables|Default|GetHandle%20Type))))
    (:then
      (if (>= (Variables|Default|GetHandle%20Option) (Utilities|Array|Length (.handletype _returnvalue)))
        (Variables|Default|SetHandle%20Option (- (Utilities|Array|Length (.handletype _returnvalue)) 1)))
      (Components|StaticMesh|SetStaticMesh (Variables|Default|GetSM_Handle_Drawer1%20A) (Utilities|Array|Get(acopy) (.handletype _returnvalue) (Variables|Default|GetHandle%20Option)))
      (Components|StaticMesh|SetStaticMesh (Variables|Default|GetSM_Handle_Drawer1%20B) (Utilities|Array|Get(acopy) (.handletype _returnvalue) (Variables|Default|GetHandle%20Option)))
      (Components|StaticMesh|SetStaticMesh (Variables|Default|GetSM_Handle_Drawer1%20C) (Utilities|Array|Get(acopy) (.handletype _returnvalue) (Variables|Default|GetHandle%20Option)))
      (Components|StaticMesh|SetStaticMesh (Variables|Default|GetSM_Handle_Drawer2_A) (Utilities|Array|Get(acopy) (.handletype _returnvalue) (Variables|Default|GetHandle%20Option)))
      (Components|StaticMesh|SetStaticMesh (Variables|Default|GetSM_Handle_Drawer2_B) (Utilities|Array|Get(acopy) (.handletype _returnvalue) (Variables|Default|GetHandle%20Option)))
      (Components|StaticMesh|SetStaticMesh (Variables|Default|GetSM_Handle_Drawer2_C) (Utilities|Array|Get(acopy) (.handletype _returnvalue) (Variables|Default|GetHandle%20Option)))
      (Components|StaticMesh|SetStaticMesh (Variables|Default|GetSM_Handle_Drawer3_A) (Utilities|Array|Get(acopy) (.handletype _returnvalue) (Variables|Default|GetHandle%20Option)))
      (Components|StaticMesh|SetStaticMesh (Variables|Default|GetSM_Handle_Drawer3_B) (Utilities|Array|Get(acopy) (.handletype _returnvalue) (Variables|Default|GetHandle%20Option)))
      (Components|StaticMesh|SetStaticMesh (Variables|Default|GetSM_Handle_Drawer3_C) (Utilities|Array|Get(acopy) (.handletype _returnvalue) (Variables|Default|GetHandle%20Option)))
      (Components|StaticMesh|SetStaticMesh (Variables|Default|GetSM_Handle_Drawer4_A) (Utilities|Array|Get(acopy) (.handletype _returnvalue) (Variables|Default|GetHandle%20Option)))
      (Components|StaticMesh|SetStaticMesh (Variables|Default|GetSM_Handle_Drawer4_B) (Utilities|Array|Get(acopy) (.handletype _returnvalue) (Variables|Default|GetHandle%20Option)))
      (Components|StaticMesh|SetStaticMesh (Variables|Default|GetSM_Handle_Drawer4_C) (Utilities|Array|Get(acopy) (.handletype _returnvalue) (Variables|Default|GetHandle%20Option)))
      (Components|StaticMesh|SetStaticMesh (Variables|Default|GetSM_Handle_Door1%20Right) (Utilities|Array|Get(acopy) (.handletype _returnvalue) (Variables|Default|GetHandle%20Option)))
      (Components|StaticMesh|SetStaticMesh (Variables|Default|GetSM_Handle_Door1%20Left) (Utilities|Array|Get(acopy) (.handletype _returnvalue) (Variables|Default|GetHandle%20Option)))
      (Components|StaticMesh|SetStaticMesh (Variables|Default|GetSM_Handle_Door2_Right) (Utilities|Array|Get(acopy) (.handletype _returnvalue) (Variables|Default|GetHandle%20Option)))
      (Components|StaticMesh|SetStaticMesh (Variables|Default|GetSM_Handle_Door2_Left) (Utilities|Array|Get(acopy) (.handletype _returnvalue) (Variables|Default|GetHandle%20Option)))
      (Rendering|Material|SetMaterial (Variables|Default|GetSM_Handle_Drawer4_C) 0 (Variables|Default|GetNew%20Handle%20Material)))))