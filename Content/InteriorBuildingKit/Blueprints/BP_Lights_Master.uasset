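; Configurable master light fixture for interior wall, ceiling, chandelier or custom lights, built entirely in the Construction Script.
; LightOption indexes the category's or override data table, resetting to the last row if lookup fails.
; That row drives base, glass and bulb meshes, plus spawned Up/Down point or spot lights with optional IES profiles.
; When lit, a dynamic material takes emissive colour from a temperature curve and intensity, and filament materials follow temperature bands.
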(event EventBeginPlay)

(event Collision|EventActorBeginOverlap
  (params (OtherActor :type Actor%20Object%20Reference)))

(event EventTick
  (params (DeltaSeconds :type Float%20%28single-precision%29)))

(fn ConstructionScript
  (bind _cast_ray_trace_shadows_ (Variables|Default|GetCast%20Ray%20Trace%20Shadows?))
  (bind _use_ies_intensity_ (Variables|Default|GetUse%20IES%20intensity?))
  (bind _custom_ies_texture (Variables|Default|GetCustom%20IES%20Texture))
  (bind _use_ies_intensity__2 (Variables|Default|GetUse%20IES%20intensity?))
  (bind _custom_ies_texture_2 (Variables|Default|GetCustom%20IES%20Texture))
  (bind _light_colour (Variables|Default|GetLight%20Colour))
  (bind _cast_ray_trace_shadows__2 (Variables|Default|GetCast%20Ray%20Trace%20Shadows?))
  (bind _attenuation_radius___down (Variables|Default|GetAttenuation%20Radius%20-%20Down))
  (bind _use_ies_intensity__3 (Variables|Default|GetUse%20IES%20intensity?))
  (bind _light_temperature (Variables|Default|GetLight%20Temperature))
  (bind _use_ies_intensity__4 (Variables|Default|GetUse%20IES%20intensity?))
  (bind _cast_dynamic_shadows____down_left_back (Variables|Default|GetCast%20Dynamic%20shadows?%20-%20Down/Left/Back))
  (bind _light_temperature_2 (Variables|Default|GetLight%20Temperature))
  (bind _light_temperature_3 (Variables|Default|GetLight%20Temperature))
  (bind _light_intensity (Variables|Default|GetLight%20Intensity))
  (bind _cast_shadows____down_left_back (Variables|Default|GetCast%20shadows?%20-%20Down/Left/Back))
  (bind _light_indirect_intensity (Variables|Default|GetLight%20Indirect%20Intensity))
  (bind _light_group___up (Variables|Default|GetLight%20Group%20-%20Up))
  (bind _attenuation_radius___up (Variables|Default|GetAttenuation%20Radius%20-%20Up))
  (bind _light_indirect_intensity_2 (Variables|Default|GetLight%20Indirect%20Intensity))
  (bind _use_ies_intensity__5 (Variables|Default|GetUse%20IES%20intensity?))
  (bind _use_ies_intensity__6 (Variables|Default|GetUse%20IES%20intensity?))
  (bind _custom_override_settings_ (Variables|Override|GetCustom%20Override%20Settings?))
  (bind _light_mobility_mode___down (Variables|Default|GetLight%20Mobility%20Mode%20-%20Down))
  (bind _light_mobility_mode___up (Variables|Default|GetLight%20Mobility%20Mode%20-%20Up))
  (bind _lighting_catagory (Variables|Default|GetLighting%20catagory))
  (bind _cast_dynamic_shadows____down_left_back_2 (Variables|Default|GetCast%20Dynamic%20shadows?%20-%20Down/Left/Back))
  (bind _light_intensity_2 (Variables|Default|GetLight%20Intensity))
  (bind _light_colour_2 (Variables|Default|GetLight%20Colour))
  (bind _cast_dynamic_shadows____up_right_forward (Variables|Default|GetCast%20Dynamic%20shadows?%20-%20Up/Right/Forward))
  (bind _cast_dynamic_shadows____up_right_forward_2 (Variables|Default|GetCast%20Dynamic%20shadows?%20-%20Up/Right/Forward))
  (bind _cast_shadows____up_right_forward (Variables|Default|GetCast%20shadows?%20-%20Up/Right/Forward))
  (bind _light_group___down (Variables|Default|GetLight%20Group%20-%20Down))
  (bind _returnvalue (select _use_ies_intensity__3 1e+02 0.1))
  (bind _returnvalue_2 (select _use_ies_intensity__5 1e+02 0.1))
  (bind _returnvalue_3 (/ _light_intensity_2 _returnvalue))
  (bind _returnvalue_4 (/ _light_intensity _returnvalue_2))
  (Transformation|SetRelativeScale3D (Variables|Default|GetMain%20Scaling) (Variables|Default|GetGeometry%20Scale%20Multiplier))
  (if (Variables|Override|GetCustom%20Override%20Settings?)
    (bind _outrownames (DataTable|GetDataTableRowNames "/Game/InteriorBuildingKit/Struct/LightTypes_CustomLights_DataTable.LightTypes_CustomLights_DataTable"))
    (bind _returnvalue_5 (Utilities|GetDataTableRow "/Game/InteriorBuildingKit/Struct/LightTypes_CustomLights_DataTable.LightTypes_CustomLights_DataTable" (Utilities|Array|Get(acopy) _outrownames (Variables|Default|GetLight%20Option)) :!label _label)
      (:then
        (Components|StaticMesh|SetStaticMesh (Variables|Default|GetSM_Wall_Lamp) (select _custom_override_settings_ (.staticmesh-base _returnvalue_5) (Utilities|Select :Index _lighting_catagory :NewEnumerator0 (.staticmesh-base (stale _returnvalue_18)) :NewEnumerator1 (.staticmesh-base (stale _returnvalue_19)) :NewEnumerator2 (.staticmesh-base (stale _returnvalue_20)))) :!label _label_2)
        (Utilities|IsValid (select _custom_override_settings_ (.staticmesh-glass _returnvalue_5) (Utilities|Select :Index _lighting_catagory :NewEnumerator0 (.staticmesh-glass (stale _returnvalue_18)) :NewEnumerator1 (.staticmesh-glass (stale _returnvalue_19)) :NewEnumerator2 (.staticmesh-glass (stale _returnvalue_20))))
          (:Is%20Valid
            (bind _returnvalue_6 (AddComponent|AddStaticMeshComponent false (Math|Transform|MakeTransform (Math|Vector|MakeVector 0.0 0.0 (select _custom_override_settings_ (.glassheight _returnvalue_5) (Utilities|Select :Index _lighting_catagory :NewEnumerator0 (.glassheight (stale _returnvalue_18)) :NewEnumerator1 (.glassheight (stale _returnvalue_19)) :NewEnumerator2 (.glassheight (stale _returnvalue_20))))) "0, 0, 0" "1.000000,1.000000,1.000000")))
            (bind _output_get (Variables|Default|SetLamp%20Glass%20Asset%20Reference _returnvalue_6))
            (Components|StaticMesh|SetStaticMesh _output_get (select _custom_override_settings_ (.staticmesh-glass _returnvalue_5) (Utilities|Select :Index _lighting_catagory :NewEnumerator0 (.staticmesh-glass (stale _returnvalue_18)) :NewEnumerator1 (.staticmesh-glass (stale _returnvalue_19)) :NewEnumerator2 (.staticmesh-glass (stale _returnvalue_20)))))
            (Rendering|SetCastShadow _output_get (not (Variables|Default|GetTurn%20on%20lights?)))
            (Rendering|Material|SetMaterial _output_get (select (Utilities|IsValid (select _custom_override_settings_ (.staticmesh-glass _returnvalue_5) (Utilities|Select :Index _lighting_catagory :NewEnumerator0 (.staticmesh-glass (stale _returnvalue_18)) :NewEnumerator1 (.staticmesh-glass (stale _returnvalue_19)) :NewEnumerator2 (.staticmesh-glass (stale _returnvalue_20))))) (select _custom_override_settings_ (.mainmaterialidchannelformaterialoverride _returnvalue_5) (Utilities|Select :Index _lighting_catagory :NewEnumerator0 (.mainmaterialidchannelformaterialoverride (stale _returnvalue_18)) :NewEnumerator1 (.mainmaterialidchannelformaterialoverride (stale _returnvalue_19)) :NewEnumerator2 (.mainmaterialidchannelformaterialoverride (stale _returnvalue_20)))) 0) (Variables|Default|GetNew%20Main%20Material)))
          (:Is%20Not%20Valid
            (Rendering|SetCastShadow (Variables|Default|GetSM_Wall_Lamp) (select _custom_override_settings_ (.shouldbasecastashadowwhenlightisturnedon? _returnvalue_5) (Utilities|Select :Index _lighting_catagory :NewEnumerator0 (.shouldbasecastashadowwhenlightisturnedon? (stale _returnvalue_18)) :NewEnumerator1 (.shouldbasecastashadowwhenlightisturnedon? (stale _returnvalue_19)) :NewEnumerator2 (.shouldbasecastashadowwhenlightisturnedon? (stale _returnvalue_20)))))))
        (Rendering|Material|SetMaterial (Variables|Default|GetSM_Wall_Lamp) (select (Utilities|IsValid (select _custom_override_settings_ (.staticmesh-glass _returnvalue_5) (Utilities|Select :Index _lighting_catagory :NewEnumerator0 (.staticmesh-glass (stale _returnvalue_18)) :NewEnumerator1 (.staticmesh-glass (stale _returnvalue_19)) :NewEnumerator2 (.staticmesh-glass (stale _returnvalue_20))))) 0 (select _custom_override_settings_ (.mainmaterialidchannelformaterialoverride _returnvalue_5) (Utilities|Select :Index _lighting_catagory :NewEnumerator0 (.mainmaterialidchannelformaterialoverride (stale _returnvalue_18)) :NewEnumerator1 (.mainmaterialidchannelformaterialoverride (stale _returnvalue_19)) :NewEnumerator2 (.mainmaterialidchannelformaterialoverride (stale _returnvalue_20))))) (Variables|Default|GetNew%20Main%20Material))
        (if (Variables|Default|GetTurn%20on%20lights?)
          (bind _returnvalue_7 (Rendering|Material|CreateDynamicMaterialInstance (select (Utilities|IsValid (Variables|Default|GetLamp%20Glass%20Asset%20Reference)) (Variables|Default|GetLamp%20Glass%20Asset%20Reference) (Variables|Default|GetSM_Wall_Lamp)) (select _custom_override_settings_ (.lightmaterialidchannelformaterialoverride _returnvalue_5) (Utilities|Select :Index _lighting_catagory :NewEnumerator0 (.lightmaterialidchannelformaterialoverride (stale _returnvalue_18)) :NewEnumerator1 (.lightmaterialidchannelformaterialoverride (stale _returnvalue_19)) :NewEnumerator2 (.lightmaterialidchannelformaterialoverride (stale _returnvalue_20)))) (select (Utilities|IsValid (select _custom_override_settings_ (.lightmaterialoverrideforwhenitsturnedonotherwisedefaultisused _returnvalue_5) (Utilities|Select :Index _lighting_catagory :NewEnumerator0 (.lightmaterialoverrideforwhenitsturnedonotherwisedefaultisused (stale _returnvalue_18)) :NewEnumerator1 (.lightmaterialoverrideforwhenitsturnedonotherwisedefaultisused (stale _returnvalue_19)) :NewEnumerator2 (.lightmaterialoverrideforwhenitsturnedonotherwisedefaultisused (stale _returnvalue_20))))) (select _custom_override_settings_ (.lightmaterialoverrideforwhenitsturnedonotherwisedefaultisused _returnvalue_5) (Utilities|Select :Index _lighting_catagory :NewEnumerator0 (.lightmaterialoverrideforwhenitsturnedonotherwisedefaultisused (stale _returnvalue_18)) :NewEnumerator1 (.lightmaterialoverrideforwhenitsturnedonotherwisedefaultisused (stale _returnvalue_19)) :NewEnumerator2 (.lightmaterialoverrideforwhenitsturnedonotherwisedefaultisused (stale _returnvalue_20)))) (select (select _custom_override_settings_ (.shouldglassmaterialbeopaque? _returnvalue_5) (Utilities|Select :Index _lighting_catagory :NewEnumerator0 (.shouldglassmaterialbeopaque? (stale _returnvalue_18)) :NewEnumerator1 (.shouldglassmaterialbeopaque? (stale _returnvalue_19)) :NewEnumerator2 (.shouldglassmaterialbeopaque? (stale _returnvalue_20)))) "/Game/InteriorBuildingKit/Material/Lighting/Defaults/MI_LightGlow_1500_Opaque.MI_LightGlow_1500_Opaque" "/Game/InteriorBuildingKit/Material/Lighting/Defaults/MI_LightGlow_500.MI_LightGlow_500")) "None" :!class /Script/Engine.PrimitiveComponent))
          (Rendering|Material|SetVectorParameterValue _returnvalue_7 "Emissive Colour" (* (Math|Curves|GetLinearColorValue (Variables|Variable|GetLight%20Temperature%20Reference) (/ (Variables|Default|GetLight%20Temperature) 6.5e+03)) (/ (Variables|Default|GetLight%20Intensity) 1e+02)) :!class /Script/Engine.MaterialInstanceDynamic)
          (Rendering|Material|SetMaterial (select (Utilities|IsValid (Variables|Default|GetLamp%20Glass%20Asset%20Reference)) (Variables|Default|GetLamp%20Glass%20Asset%20Reference) (Variables|Default|GetSM_Wall_Lamp)) (select _custom_override_settings_ (.lightmaterialidchannelformaterialoverride _returnvalue_5) (Utilities|Select :Index _lighting_catagory :NewEnumerator0 (.lightmaterialidchannelformaterialoverride (stale _returnvalue_18)) :NewEnumerator1 (.lightmaterialidchannelformaterialoverride (stale _returnvalue_19)) :NewEnumerator2 (.lightmaterialidchannelformaterialoverride (stale _returnvalue_20)))) _returnvalue_7))
        (Utilities|IsValid (select _custom_override_settings_ (.lightbulbmesh _returnvalue_5) (Utilities|Select :Index _lighting_catagory :NewEnumerator0 (.lightbulbmesh (stale _returnvalue_18)) :NewEnumerator1 (.lightbulbmesh (stale _returnvalue_19)) :NewEnumerator2 (.lightbulbmesh (stale _returnvalue_20))))
          (:Is%20Valid
            (for _array_element (select _custom_override_settings_ (.lightbulblocation _returnvalue_5) (Utilities|Select :Index _lighting_catagory :NewEnumerator0 (.lightbulblocation (stale _returnvalue_18)) :NewEnumerator1 (.lightbulblocation (stale _returnvalue_19)) :NewEnumerator2 (.lightbulblocation (stale _returnvalue_20))))
              (if (Variables|Default|GetTurn%20on%20lights?)
                (bind _returnvalue_8 (AddComponent|AddStaticMeshComponent false _array_element)) ; No Shadow
                (else
                  (bind _returnvalue_9 (AddComponent|AddStaticMeshComponent false _array_element)) ; Cast Shadow
                ))
              (Components|StaticMesh|SetStaticMesh (select (Variables|Default|GetTurn%20on%20lights?) _returnvalue_8 _returnvalue_9) (select _custom_override_settings_ (.lightbulbmesh _returnvalue_5) (Utilities|Select :Index _lighting_catagory :NewEnumerator0 (.lightbulbmesh (stale _returnvalue_18)) :NewEnumerator1 (.lightbulbmesh (stale _returnvalue_19)) :NewEnumerator2 (.lightbulbmesh (stale _returnvalue_20)))))
              (Transformation|AttachComponentToComponent (select (Variables|Default|GetTurn%20on%20lights?) _returnvalue_8 _returnvalue_9) (Variables|Default|GetLight%20Group%20-%20Lightbulbs) "None" "KeepRelative" "KeepRelative" "KeepRelative" true)
              (if (Variables|Default|GetTurn%20on%20lights?)
                (Rendering|Material|SetMaterial (select (Variables|Default|GetTurn%20on%20lights?) _returnvalue_8 _returnvalue_9) (select _custom_override_settings_ (.filamentidchannel _returnvalue_5) (Utilities|Select :Index _lighting_catagory :NewEnumerator0 (.filamentidchannel (stale _returnvalue_18)) :NewEnumerator1 (.filamentidchannel (stale _returnvalue_19)) :NewEnumerator2 (.filamentidchannel (stale _returnvalue_20)))) (Utilities|Select :Index (Math|Integer|Clamp(Integer) (+ (Math|Conversions|ToInteger(Boolean) (> _light_temperature 1e+03)) (Math|Conversions|ToInteger(Boolean) (> _light_temperature 2e+03)) (Math|Conversions|ToInteger(Boolean) (> _light_temperature 3e+03)) (Math|Conversions|ToInteger(Boolean) (> _light_temperature 4e+03)) (Math|Conversions|ToInteger(Boolean) (> _light_temperature 5e+03)) (Math|Conversions|ToInteger(Boolean) (> _light_temperature 6e+03)) (Math|Conversions|ToInteger(Boolean) (> _light_temperature 7e+03))) 0 6) :Option%200 "/Game/InteriorBuildingKit/Material/Lighting/Defaults/MI_LightGlow_500_Opaque.MI_LightGlow_500_Opaque" :Option%201 "/Game/InteriorBuildingKit/Material/Lighting/Defaults/MI_LightGlow_1500_Opaque.MI_LightGlow_1500_Opaque" :Option%202 "/Game/InteriorBuildingKit/Material/Lighting/Defaults/MI_LightGlow_2500_Opaque.MI_LightGlow_2500_Opaque" :Option%203 "/Game/InteriorBuildingKit/Material/Lighting/Defaults/MI_LightGlow_3500_Opaque.MI_LightGlow_3500_Opaque" :Option%204 "/Game/InteriorBuildingKit/Material/Lighting/Defaults/MI_LightGlow_4500_Opaque.MI_LightGlow_4500_Opaque" :Option%205 "/Game/InteriorBuildingKit/Material/Lighting/Defaults/MI_LightGlow_5500_Opaque.MI_LightGlow_5500_Opaque" :Option%206 "/Game/InteriorBuildingKit/Material/Lighting/Defaults/MI_LightGlow_6500_Opaque.MI_LightGlow_6500_Opaque" :Option%207 "/Game/InteriorBuildingKit/Material/Lighting/Defaults/MI_LightGlow_6500_Opaque.MI_LightGlow_6500_Opaque")))))
          (:Is%20Not%20Valid
            _))
        (if (Variables|Default|GetTurn%20on%20lights?)
          (Utilities|FlowControl|Sequence
            (:then_0
              (Utilities|FlowControl|Sequence
                (:then_0
                  ;[1 1 1] Light Creation - Up
                  (if (Utilities|Enum|Equal(Enum) (select _custom_override_settings_ (.lighttype-up _returnvalue_5) (Utilities|Select :Index _lighting_catagory :NewEnumerator0 (.lighttype-up (stale _returnvalue_18)) :NewEnumerator1 (.lighttype-up (stale _returnvalue_19)) :NewEnumerator2 (.lighttype-up (stale _returnvalue_20)))) "NewEnumerator0")
                    (for _array_element_2 (select _custom_override_settings_ (.lighttransform-up _returnvalue_5) (Utilities|Select :Index _lighting_catagory :NewEnumerator0 (.lighttransform-up (stale _returnvalue_18)) :NewEnumerator1 (.lighttransform-up (stale _returnvalue_19)) :NewEnumerator2 (.lighttransform-up (stale _returnvalue_20))))
                      (if _cast_dynamic_shadows____up_right_forward_2
                        (bind _returnvalue_10 (AddComponent|AddPointLightComponent false _array_element_2)) ; Static/Dynamic
                        (else
                          (bind _returnvalue_11 (AddComponent|AddPointLightComponent false _array_element_2)) ; Static
                        ))
                      (Transformation|AttachComponentToComponent (select _cast_dynamic_shadows____up_right_forward_2 _returnvalue_10 _returnvalue_11) _light_group___up "None" "KeepRelative" "KeepRelative" "KeepRelative" true)
                      (Class|LightComponent|SetUseIESBrightness (select _cast_dynamic_shadows____up_right_forward_2 _returnvalue_10 _returnvalue_11) _use_ies_intensity_)
                      (Transformation|SetMobility (select _cast_dynamic_shadows____up_right_forward_2 _returnvalue_10 _returnvalue_11) _light_mobility_mode___up)
                      (Rendering|Components|Light|SetCastShadows (select _cast_dynamic_shadows____up_right_forward_2 _returnvalue_10 _returnvalue_11) _cast_shadows____up_right_forward)
                      (Rendering|Components|Light|SetIntensity (select _cast_dynamic_shadows____up_right_forward_2 _returnvalue_10 _returnvalue_11) (* (select _custom_override_settings_ (.defaultlightintensity-up _returnvalue_5) (Utilities|Select :Index _lighting_catagory :NewEnumerator0 (.defaultlightintensity-up (stale _returnvalue_18)) :NewEnumerator1 (.defaultlightintensity-up (stale _returnvalue_19)) :NewEnumerator2 (.defaultlightintensity-up (stale _returnvalue_20)))) _returnvalue_4))
                      (if _use_ies_intensity__6
                        (Rendering|Components|Light|SetLightColor (select _cast_dynamic_shadows____up_right_forward_2 _returnvalue_10 _returnvalue_11) (* (Variables|Default|GetLight%20Colour) (Math|Conversions|ToLinearColor(Float) (/ (* (select _custom_override_settings_ (.defaultlightintensity-up _returnvalue_5) (Utilities|Select :Index _lighting_catagory :NewEnumerator0 (.defaultlightintensity-up (stale _returnvalue_18)) :NewEnumerator1 (.defaultlightintensity-up (stale _returnvalue_19)) :NewEnumerator2 (.defaultlightintensity-up (stale _returnvalue_20)))) _returnvalue_4) 1e+02))) true)
                        (Class|LightComponent|SetTemperature (select _cast_dynamic_shadows____up_right_forward_2 _returnvalue_10 _returnvalue_11) _light_temperature_3)
                        (Class|LightComponent|SetIESTexture (select _cast_dynamic_shadows____up_right_forward_2 _returnvalue_10 _returnvalue_11) (select (Utilities|IsValid _custom_ies_texture) _custom_ies_texture (select _custom_override_settings_ (.texturelightprofile-up _returnvalue_5) (Utilities|Select :Index _lighting_catagory :NewEnumerator0 (.texturelightprofile-up (stale _returnvalue_18)) :NewEnumerator1 (.texturelightprofile-up (stale _returnvalue_19)) :NewEnumerator2 (.texturelightprofile-up (stale _returnvalue_20))))))
                        (else
                          (Rendering|Components|Light|SetLightColor (select _cast_dynamic_shadows____up_right_forward_2 _returnvalue_10 _returnvalue_11) _light_colour_2 true)))
                      (Class|PointLightComponent|SetSourceRadius (select _cast_dynamic_shadows____up_right_forward_2 _returnvalue_10 _returnvalue_11) (select _custom_override_settings_ (.lightsourceradius-up _returnvalue_5) (Utilities|Select :Index _lighting_catagory :NewEnumerator0 (.lightsourceradius-up (stale _returnvalue_18)) :NewEnumerator1 (.lightsourceradius-up (stale _returnvalue_19)) :NewEnumerator2 (.lightsourceradius-up (stale _returnvalue_20)))))
                      (Rendering|Lighting|SetAttenuationRadius (select _cast_dynamic_shadows____up_right_forward_2 _returnvalue_10 _returnvalue_11) _attenuation_radius___up)
                      (Class|LightComponent|SetIndirectLightingIntensity (select _cast_dynamic_shadows____up_right_forward_2 _returnvalue_10 _returnvalue_11) _light_indirect_intensity_2)
                      (Class|LightComponentBase|SetCastRaytracedShadow (select _cast_dynamic_shadows____up_right_forward_2 _returnvalue_10 _returnvalue_11) _cast_ray_trace_shadows_))))
                (:then_1
                  (if (Utilities|Enum|Equal(Enum) (select _custom_override_settings_ (.lighttype-up _returnvalue_5) (Utilities|Select :Index _lighting_catagory :NewEnumerator0 (.lighttype-up (stale _returnvalue_18)) :NewEnumerator1 (.lighttype-up (stale _returnvalue_19)) :NewEnumerator2 (.lighttype-up (stale _returnvalue_20)))) "NewEnumerator1")
                    (for _array_element_3 (select _custom_override_settings_ (.lighttransform-up _returnvalue_5) (Utilities|Select :Index _lighting_catagory :NewEnumerator0 (.lighttransform-up (stale _returnvalue_18)) :NewEnumerator1 (.lighttransform-up (stale _returnvalue_19)) :NewEnumerator2 (.lighttransform-up (stale _returnvalue_20))))
                      (if _cast_dynamic_shadows____up_right_forward
                        (bind _returnvalue_12 (AddComponent|AddSpotLightComponent false _array_element_3)) ; Static/Dynamic
                        (else
                          (bind _returnvalue_13 (AddComponent|AddSpotLightComponent false _array_element_3)) ; Static
                        ))
                      (Transformation|AttachComponentToComponent (select _cast_dynamic_shadows____up_right_forward _returnvalue_12 _returnvalue_13) _light_group___up "None" "KeepRelative" "KeepRelative" "KeepRelative" true)
                      (Class|LightComponent|SetUseIESBrightness (select _cast_dynamic_shadows____up_right_forward _returnvalue_12 _returnvalue_13) _use_ies_intensity_)
                      (Transformation|SetMobility (select _cast_dynamic_shadows____up_right_forward _returnvalue_12 _returnvalue_13) _light_mobility_mode___up)
                      (Rendering|Components|Light|SetCastShadows (select _cast_dynamic_shadows____up_right_forward _returnvalue_12 _returnvalue_13) _cast_shadows____up_right_forward)
                      (Rendering|Components|Light|SetIntensity (select _cast_dynamic_shadows____up_right_forward _returnvalue_12 _returnvalue_13) (* (select _custom_override_settings_ (.defaultlightintensity-up _returnvalue_5) (Utilities|Select :Index _lighting_catagory :NewEnumerator0 (.defaultlightintensity-up (stale _returnvalue_18)) :NewEnumerator1 (.defaultlightintensity-up (stale _returnvalue_19)) :NewEnumerator2 (.defaultlightintensity-up (stale _returnvalue_20)))) _returnvalue_4))
                      (if _use_ies_intensity__6
                        (Rendering|Components|Light|SetLightColor (select _cast_dynamic_shadows____up_right_forward _returnvalue_12 _returnvalue_13) (* (Variables|Default|GetLight%20Colour) (Math|Conversions|ToLinearColor(Float) (/ (* (select _custom_override_settings_ (.defaultlightintensity-up _returnvalue_5) (Utilities|Select :Index _lighting_catagory :NewEnumerator0 (.defaultlightintensity-up (stale _returnvalue_18)) :NewEnumerator1 (.defaultlightintensity-up (stale _returnvalue_19)) :NewEnumerator2 (.defaultlightintensity-up (stale _returnvalue_20)))) _returnvalue_4) 1e+02))) true)
                        (Class|LightComponent|SetTemperature (select _cast_dynamic_shadows____up_right_forward _returnvalue_12 _returnvalue_13) _light_temperature_3)
                        (Class|LightComponent|SetIESTexture (select _cast_dynamic_shadows____up_right_forward _returnvalue_12 _returnvalue_13) (select (Utilities|IsValid _custom_ies_texture) _custom_ies_texture (select _custom_override_settings_ (.texturelightprofile-up _returnvalue_5) (Utilities|Select :Index _lighting_catagory :NewEnumerator0 (.texturelightprofile-up (stale _returnvalue_18)) :NewEnumerator1 (.texturelightprofile-up (stale _returnvalue_19)) :NewEnumerator2 (.texturelightprofile-up (stale _returnvalue_20))))))
                        (else
                          (Rendering|Components|Light|SetLightColor (select _cast_dynamic_shadows____up_right_forward _returnvalue_12 _returnvalue_13) _light_colour_2 true)))
                      (Class|PointLightComponent|SetSourceRadius (select _cast_dynamic_shadows____up_right_forward _returnvalue_12 _returnvalue_13) (select _custom_override_settings_ (.lightsourceradius-up _returnvalue_5) (Utilities|Select :Index _lighting_catagory :NewEnumerator0 (.lightsourceradius-up (stale _returnvalue_18)) :NewEnumerator1 (.lightsourceradius-up (stale _returnvalue_19)) :NewEnumerator2 (.lightsourceradius-up (stale _returnvalue_20)))))
                      (Rendering|Lighting|SetAttenuationRadius (select _cast_dynamic_shadows____up_right_forward _returnvalue_12 _returnvalue_13) _attenuation_radius___up)
                      (Rendering|Lighting|SetOuterConeAngle (select _cast_dynamic_shadows____up_right_forward _returnvalue_12 _returnvalue_13) (Variables|Default|GetOuter%20Cone%20Angle%20-%20Up))
                      (Class|LightComponent|SetIndirectLightingIntensity (select _cast_dynamic_shadows____up_right_forward _returnvalue_12 _returnvalue_13) _light_indirect_intensity_2)
                      (Class|LightComponentBase|SetCastRaytracedShadow (select _cast_dynamic_shadows____up_right_forward _returnvalue_12 _returnvalue_13) _cast_ray_trace_shadows_))))))
            (:then_1
              (Utilities|FlowControl|Sequence
                (:then_0
                  ;[1 1 1] Light Creation - Down
                  (if (Utilities|Enum|Equal(Enum) (select _custom_override_settings_ (.lighttype-down _returnvalue_5) (Utilities|Select :Index _lighting_catagory :NewEnumerator0 (.lighttype-down (stale _returnvalue_18)) :NewEnumerator1 (.lighttype-down (stale _returnvalue_19)) :NewEnumerator2 (.lighttype-down (stale _returnvalue_20)))) "NewEnumerator0")
                    (for _array_element_4 (select _custom_override_settings_ (.lighttransform-down _returnvalue_5) (Utilities|Select :Index _lighting_catagory :NewEnumerator0 (.lighttransform-down (stale _returnvalue_18)) :NewEnumerator1 (.lighttransform-down (stale _returnvalue_19)) :NewEnumerator2 (.lighttransform-down (stale _returnvalue_20))))
                      (if _cast_dynamic_shadows____down_left_back_2
                        (bind _returnvalue_14 (AddComponent|AddPointLightComponent false _array_element_4)) ; Static/Dynamic
                        (else
                          (bind _returnvalue_15 (AddComponent|AddPointLightComponent false _array_element_4)) ; Static
                        ))
                      (Transformation|AttachComponentToComponent (select _cast_dynamic_shadows____down_left_back_2 _returnvalue_14 _returnvalue_15) _light_group___down "None" "KeepRelative" "KeepRelative" "KeepRelative" true)
                      (Class|LightComponent|SetUseIESBrightness (select _cast_dynamic_shadows____down_left_back_2 _returnvalue_14 _returnvalue_15) _use_ies_intensity__2)
                      (Transformation|SetMobility (select _cast_dynamic_shadows____down_left_back_2 _returnvalue_14 _returnvalue_15) _light_mobility_mode___down)
                      (Rendering|Components|Light|SetCastShadows (select _cast_dynamic_shadows____down_left_back_2 _returnvalue_14 _returnvalue_15) _cast_shadows____down_left_back)
                      (Rendering|Components|Light|SetIntensity (select _cast_dynamic_shadows____down_left_back_2 _returnvalue_14 _returnvalue_15) (* (select _custom_override_settings_ (.defaultlightintensity-down _returnvalue_5) (Utilities|Select :Index _lighting_catagory :NewEnumerator0 (.defaultlightintensity-down (stale _returnvalue_18)) :NewEnumerator1 (.defaultlightintensity-down (stale _returnvalue_19)) :NewEnumerator2 (.defaultlightintensity-down (stale _returnvalue_20)))) _returnvalue_3))
                      (if _use_ies_intensity__4
                        (Rendering|Components|Light|SetLightColor (select _cast_dynamic_shadows____down_left_back_2 _returnvalue_14 _returnvalue_15) (* (Variables|Default|GetLight%20Colour) (Math|Conversions|ToLinearColor(Float) (/ (* (select _custom_override_settings_ (.defaultlightintensity-down _returnvalue_5) (Utilities|Select :Index _lighting_catagory :NewEnumerator0 (.defaultlightintensity-down (stale _returnvalue_18)) :NewEnumerator1 (.defaultlightintensity-down (stale _returnvalue_19)) :NewEnumerator2 (.defaultlightintensity-down (stale _returnvalue_20)))) _returnvalue_3) 1e+02))) true)
                        (Class|LightComponent|SetTemperature (select _cast_dynamic_shadows____down_left_back_2 _returnvalue_14 _returnvalue_15) _light_temperature_2)
                        (Class|LightComponent|SetIESTexture (select _cast_dynamic_shadows____down_left_back_2 _returnvalue_14 _returnvalue_15) (select (Utilities|IsValid _custom_ies_texture_2) _custom_ies_texture_2 (select _custom_override_settings_ (.texturelightprofile-down _returnvalue_5) (Utilities|Select :Index _lighting_catagory :NewEnumerator0 (.texturelightprofile-down (stale _returnvalue_18)) :NewEnumerator1 (.texturelightprofile-down (stale _returnvalue_19)) :NewEnumerator2 (.texturelightprofile-down (stale _returnvalue_20))))))
                        (else
                          (Rendering|Components|Light|SetLightColor (select _cast_dynamic_shadows____down_left_back_2 _returnvalue_14 _returnvalue_15) _light_colour true)))
                      (Class|PointLightComponent|SetSourceRadius (select _cast_dynamic_shadows____down_left_back_2 _returnvalue_14 _returnvalue_15) (select _custom_override_settings_ (.lightsourceradius-down _returnvalue_5) (Utilities|Select :Index _lighting_catagory :NewEnumerator0 (.lightsourceradius-down (stale _returnvalue_18)) :NewEnumerator1 (.lightsourceradius-down (stale _returnvalue_19)) :NewEnumerator2 (.lightsourceradius-down (stale _returnvalue_20)))))
                      (Rendering|Lighting|SetAttenuationRadius (select _cast_dynamic_shadows____down_left_back_2 _returnvalue_14 _returnvalue_15) _attenuation_radius___down)
                      (Class|LightComponent|SetIndirectLightingIntensity (select _cast_dynamic_shadows____down_left_back_2 _returnvalue_14 _returnvalue_15) _light_indirect_intensity)
                      (Class|LightComponentBase|SetCastRaytracedShadow (select _cast_dynamic_shadows____down_left_back_2 _returnvalue_14 _returnvalue_15) _cast_ray_trace_shadows__2))))
                (:then_1
                  (if (Utilities|Enum|Equal(Enum) (select _custom_override_settings_ (.lighttype-down _returnvalue_5) (Utilities|Select :Index _lighting_catagory :NewEnumerator0 (.lighttype-down (stale _returnvalue_18)) :NewEnumerator1 (.lighttype-down (stale _returnvalue_19)) :NewEnumerator2 (.lighttype-down (stale _returnvalue_20)))) "NewEnumerator1")
                    (for _array_element_5 (select _custom_override_settings_ (.lighttransform-down _returnvalue_5) (Utilities|Select :Index _lighting_catagory :NewEnumerator0 (.lighttransform-down (stale _returnvalue_18)) :NewEnumerator1 (.lighttransform-down (stale _returnvalue_19)) :NewEnumerator2 (.lighttransform-down (stale _returnvalue_20))))
                      (if _cast_dynamic_shadows____down_left_back
                        (bind _returnvalue_16 (AddComponent|AddSpotLightComponent false _array_element_5)) ; Static/Dynamic
                        (else
                          (bind _returnvalue_17 (AddComponent|AddSpotLightComponent false _array_element_5)) ; Static
                        ))
                      (Transformation|AttachComponentToComponent (select _cast_dynamic_shadows____down_left_back _returnvalue_16 _returnvalue_17) _light_group___down "None" "KeepRelative" "KeepRelative" "KeepRelative" true)
                      (Class|LightComponent|SetUseIESBrightness (select _cast_dynamic_shadows____down_left_back _returnvalue_16 _returnvalue_17) _use_ies_intensity__2)
                      (Transformation|SetMobility (select _cast_dynamic_shadows____down_left_back _returnvalue_16 _returnvalue_17) _light_mobility_mode___down)
                      (Rendering|Components|Light|SetCastShadows (select _cast_dynamic_shadows____down_left_back _returnvalue_16 _returnvalue_17) _cast_shadows____down_left_back)
                      (Rendering|Components|Light|SetIntensity (select _cast_dynamic_shadows____down_left_back _returnvalue_16 _returnvalue_17) (* (select _custom_override_settings_ (.defaultlightintensity-down _returnvalue_5) (Utilities|Select :Index _lighting_catagory :NewEnumerator0 (.defaultlightintensity-down (stale _returnvalue_18)) :NewEnumerator1 (.defaultlightintensity-down (stale _returnvalue_19)) :NewEnumerator2 (.defaultlightintensity-down (stale _returnvalue_20)))) _returnvalue_3))
                      (if _use_ies_intensity__4
                        (Rendering|Components|Light|SetLightColor (select _cast_dynamic_shadows____down_left_back _returnvalue_16 _returnvalue_17) (* (Variables|Default|GetLight%20Colour) (Math|Conversions|ToLinearColor(Float) (/ (* (select _custom_override_settings_ (.defaultlightintensity-down _returnvalue_5) (Utilities|Select :Index _lighting_catagory :NewEnumerator0 (.defaultlightintensity-down (stale _returnvalue_18)) :NewEnumerator1 (.defaultlightintensity-down (stale _returnvalue_19)) :NewEnumerator2 (.defaultlightintensity-down (stale _returnvalue_20)))) _returnvalue_3) 1e+02))) true)
                        (Class|LightComponent|SetTemperature (select _cast_dynamic_shadows____down_left_back _returnvalue_16 _returnvalue_17) _light_temperature_2)
                        (Class|LightComponent|SetIESTexture (select _cast_dynamic_shadows____down_left_back _returnvalue_16 _returnvalue_17) (select (Utilities|IsValid _custom_ies_texture_2) _custom_ies_texture_2 (select _custom_override_settings_ (.texturelightprofile-down _returnvalue_5) (Utilities|Select :Index _lighting_catagory :NewEnumerator0 (.texturelightprofile-down (stale _returnvalue_18)) :NewEnumerator1 (.texturelightprofile-down (stale _returnvalue_19)) :NewEnumerator2 (.texturelightprofile-down (stale _returnvalue_20))))))
                        (else
                          (Rendering|Components|Light|SetLightColor (select _cast_dynamic_shadows____down_left_back _returnvalue_16 _returnvalue_17) _light_colour true)))
                      (Class|PointLightComponent|SetSourceRadius (select _cast_dynamic_shadows____down_left_back _returnvalue_16 _returnvalue_17) (select _custom_override_settings_ (.lightsourceradius-down _returnvalue_5) (Utilities|Select :Index _lighting_catagory :NewEnumerator0 (.lightsourceradius-down (stale _returnvalue_18)) :NewEnumerator1 (.lightsourceradius-down (stale _returnvalue_19)) :NewEnumerator2 (.lightsourceradius-down (stale _returnvalue_20)))))
                      (Rendering|Lighting|SetAttenuationRadius (select _cast_dynamic_shadows____down_left_back _returnvalue_16 _returnvalue_17) _attenuation_radius___down)
                      (Rendering|Lighting|SetOuterConeAngle (select _cast_dynamic_shadows____down_left_back _returnvalue_16 _returnvalue_17) (Variables|Default|GetOuter%20Cone%20Angle%20-%20Down))
                      (Class|LightComponent|SetIndirectLightingIntensity (select _cast_dynamic_shadows____down_left_back _returnvalue_16 _returnvalue_17) _light_indirect_intensity)
                      (Class|LightComponentBase|SetCastRaytracedShadow (select _cast_dynamic_shadows____down_left_back _returnvalue_16 _returnvalue_17) _cast_ray_trace_shadows__2)))))))))
      (:RowNotFound
        (Variables|Default|SetLight%20Option (- (Utilities|Array|Length _outrownames) 1))
        (goto _label)))
    (else
      (Utilities|FlowControl|Sequence
        (:then_0
          (if (Utilities|Enum|Equal(Enum) (Variables|Default|GetLighting%20catagory) "NewEnumerator0")
            (bind _outrownames_2 (DataTable|GetDataTableRowNames "/Game/InteriorBuildingKit/Struct/LightTypes_Walls_DataTable.LightTypes_Walls_DataTable"))
            (bind _returnvalue_18 (Utilities|GetDataTableRow "/Game/InteriorBuildingKit/Struct/LightTypes_Walls_DataTable.LightTypes_Walls_DataTable" (Utilities|Array|Get(acopy) _outrownames_2 (Variables|Default|GetLight%20Option)) :!label _label_3)
              (:then
                (goto _label_2))
              (:RowNotFound
                (Variables|Default|SetLight%20Option (- (Utilities|Array|Length _outrownames_2) 1))
                (goto _label_3)))))
        (:then_1
          (if (Utilities|Enum|Equal(Enum) (Variables|Default|GetLighting%20catagory) "NewEnumerator1")
            (bind _outrownames_3 (DataTable|GetDataTableRowNames "/Game/InteriorBuildingKit/Struct/LightTypes_Ceiling_DataTable.LightTypes_Ceiling_DataTable"))
            (bind _returnvalue_19 (Utilities|GetDataTableRow "/Game/InteriorBuildingKit/Struct/LightTypes_Ceiling_DataTable.LightTypes_Ceiling_DataTable" (Utilities|Array|Get(acopy) _outrownames_3 (Variables|Default|GetLight%20Option)) :!label _label_4)
              (:then
                (goto _label_2))
              (:RowNotFound
                (Variables|Default|SetLight%20Option (- (Utilities|Array|Length _outrownames_3) 1))
                (goto _label_4)))))
        (:then_2
          (if (Utilities|Enum|Equal(Enum) (Variables|Default|GetLighting%20catagory) "NewEnumerator2")
            (bind _outrownames_4 (DataTable|GetDataTableRowNames "/Game/InteriorBuildingKit/Struct/LightTypes_Chandelier_DataTable.LightTypes_Chandelier_DataTable"))
            (bind _returnvalue_20 (Utilities|GetDataTableRow "/Game/InteriorBuildingKit/Struct/LightTypes_Chandelier_DataTable.LightTypes_Chandelier_DataTable" (Utilities|Array|Get(acopy) _outrownames_4 (Variables|Default|GetLight%20Option)) :!label _label_5)
              (:then
                (goto _label_2))
              (:RowNotFound
                (Variables|Default|SetLight%20Option (- (Utilities|Array|Length _outrownames_4) 1))
                (goto _label_5)))))))))