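; Configurable corner kitchen cabinet for building interiors, assembled entirely in the Construction Script with no runtime logic.
; Open-state values lerp the yaw of five doors across three cabinet sections.
; Clamped height arrays spawn shelf meshes in the first and third sections, with optional wood material overrides.
; A handle-type enum selects a data table row, and an upper-capped option index picks the mesh for all handles, which share one material.
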(event EventBeginPlay)

(event Collision|EventActorBeginOverlap
  (params (OtherActor :type Actor%20Object%20Reference)))

(event EventTick
  (params (DeltaSeconds :type Float%20%28single-precision%29)))

(fn ConstructionScript
  (bind _new_wood_material___flat_wood (Variables|Default|GetNew%20Wood%20Material%20-%20Flat%20Wood))
  (bind _new_wood_material___flat_wood_2 (Variables|Default|GetNew%20Wood%20Material%20-%20Flat%20Wood))
  (bind _new_wood_material___trim_wood (Variables|Default|GetNew%20Wood%20Material%20-%20Trim%20Wood))
  (bind _new_wood_material___flat_wood_3 (Variables|Default|GetNew%20Wood%20Material%20-%20Flat%20Wood))
  (Transformation|SetRelativeRotation (Variables|Default|GetSM_Kitchen_Door1%20Left) (Math|Rotator|MakeRotator 0.0 0.0 (Math|Float|Lerp 0.0 179.0 (Variables|Default|GetOpen%20State%20-%20Cabinet1%20Left%20Door))) false false)
  (Transformation|SetRelativeRotation (Variables|Default|GetSM_Kitchen_Door1%20Right) (Math|Rotator|MakeRotator 0.0 0.0 (Math|Float|Lerp 0.0 -125.0 (Variables|Default|GetOpen%20State%20-%20Cabinet1%20Right%20Door))) false false)
  (Transformation|SetRelativeRotation (Variables|Default|GetSM_Kitchen_Door2) (Math|Rotator|MakeRotator 0.0 0.0 (Math|Float|Lerp 45.0 179.0 (Variables|Default|GetOpen%20State%20-%20Cabinet2))) false false)
  (Transformation|SetRelativeRotation (Variables|Default|GetSM_Kitchen_Door3%20Left) (Math|Rotator|MakeRotator 0.0 0.0 (Math|Float|Lerp 9e+01 215.0 (Variables|Default|GetOpen%20State%20-%20Cabinet3%20Left%20Door))) false false)
  (Transformation|SetRelativeRotation (Variables|Default|GetSM_Kitchen_Door3%20Right) (Math|Rotator|MakeRotator 0.0 0.0 (Math|Float|Lerp 9e+01 -89.0 (Variables|Default|GetOpen%20State%20-%20Cabinet3%20Right%20Door))) false false)
  (for (_array_element _array_index) (Variables|Default|GetCabinet1%20Shelf%20Height)
    (Utilities|Array|SetArrayElem (Variables|Default|GetCabinet1%20Shelf%20Height) _array_index (Math|Float|Clamp(Float) _array_element 1e+01 75.0))
    (bind _returnvalue (AddComponent|AddStaticMeshComponent false (Math|Transform|MakeTransform (Math|Vector|MakeVector 0.0 0.0 (- (Math|Float|Clamp(Float) _array_element 1e+01 75.0) 8e+01)) "0, 0, 0" "1.000000,1.000000,1.000000")))
    (Utilities|IsValid _new_wood_material___flat_wood_3
      (:Is%20Valid
        (Rendering|Material|SetMaterial _returnvalue 0 _new_wood_material___flat_wood_3))))
  (for (_array_element_2 _array_index_2) (Variables|Default|GetCabinet3%20Shelf%20Height)
    (Utilities|Array|SetArrayElem (Variables|Default|GetCabinet3%20Shelf%20Height) _array_index_2 (Math|Float|Clamp(Float) _array_element_2 1e+01 75.0))
    (bind _returnvalue_2 (AddComponent|AddStaticMeshComponent false (Math|Transform|MakeTransform (Math|Vector|MakeVector 1.2e+02 1.2e+02 (- (Math|Float|Clamp(Float) _array_element_2 1e+01 75.0) 8e+01)) "0.000000,90.000000, 0" "1.000000,1.000000,1.000000")))
    (Utilities|IsValid _new_wood_material___flat_wood
      (:Is%20Valid
        (Rendering|Material|SetMaterial _returnvalue_2 0 _new_wood_material___flat_wood))))
  (Utilities|IsValid _new_wood_material___flat_wood_2
    (:Is%20Valid
      (Rendering|Material|SetMaterial (Variables|Default|GetSM_Kitchen_Door1%20Left) 0 _new_wood_material___flat_wood_2))
    (:Is%20Not%20Valid
      _))
  (Utilities|IsValid _new_wood_material___trim_wood
    (:Is%20Valid
      (Rendering|Material|SetMaterial (Variables|Default|GetSM_Kitchen_Counter_Base1) 1 _new_wood_material___trim_wood))
    (:Is%20Not%20Valid
      _))
  (bind _returnvalue_3 (Utilities|GetDataTableRow "/Game/InteriorBuildingKit/Struct/CounterHandleTypes_DataTable.CounterHandleTypes_DataTable" (Utilities|String|StringToName (Utilities|String|EnumtoString (Variables|Default|GetHandle%20Type))))
    (:then
      (if (>= (Variables|Default|GetHandle%20Option) (Utilities|Array|Length (.handletype _returnvalue_3)))
        (Variables|Default|SetHandle%20Option (- (Utilities|Array|Length (.handletype _returnvalue_3)) 1)))
      (Components|StaticMesh|SetStaticMesh (Variables|Default|GetSM_Handle_Door2) (Utilities|Array|Get(acopy) (.handletype _returnvalue_3) (Variables|Default|GetHandle%20Option)))
      (Components|StaticMesh|SetStaticMesh (Variables|Default|GetSM_Handle_Door1_Left) (Utilities|Array|Get(acopy) (.handletype _returnvalue_3) (Variables|Default|GetHandle%20Option)))
      (Components|StaticMesh|SetStaticMesh (Variables|Default|GetSM_Handle_Door1_Right) (Utilities|Array|Get(acopy) (.handletype _returnvalue_3) (Variables|Default|GetHandle%20Option)))
      (Components|StaticMesh|SetStaticMesh (Variables|Default|GetSM_Handle_Door3_Right) (Utilities|Array|Get(acopy) (.handletype _returnvalue_3) (Variables|Default|GetHandle%20Option)))
      (Components|StaticMesh|SetStaticMesh (Variables|Default|GetSM_Handle_Door3_Left) (Utilities|Array|Get(acopy) (.handletype _returnvalue_3) (Variables|Default|GetHandle%20Option)))
      (Rendering|Material|SetMaterial (Variables|Default|GetSM_Handle_Door3_Left) 0 (Variables|Default|GetNew%20Handle%20Material)))))