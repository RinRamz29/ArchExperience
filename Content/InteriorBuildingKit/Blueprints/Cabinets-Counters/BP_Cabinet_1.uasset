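; Configurable two-door kitchen cabinet from the interior building kit, built entirely in the construction script with no active runtime logic.
; Per-door open values set each door's yaw in opposite directions, and the clamped height array spawns shelf meshes.
; Optional wood materials override doors, base, shelves and trim.
; The handle type enum selects a data table row, whose mesh list supplies both handles via a capped option index.
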(event EventBeginPlay)

(event Collision|EventActorBeginOverlap
  (params (OtherActor :type Actor%20Object%20Reference)))

(event EventTick
  (params (DeltaSeconds :type Float%20%28single-precision%29)))

(fn ConstructionScript
  (bind _new_wood_material___flat_wood (Variables|Default|GetNew%20Wood%20Material%20-%20Flat%20Wood))
  (bind _new_wood_material___flat_wood_2 (Variables|Default|GetNew%20Wood%20Material%20-%20Flat%20Wood))
  (bind _new_wood_material___trim_wood (Variables|Default|GetNew%20Wood%20Material%20-%20Trim%20Wood))
  (Transformation|SetRelativeRotation (Variables|Default|GetSM_Kitchen_Door%20Left) (Math|Rotator|MakeRotator 0.0 0.0 (Math|Float|Lerp 0.0 179.0 (Variables|Default|GetOpen%20State%20-%20Left%20Door))) false false)
  (Transformation|SetRelativeRotation (Variables|Default|GetSM_Kitchen_Door%20Right) (Math|Rotator|MakeRotator 0.0 0.0 (Math|Float|Lerp 0.0 -179.0 (Variables|Default|GetOpen%20State%20-%20Right%20Door))) false false)
  (for (_array_element _array_index) (Variables|Default|GetShelf%20Height)
    (Utilities|Array|SetArrayElem (Variables|Default|GetShelf%20Height) _array_index (Math|Float|Clamp(Float) _array_element 1e+01 75.0))
    (bind _returnvalue (AddComponent|AddStaticMeshComponent false (Math|Transform|MakeTransform (Math|Vector|MakeVector 0.0 0.0 (- (Math|Float|Clamp(Float) _array_element 1e+01 75.0) 8e+01)) "0, 0, 0" "1.000000,1.000000,1.000000")))
    (Utilities|IsValid _new_wood_material___flat_wood
      (:Is%20Valid
        (Rendering|Material|SetMaterial _returnvalue 0 _new_wood_material___flat_wood))))
  (Utilities|IsValid _new_wood_material___flat_wood_2
    (:Is%20Valid
      (Rendering|Material|SetMaterial (Variables|Default|GetSM_Kitchen_Door%20Left) 0 _new_wood_material___flat_wood_2))
    (:Is%20Not%20Valid
      _))
  (Utilities|IsValid _new_wood_material___trim_wood
    (:Is%20Valid
      (Rendering|Material|SetMaterial (Variables|Default|GetSM_Kitchen_Counter_Base1) 1 _new_wood_material___trim_wood))
    (:Is%20Not%20Valid
      _))
  (bind _returnvalue_2 (Utilities|GetDataTableRow "/Game/InteriorBuildingKit/Struct/CounterHandleTypes_DataTable.CounterHandleTypes_DataTable" (Utilities|String|StringToName (Utilities|String|EnumtoString (Variables|Default|GetHandle%20Type))))
    (:then
      (if (>= (Variables|Default|GetHandle%20Option) (Utilities|Array|Length (.handletype _returnvalue_2)))
        (Variables|Default|SetHandle%20Option (- (Utilities|Array|Length (.handletype _returnvalue_2)) 1)))
      (Components|StaticMesh|SetStaticMesh (Variables|Default|GetSM_Handle_Left) (Utilities|Array|Get(acopy) (.handletype _returnvalue_2) (Variables|Default|GetHandle%20Option)))
      (Components|StaticMesh|SetStaticMesh (Variables|Default|GetSM_Handle_Right) (Utilities|Array|Get(acopy) (.handletype _returnvalue_2) (Variables|Default|GetHandle%20Option)))
      (Rendering|Material|SetMaterial (Variables|Default|GetSM_Handle_Left) 0 (Variables|Default|GetNew%20Handle%20Material)))))