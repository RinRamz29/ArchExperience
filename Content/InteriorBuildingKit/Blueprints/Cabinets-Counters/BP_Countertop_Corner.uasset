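; Configurable corner kitchen countertop prop with two cabinets, each having double doors, a drawer and adjustable shelves.
; The Construction Script lerps doors and drawers from per-part open values and spawns shelf meshes at clamped heights from two arrays.
; It applies optional countertop and wood material overrides.
; Handle meshes come from a data table row keyed by handle type, with the option index capped, and receive a handle material.
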(event EventBeginPlay)

(event Collision|EventActorBeginOverlap
  (params (OtherActor :type Actor%20Object%20Reference)))

(event EventTick
  (params (DeltaSeconds :type Float%20%28single-precision%29)))

(fn ConstructionScript
  (bind _new_wood_material___trim_wood (Variables|Default|GetNew%20Wood%20Material%20-%20Trim%20Wood))
  (bind _new_wood_material___flat_wood (Variables|Default|GetNew%20Wood%20Material%20-%20Flat%20Wood))
  (bind _new_wood_material___flat_wood_2 (Variables|Default|GetNew%20Wood%20Material%20-%20Flat%20Wood))
  (bind _new_countertop_material (Variables|Default|GetNew%20Countertop%20Material))
  (bind _new_wood_material___flat_wood_3 (Variables|Default|GetNew%20Wood%20Material%20-%20Flat%20Wood))
  (Utilities|IsValid _new_countertop_material
    (:Is%20Valid
      (Rendering|Material|SetMaterial (Variables|Default|GetSM_Kitchen_Countertop) 0 _new_countertop_material))
    (:Is%20Not%20Valid
      _))
  (Transformation|SetRelativeRotation (Variables|Default|GetSM_Kitchen_Door%20Left) (Math|Rotator|MakeRotator 0.0 0.0 (Math|Float|Lerp 0.0 179.0 (Variables|Default|GetOpen%20State%201%20-%20Left%20Door))) false false)
  (Transformation|SetRelativeRotation (Variables|Default|GetSM_Kitchen_Door%20Right) (Math|Rotator|MakeRotator 0.0 0.0 (Math|Float|Lerp 0.0 -179.0 (Variables|Default|GetOpen%20State%201%20-%20Right%20Door))) false false)
  (Transformation|SetRelativeLocation (Variables|Default|GetSM_Kitchen_Drawer) (Math|Vector|MakeVector 0.0 (Math|Float|Lerp 0.0 55.0 (Variables|Default|GetOpen%20State%201%20-%20Drawer)) 0.0) false false)
  (Transformation|SetRelativeRotation (Variables|Default|GetSM_Kitchen_Door2%20Left) (Math|Rotator|MakeRotator 0.0 0.0 (Math|Float|Lerp 0.0 179.0 (Variables|Default|GetOpen%20State%202%20-%20Left%20Door))) false false)
  (Transformation|SetRelativeRotation (Variables|Default|GetSM_Kitchen_Door2%20Right) (Math|Rotator|MakeRotator 0.0 0.0 (Math|Float|Lerp 0.0 -179.0 (Variables|Default|GetOpen%20State%202%20-%20Right%20Door))) false false)
  (Transformation|SetRelativeLocation (Variables|Default|GetSM_Kitchen_Drawer2) (Math|Vector|MakeVector 0.0 (Math|Float|Lerp 0.0 55.0 (Variables|Default|GetOpen%20State%202%20-%20Drawer)) 0.0) false false)
  (for (_array_element _array_index) (Variables|Default|GetCabinet%201%20-%20Shelf%20Height)
    (Utilities|Array|SetArrayElem (Variables|Default|GetCabinet%201%20-%20Shelf%20Height) _array_index (Math|Float|Clamp(Float) _array_element 1e+01 75.0))
    (bind _returnvalue (AddComponent|AddStaticMeshComponent false (Math|Transform|MakeTransform (Math|Vector|MakeVector 0.0 0.0 (Math|Float|Clamp(Float) _array_element 1e+01 75.0)) "0, 0, 0" "1.000000,1.000000,1.000000")))
    (Utilities|IsValid _new_wood_material___flat_wood_2
      (:Is%20Valid
        (Rendering|Material|SetMaterial _returnvalue 0 _new_wood_material___flat_wood_2))))
  (for (_array_element_2 _array_index_2) (Variables|Default|GetCabinet%202%20-%20Shelf%20Height)
    (Utilities|Array|SetArrayElem (Variables|Default|GetCabinet%202%20-%20Shelf%20Height) _array_index_2 (Math|Float|Clamp(Float) _array_element_2 1e+01 75.0))
    (bind _returnvalue_2 (AddComponent|AddStaticMeshComponent false (Math|Transform|MakeTransform (Math|Vector|MakeVector 85.0 85.0 (Math|Float|Clamp(Float) _array_element_2 1e+01 75.0)) "0,90.000000, 0" "1.000000,1.000000,1.000000")))
    (Utilities|IsValid _new_wood_material___flat_wood
      (:Is%20Valid
        (Rendering|Material|SetMaterial _returnvalue_2 0 _new_wood_material___flat_wood))))
  (Utilities|IsValid _new_wood_material___flat_wood_3
    (:Is%20Valid
      (Rendering|Material|SetMaterial (Variables|Default|GetSM_Kitchen_Drawer) 0 _new_wood_material___flat_wood_3))
    (:Is%20Not%20Valid
      _))
  (Utilities|IsValid _new_wood_material___trim_wood
    (:Is%20Valid
      (Rendering|Material|SetMaterial (Variables|Default|GetSM_Kitchen_Counter_Base1) 1 _new_wood_material___trim_wood))
    (:Is%20Not%20Valid
      _))
  (bind _returnvalue_3 (Utilities|GetDataTableRow "/Game/InteriorBuildingKit/Struct/CounterHandleTypes_DataTable.CounterHandleTypes_DataTable" (Utilities|String|StringToName (Utilities|String|EnumtoString (Variables|Default|GetHandle%20Type))))
    (:then
      (if (>= (Variables|Default|GetHandle%20Option) (Utilities|Array|Length (.handletype _returnvalue_3)))
        (Variables|Default|SetHandle%20Option (- (Utilities|Array|Length (.handletype _returnvalue_3)) 1)))
      (Components|StaticMesh|SetStaticMesh (Variables|Default|GetSM_Handle_Door%20Right) (Utilities|Array|Get(acopy) (.handletype _returnvalue_3) (Variables|Default|GetHandle%20Option)))
      (Components|StaticMesh|SetStaticMesh (Variables|Default|GetSM_Handle_Drawer) (Utilities|Array|Get(acopy) (.handletype _returnvalue_3) (Variables|Default|GetHandle%20Option)))
      (Components|StaticMesh|SetStaticMesh (Variables|Default|GetSM_Handle_Door%20Left) (Utilities|Array|Get(acopy) (.handletype _returnvalue_3) (Variables|Default|GetHandle%20Option)))
      (Components|StaticMesh|SetStaticMesh (Variables|Default|GetSM_Handle_Door2%20Right) (Utilities|Array|Get(acopy) (.handletype _returnvalue_3) (Variables|Default|GetHandle%20Option)))
      (Components|StaticMesh|SetStaticMesh (Variables|Default|GetSM_Handle_Drawer2) (Utilities|Array|Get(acopy) (.handletype _returnvalue_3) (Variables|Default|GetHandle%20Option)))
      (Components|StaticMesh|SetStaticMesh (Variables|Default|GetSM_Handle_Door2%20Left) (Utilities|Array|Get(acopy) (.handletype _returnvalue_3) (Variables|Default|GetHandle%20Option)))
      (Rendering|Material|SetMaterial (Variables|Default|GetSM_Handle_Door2%20Left) 0 (Variables|Default|GetNew%20Handle%20Material)))))