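; Configurable kitchen counter from an interior building kit, assembled entirely in the Construction Script from exposed options.
; With a sink, it adds data-table sink and drain meshes, swaps countertop and base, and replaces the drawer with a blank front.
; Otherwise it slides the drawer and spawns height-clamped shelves.
; Both variants pose doors by open-state values, apply material overrides and choose data-table handles, clamping out-of-range handle options.
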(event EventBeginPlay)

(event Collision|EventActorBeginOverlap
  (params (OtherActor :type Actor%20Object%20Reference)))

(event EventTick
  (params (DeltaSeconds :type Float%20%28single-precision%29)))

(fn ConstructionScript
  (bind _new_wood_material___flat_wood (Variables|Default|GetNew%20Wood%20Material%20-%20Flat%20Wood))
  (bind _new_wood_material___flat_wood_2 (Variables|Default|GetNew%20Wood%20Material%20-%20Flat%20Wood))
  (bind _new_wood_material___trim_wood (Variables|Default|GetNew%20Wood%20Material%20-%20Trim%20Wood))
  (bind _new_countertop_material (Variables|Default|GetNew%20Countertop%20Material))
  (bind _sm_kitchen_drawer (Variables|Default|GetSM_Kitchen_Drawer))
  (if (Variables|Default|GetSection%201%20Sink?)
    (bind _outrownames (DataTable|GetDataTableRowNames "/Game/InteriorBuildingKit/Struct/Sinks_DataTable.Sinks_DataTable"))
    (bind _returnvalue (Utilities|GetDataTableRow "/Game/InteriorBuildingKit/Struct/Sinks_DataTable.Sinks_DataTable" (Utilities|Array|Get(acopy) _outrownames (Variables|Default|GetSink%20Option)) :!label _label)
      (:then
        (Components|StaticMesh|SetStaticMesh (Variables|Default|GetSM_Kitchen_Countertop) (select (Variables|Default|GetSection%201%20Sink?) "/Game/InteriorBuildingKit/Geometry/Assets/KitchenCounters/SM_Kitchen_Countertop1_Sink1.SM_Kitchen_Countertop1_Sink1" "/Game/InteriorBuildingKit/Geometry/Assets/KitchenCounters/SM_Kitchen_Countertop1.SM_Kitchen_Countertop1"))
        (bind _returnvalue_2 (AddComponent|AddStaticMeshComponent false (Math|Transform|MakeTransform "0,-35.000000, 0" "0, 0, 0" "1.000000,1.000000,1.000000"))) ; Adds Sink Geometry
        (Components|StaticMesh|SetStaticMesh _returnvalue_2 (.sinkgeometry _returnvalue))
        (Rendering|Material|SetMaterial _returnvalue_2 (.sinkmaterialidmain _returnvalue) (Variables|Default|GetNew%20Sink%20Material%20-%20Main))
        (Rendering|Material|SetMaterial _returnvalue_2 (.sinkmaterialidmetal _returnvalue) (Variables|Default|GetNew%20Sink%20Material%20-%20Metal))
        (bind _returnvalue_3 (AddComponent|AddStaticMeshComponent false (Math|Transform|MakeTransform "0,-35.000000, 0" "0, 0, 0" "1.000000,1.000000,1.000000"))) ; Adds Sink Drain
        (Components|StaticMesh|SetStaticMesh _returnvalue_3 (.draingeometry _returnvalue)))
      (:RowNotFound
        (Variables|Default|SetSink%20Option (- (Utilities|Array|Length _outrownames) 1))
        (goto _label))))
  (Utilities|IsValid _new_countertop_material
    (:Is%20Valid
      (Rendering|Material|SetMaterial (Variables|Default|GetSM_Kitchen_Countertop) 0 _new_countertop_material))
    (:Is%20Not%20Valid
      _))
  (Transformation|SetRelativeRotation (Variables|Default|GetSM_Kitchen_Door%20Left) (Math|Rotator|MakeRotator 0.0 0.0 (Math|Float|Lerp 0.0 179.0 (Variables|Default|GetOpen%20State%20-%20Left%20Door))) false false)
  (Transformation|SetRelativeRotation (Variables|Default|GetSM_Kitchen_Door%20Right) (Math|Rotator|MakeRotator 0.0 0.0 (Math|Float|Lerp 0.0 -179.0 (Variables|Default|GetOpen%20State%20-%20Right%20Door))) false false)
  (if (Variables|Default|GetSection%201%20Sink?)
    (Components|DestroyComponent (Variables|Default|GetSM_Handle_Drawer))
    (Components|StaticMesh|SetStaticMesh _sm_kitchen_drawer "/Game/InteriorBuildingKit/Geometry/Assets/KitchenCounters/SM_Kitchen_Counter_FrontBlank1.SM_Kitchen_Counter_FrontBlank1")
    (Components|StaticMesh|SetStaticMesh (Variables|Default|GetSM_Kitchen_Counter_Base1) "/Game/InteriorBuildingKit/Geometry/Assets/KitchenCounters/SM_Kitchen_Counter_SinkBase.SM_Kitchen_Counter_SinkBase")
    (else
      (Transformation|SetRelativeLocation _sm_kitchen_drawer (Math|Vector|MakeVector 0.0 (Math|Float|Lerp 0.0 55.0 (Variables|Default|GetOpen%20State%20-%20Drawer)) 0.0) false false)))
  (if (Variables|Default|GetSection%201%20Sink?)
    _
    (else
      (for (_array_element _array_index) (Variables|Default|GetShelf%20Height)
        (Utilities|Array|SetArrayElem (Variables|Default|GetShelf%20Height) _array_index (Math|Float|Clamp(Float) _array_element 1e+01 75.0))
        (bind _returnvalue_4 (AddComponent|AddStaticMeshComponent false (Math|Transform|MakeTransform (Math|Vector|MakeVector 0.0 0.0 (Math|Float|Clamp(Float) _array_element 1e+01 75.0)) "0, 0, 0" "1.000000,1.000000,1.000000")))
        (Utilities|IsValid _new_wood_material___flat_wood
          (:Is%20Valid
            (Rendering|Material|SetMaterial _returnvalue_4 0 _new_wood_material___flat_wood))))))
  (Utilities|IsValid _new_wood_material___flat_wood_2
    (:Is%20Valid
      (Rendering|Material|SetMaterial (Variables|Default|GetSM_Kitchen_Drawer) 0 _new_wood_material___flat_wood_2))
    (:Is%20Not%20Valid
      _))
  (Utilities|IsValid _new_wood_material___trim_wood
    (:Is%20Valid
      (Rendering|Material|SetMaterial (Variables|Default|GetSM_Kitchen_Counter_Base1) 1 _new_wood_material___trim_wood))
    (:Is%20Not%20Valid
      _))
  (bind _returnvalue_5 (Utilities|GetDataTableRow "/Game/InteriorBuildingKit/Struct/CounterHandleTypes_DataTable.CounterHandleTypes_DataTable" (Utilities|String|StringToName (Utilities|String|EnumtoString (Variables|Default|GetHandle%20Type))))
    (:then
      (if (>= (Variables|Default|GetHandle%20Option) (Utilities|Array|Length (.handletype _returnvalue_5)))
        (Variables|Default|SetHandle%20Option (- (Utilities|Array|Length (.handletype _returnvalue_5)) 1)))
      (Components|StaticMesh|SetStaticMesh (Variables|Default|GetSM_Handle_Left) (Utilities|Array|Get(acopy) (.handletype _returnvalue_5) (Variables|Default|GetHandle%20Option)))
      (Components|StaticMesh|SetStaticMesh (Variables|Default|GetSM_Handle_Right) (Utilities|Array|Get(acopy) (.handletype _returnvalue_5) (Variables|Default|GetHandle%20Option)))
      (Components|StaticMesh|SetStaticMesh (Variables|Default|GetSM_Handle_Drawer) (Utilities|Array|Get(acopy) (.handletype _returnvalue_5) (Variables|Default|GetHandle%20Option)))
      (Rendering|Material|SetMaterial (Variables|Default|GetSM_Handle_Left) 0 (Variables|Default|GetNew%20Handle%20Material)))))