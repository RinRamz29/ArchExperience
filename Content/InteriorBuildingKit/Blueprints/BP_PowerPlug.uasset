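; BP_PowerPlug is an interior-kit prop that builds a power cable with an optional end plug in its construction script.
; A referenced wall plug's selected port, if valid, sets EndLocation, to which the spline's last point and tangent align.
; Spline mesh segments form the cable with configurable mesh, width, twist, material and self-shadow-only variant.
; A data table row keyed by plug type supplies the spline-end offset and plug mesh.
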(event EventBeginPlay)

(event Collision|EventActorBeginOverlap
  (params (OtherActor :type Actor%20Object%20Reference)))

(event EventTick
  (params (DeltaSeconds :type Float%20%28single-precision%29)))

(fn ConstructionScript
  (bind _returnvalue (Transformation|GetActorTransform))
  (bind _cable_width (Variables|Default|GetCable%20Width))
  (bind _custom_cable_asset (Variables|Default|GetCustom%20Cable%20Asset))
  (bind _spline (Variables|Default|GetSpline))
  (bind _wall_plug_port (Variables|Default|GetWall%20Plug%20Port))
  (bind _wall_plug_bp_reference (Variables|Default|GetWall%20Plug%20BP%20Reference))
  (bind _spline_2 (Variables|Default|GetSpline))
  (bind _returnvalue_2 (Spline|GetNumberOfSplinePoints _spline_2))
  (bind _returnvalue_3 (- _wall_plug_port 1))
  (bind _plug_destination_1 (Variables|/Game/InteriorBuildingKit/Blueprints/BP_WallPlug.BP_WallPlug_C|GetPlug%20Destination%201 _wall_plug_bp_reference))
  (bind _plug_destination_2 (Variables|/Game/InteriorBuildingKit/Blueprints/BP_WallPlug.BP_WallPlug_C|GetPlug%20Destination%202 _wall_plug_bp_reference))
  (bind _returnvalue_4 (- _returnvalue_2 1))
  (Utilities|IsValid _wall_plug_bp_reference
    (:Is%20Valid
      (Variables|Default|SetEnd%20Location (Math|Transform|MakeTransform (Utilities|Select :Index _returnvalue_3 :Option%200 (Math|Transform|InverseTransformLocation _returnvalue (Transformation|GetWorldLocation _plug_destination_1)) :Option%201 (Math|Transform|InverseTransformLocation _returnvalue (Transformation|GetWorldLocation _plug_destination_2))) (Utilities|Select :Index _returnvalue_3 :Option%200 (Math|Transform|InverseTransformRotation _returnvalue (Transformation|GetWorldRotation _plug_destination_1)) :Option%201 (Math|Transform|InverseTransformRotation _returnvalue (Transformation|GetWorldRotation _plug_destination_2))) (.scale (Variables|Default|GetEnd%20Location)))))
    (:Is%20Not%20Valid
      _))
  (bind _returnvalue_5 (Utilities|GetDataTableRow "/Game/InteriorBuildingKit/Struct/PowerPlug_DataTable.PowerPlug_DataTable" (Utilities|String|StringToName (Utilities|String|EnumtoString (Variables|Default|GetPlug%20Type))))
    (:then
      (Spline|SetLocationatSplinePoint (Variables|Default|GetSpline) _returnvalue_4 (select (Variables|Default|GetUse%20end%20plug?) (+ (Math|Transform|TransformDirection (Variables|Default|GetEnd%20Location) (.location (.locationoffsetforsplineend _returnvalue_5))) (.Location (Math|Transform|BreakTransform (Variables|Default|GetEnd%20Location)))) (.Location (Math|Transform|BreakTransform (Variables|Default|GetEnd%20Location)))) "Local" true)
      (Spline|SetTangentatSplinePoint (Variables|Default|GetSpline) _returnvalue_4 (* (Math|Rotator|GetRotationXVector (Math|Rotator|SelectRotator (Math|Transform|TransformRotation (Variables|Default|GetEnd%20Location) (.rotation (.locationoffsetforsplineend _returnvalue_5))) (.rotation (Variables|Default|GetEnd%20Location)) (Variables|Default|GetUse%20end%20plug?))) (* (.x (.scale (Variables|Default|GetEnd%20Location))) -1e+01)) "Local" true)
      (for _index (range 0 (- (Spline|GetNumberOfSplinePoints (Variables|Default|GetSpline)) 2))
        (if (Variables|Default|GetShould%20cable%20self%20shadow%20only?)
          (bind _returnvalue_6 (AddComponent|AddSplineMeshComponent false))
          (else
            (bind _returnvalue_7 (AddComponent|AddSplineMeshComponent false))))
        (SplineMesh|SetForwardAxis (select (Variables|Default|GetShould%20cable%20self%20shadow%20only?) _returnvalue_6 _returnvalue_7) (Variables|Default|GetForward%20Axis) true)
        (SplineMesh|SetSplineUpDir (select (Variables|Default|GetShould%20cable%20self%20shadow%20only?) _returnvalue_6 _returnvalue_7) (Variables|Default|GetSpline%20Up%20Direction) true)
        (Components|StaticMesh|SetStaticMesh (select (Variables|Default|GetShould%20cable%20self%20shadow%20only?) _returnvalue_6 _returnvalue_7) (select (Utilities|IsValid _custom_cable_asset) _custom_cable_asset (Utilities|Select :Index (Variables|Default|GetCable%20Options) :Option%200 "/Game/InteriorBuildingKit/Geometry/Assets/WallDetails/Plugs/SM_WallPlug_Cable1.SM_WallPlug_Cable1" :Option%201 "/Game/InteriorBuildingKit/Geometry/Assets/WallDetails/Plugs/SM_WallPlug_Cable1.SM_WallPlug_Cable1")))
        (SplineMesh|SetStartandEnd (select (Variables|Default|GetShould%20cable%20self%20shadow%20only?) _returnvalue_6 _returnvalue_7) (.location (Spline|GetTransformatSplinePoint _spline _index "Local" false)) (Spline|GetTangentatSplinePoint _spline _index "Local") (.location (Spline|GetTransformatSplinePoint _spline (+ _index 1) "Local" false)) (Spline|GetTangentatSplinePoint _spline (+ _index 1) "Local") true :!class /Script/Engine.SplineMeshComponent)
        (Class|SplineMeshComponent|SetStartRoll (select (Variables|Default|GetShould%20cable%20self%20shadow%20only?) _returnvalue_6 _returnvalue_7) (* (Math|Conversions|ToFloat(Integer) _index) (Variables|Default|GetTwist)) true)
        (Class|SplineMeshComponent|SetEndRoll (select (Variables|Default|GetShould%20cable%20self%20shadow%20only?) _returnvalue_6 _returnvalue_7) (* (Math|Conversions|ToFloat(Integer) (+ _index 1)) (Variables|Default|GetTwist)) true)
        (SplineMesh|SetStartScale (select (Variables|Default|GetShould%20cable%20self%20shadow%20only?) _returnvalue_6 _returnvalue_7) (Math|Vector2D|MakeVector2D _cable_width _cable_width) true :!class /Script/Engine.SplineMeshComponent)
        (SplineMesh|SetEndScale (select (Variables|Default|GetShould%20cable%20self%20shadow%20only?) _returnvalue_6 _returnvalue_7) (Math|Vector2D|MakeVector2D _cable_width _cable_width) true :!class /Script/Engine.SplineMeshComponent)
        (Rendering|Material|SetMaterial (select (Variables|Default|GetShould%20cable%20self%20shadow%20only?) _returnvalue_6 _returnvalue_7) 0 (Variables|Default|GetCustom%20Cable%20Material)))
      (if (Variables|Default|GetUse%20end%20plug?)
        (bind _returnvalue_8 (Utilities|GetDataTableRow "/Game/InteriorBuildingKit/Struct/PowerPlug_DataTable.PowerPlug_DataTable" (Utilities|String|StringToName (Utilities|String|EnumtoString (Variables|Default|GetPlug%20Type))))
          (:then
            (bind _returnvalue_9 (AddComponent|AddStaticMeshComponent false (Math|Transform|MakeTransform (.location (Variables|Default|GetEnd%20Location)) (.rotation (Variables|Default|GetEnd%20Location)) "1.000000,1.000000,1.000000")))
            (Components|StaticMesh|SetStaticMesh _returnvalue_9 (Utilities|Array|Get(acopy) (.assettypes _returnvalue_8) (Variables|Default|GetPlug%20Options)))
            (Class|SceneComponent|AddLocalTransform _returnvalue_9 (Math|Transform|MakeTransform "0, 0, 0" "0,-90.000000, 0" "1.000000,1.000000,1.000000") false false)
            (Rendering|Material|SetMaterial _returnvalue_9 (Variables|Default|GetCustom%20Plug%20Material%20ID%20Number) (Variables|Default|GetCustom%20Plug%20Material))))))))