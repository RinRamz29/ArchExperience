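; Adjustable lamp prop that poses its jointed arm and head from a LightPosition transform in the construction script.
; LightPosition is clamped to a range in the X-Z plane, and its look-at pitch from the joint tilts the joint and counter-rotates the head, which adds the transform's own pitch.
; Distance to the target slides the pole, both light groups snap to the head, and NewMainMaterial is applied to the three meshes.
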(event EventBeginPlay
  (|CallParentFunction) ; This node is disabled and will not be called.\nDrag off pins to build functionality.
)

(event Collision|EventActorBeginOverlap
  (params (OtherActor :type Actor%20Object%20Reference))
  (|CallParentFunction OtherActor) ; This node is disabled and will not be called.\nDrag off pins to build functionality.
)

(event EventTick
  (params (DeltaSeconds :type Float%20%28single-precision%29))
  (|CallParentFunction DeltaSeconds) ; This node is disabled and will not be called.\nDrag off pins to build functionality.
)

(fn ConstructionScript
  (bind _sm_lamp1_head (Variables|Default|GetSM_Lamp1_Head))
  (|CallParentFunction)
  (Variables|Default|SetLight%20Position (Math|Transform|MakeTransform (Math|Vector|MakeVector (Math|Float|Clamp(Float) (.x (.location (Variables|Default|GetLight%20Position))) -1.5e+02 -1e+01) 0.0 (Math|Float|Clamp(Float) (.z (.location (Variables|Default|GetLight%20Position))) 25.0 3e+02)) (Math|Rotator|MakeRotator 0.0 (.pitch (.rotation (Variables|Default|GetLight%20Position))) 0.0) (.scale (Variables|Default|GetLight%20Position))))
  (Transformation|SetRelativeRotation (Variables|Default|GetSM_Lamp1_Joint1) (Math|Rotator|MakeRotator 0.0 (Math|Float|Lerp 0.0 -65.0 (Math|Float|Clamp(Float) (/ (.pitch (Math|Rotator|FindLookatRotation (Variables|/Script/Engine.SceneComponent|GetRelativeLocation (Variables|Default|GetSM_Lamp1_Joint1)) (.location (Variables|Default|GetLight%20Position)))) 5e+01) -1.0)) 0.0) false false)
  (Transformation|SetRelativeRotation _sm_lamp1_head (Math|Rotator|MakeRotator 0.0 (Math|Float|Lerp 0.0 65.0 (Math|Float|Clamp(Float) (/ (.pitch (Math|Rotator|FindLookatRotation (Variables|/Script/Engine.SceneComponent|GetRelativeLocation (Variables|Default|GetSM_Lamp1_Joint1)) (.location (Variables|Default|GetLight%20Position)))) 5e+01) -1.0)) 0.0) false false)
  (Transformation|AddLocalRotation _sm_lamp1_head (Math|Rotator|MakeRotator 0.0 (.pitch (.rotation (Variables|Default|GetLight%20Position))) 0.0) false false)
  (Transformation|SetRelativeLocation (Variables|Default|GetSM_Lamp1_Pole) (Math|Vector|MakeVector (Math|Float|Lerp 45.0 -2e+01 (Math|Float|Clamp(Float) (/ (- (Math|Vector|VectorLength (- (Variables|/Script/Engine.SceneComponent|GetRelativeLocation (Variables|Default|GetSM_Lamp1_Joint1)) (.location (Variables|Default|GetLight%20Position)))) 5e+01) 75.0))) 0.0 2e+01) false false)
  (Transformation|AttachComponentToComponent (Variables|Default|GetLight%20Group%20-%20Lightbulbs) (Variables|Default|GetSM_Lamp1_Head) "None" "SnapToTarget" "SnapToTarget" "KeepRelative" true)
  (Transformation|AttachComponentToComponent (Variables|Default|GetLight%20Group%20-%20Down) (Variables|Default|GetSM_Lamp1_Head) "None" "SnapToTarget" "SnapToTarget" "KeepRelative" true)
  (Rendering|Material|SetMaterial (Variables|Default|GetSM_Lamp1_Joint1) 0 (Variables|Default|GetNew%20Main%20Material)))